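; BP_PlayerController is a player controller that passes a player's character choice to the lobby game mode.
; SelectCharacter checks that the game mode is valid, casts it to BP_LobbyGameMode, then calls its SelectCharacter with itself and the chosen class.
; A block that would show a CharacterSelect widget to the local player is unconnected and never runs; BeginPlay and Tick do nothing.
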(event `self.ReceiveBeginPlay`)

(event `SelectCharacter`
  (params (CharacterClass :type "GB_PlayableCharacter Class Reference"))
  (bind _returnvalue (`GameplayStatics.GetGameMode`))
  (`/Engine/EditorBlueprintResources/StandardMacros.IsValid` _returnvalue
    (:`Is Valid`
      (bind _asbp_lobby_game_mode (cast `/Game/GameModes/BP_LobbyGameMode` _returnvalue))
      (`/Game/GameModes/BP_LobbyGameMode.SelectCharacter` _asbp_lobby_game_mode self CharacterClass))))

(fn `UserConstructionScript`)