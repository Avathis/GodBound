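; BP_FireBall1 is a fireball projectile that damages GB_Character actors it overlaps, excluding player 0's character.
; On overlap it applies the BP_DAMAGE_REMOVEAFTER gameplay effect through the target's Ability System Component, then destroys itself.
; Overlapping the player only prints a debug string.
; Disconnected leftovers hold an older BP_DamageEffect hit check and a pitch rotation test; no movement logic appears in the graphs.
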(event `self.ReceiveBeginPlay`)

(event `self.ReceiveActorBeginOverlap`
  (params (OtherActor :type "Actor Object Reference"))
  (bind _returnvalue (`AbilitySystemBlueprintLibrary.GetAbilitySystemComponent` OtherActor))
  (bind _asgb_character (cast `GB_Character` OtherActor))
  (`/Engine/EditorBlueprintResources/StandardMacros.IsValid` _returnvalue
    (:`Is Valid`
      (if (!= _asgb_character (`GameplayStatics.GetPlayerCharacter` 0))
        (if true
          (`AbilitySystemComponent.BP_ApplyGameplayEffectToSelf` :`self` _returnvalue :`GameplayEffectClass` "/Game/Effects/BP_DAMAGE_REMOVEAFTER.BP_DAMAGE_REMOVEAFTER_C")
          (`self.K2_DestroyActor`))
        (else
          (`KismetSystemLibrary.PrintString` "Lol"))))))

(event `self.ReceiveHit`
  (params (MyComp :type "PrimitiveComponent Object Reference") (Other :type "Actor Object Reference") (OtherComp :type "PrimitiveComponent Object Reference") (bSelfMoved :type Boolean) (HitLocation :type "Vector Structure") (HitNormal :type "Vector Structure") (NormalImpulse :type "Vector Structure") (Hit :type "HitResult Structure (by ref)")))

(fn `UserConstructionScript`)