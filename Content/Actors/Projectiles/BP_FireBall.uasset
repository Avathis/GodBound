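; Fireball projectile actor that applies damage through the Gameplay Ability System when it overlaps another actor.
; On overlap with a valid Ability System Component, it compares the other actor, then either applies BP_DamageEffect to that component and destroys itself, or prints a debug string.
; Construction, BeginPlay and Tick do nothing, and leftover mesh rotation logic is disconnected.
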(event `self.ReceiveBeginPlay`)

(event `self.ReceiveActorBeginOverlap`
  (params (OtherActor :type "Actor Object Reference"))
  (bind _returnvalue (`AbilitySystemBlueprintLibrary.GetAbilitySystemComponent` null))
  (`/Engine/EditorBlueprintResources/StandardMacros.IsValid` _returnvalue
    (:`Is Valid`
      (if (!= OtherActor null)
        (`AbilitySystemComponent.BP_ApplyGameplayEffectToSelf` :`self` _returnvalue :`GameplayEffectClass` "/Game/Effects/BP_DamageEffect.BP_DamageEffect_C")
        (`self.K2_DestroyActor`)
        (else
          (`KismetSystemLibrary.PrintString` "Lol"))))))

(fn `UserConstructionScript`)