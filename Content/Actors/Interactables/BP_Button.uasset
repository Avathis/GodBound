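; BP_Button is an interactable button actor that animates a press when interacted with.
; InteractwithActor calls InteractAction, which plays a timeline that drives the Cylinder's relative Y position.
; Each tick it stores the ButtonCube's world location and the Cylinder's world rotation as left-hand position and rotation, while GetLeftHandIK returns only a zero vector.
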(event `self.ReceiveBeginPlay`)

(event `self.ReceiveTick`
  (params (DeltaSeconds :type "Float (single-precision)"))
  (set `self.LeftHandPosition` (`SceneComponent.K2_GetComponentLocation` (`self.ButtonCube`)))
  (set `self.LefttHandRotation` (`SceneComponent.K2_GetComponentRotation` (`self.Cylinder`))))

(event `self.InteractAction`
  (bind _cylinder (`self.Cylinder`))
  (bind (_relativelocation_x _relativelocation_y _relativelocation_z) (`KismetMathLibrary.BreakVector` (`SceneComponent.RelativeLocation` _cylinder)))
  (bind (_direction _newtrack_0) (`Timeline|Timeline`)
    (:`Update`
      (`SceneComponent.K2_SetRelativeLocation` _cylinder (`KismetMathLibrary.MakeVector` _relativelocation_x _newtrack_0 _relativelocation_z) false false))))

(event `/Game/Actors/Interactables/BI_Interacts.InteractWithActor`
  (`self.InteractAction`))

(fn `GetLeftHandIK`
  (returns (ReturnValue :type "Vector Structure"))
  (return (0.0 0.0 0.0)))

(fn `UserConstructionScript`)