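; Hephaestus character Blueprint built on the Gameplay Ability System, granting sprint, jump and a placeholder ability at BeginPlay and starting out of combat.
; Events forward combat changes and drive movement state and walk speed through the advanced movement component.
; A timeline ramps speed while charge sprint lasts, and ability sprint switches rotation to follow movement at reduced speed.
; Disconnected nodes hold debug prints and test grants for fire and lightning abilities.
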(event `self.ReceiveBeginPlay`
  (`self.GrantAbility` "/Game/Characters/Blueprints/SharedAbilities/GA_Sprint.GA_Sprint_C" 1 3)
  (`self.GrantAbility` "/Game/Characters/Blueprints/Hephaestus/Abilities/Jump/GA_Heph_Jump.GA_Heph_Jump_C" 0 4)
  (`self.GrantAbility` "/Game/Characters/Blueprints/Hephaestus/Abilities/TrashThisAFter.TrashThisAFter_C" 0 7)
  (`AbilitySystemComponent.BP_ApplyGameplayEffectToSelf` :`self` (`self.AbilitySystemComponent`) :`GameplayEffectClass` "/Game/Characters/Blueprints/Hephaestus/Abilities/EnterExitCombat/GE_OutOfCombat.GE_OutOfCombat_C"))

(event `self.ReceiveTick`
  (params (DeltaSeconds :type "Float (single-precision)")))

(event `self.Change Movement Type`
  (params (NewMovmentType :type "EMovementState Enum" :default "EMS_Idle"))
  (bind _returnvalue (`self.GetAdvMovementComponent`))
  (`GB_CharacterMovementComponent.ChangeMovementState` _returnvalue NewMovmentType))

(event `/Game/Interfaces/BPI_AbilityInterface.ExitCombatI`
  (`self.ExitCombat`))

(event `/Game/Interfaces/BPI_AbilityInterface.EnterCombatI`
  (`self.EnterCombat`))

(event `/Game/Interfaces/BPI_AbilityInterface.AddSpeed`
  (params (AddedSpeed :type "Float (double-precision)"))
  (bind _returnvalue (`self.GetAdvMovementComponent`))
  (`self.Change Movemnt Speed` (+ (`CharacterMovementComponent.MaxWalkSpeed` _returnvalue) AddedSpeed)))

(event `/Game/Interfaces/BPI_AbilityInterface.GraduallyAddSpeed`
  (params (NewMaxSpeed :type "Float (double-precision)"))
  (bind (_direction _movespeed) (`Timeline|ChargedSpeedTL` :!via `PlayFromStart` :!label _label)
    (:`Update`
      (bind _returnvalue (`self.GetAdvMovementComponent`))
      (bind _returnvalue_2 (`GB_CharacterMovementComponent.GetMovementType` _returnvalue))
      (if (`|EnumInequality` _returnvalue_2 "EMS_HephaestusChargeSprint")
        (goto _label :!via `Stop`)
        (else
          (set `CharacterMovementComponent.MaxWalkSpeed` (`KismetMathLibrary.Lerp` (`CharacterMovementComponent.MaxWalkSpeed` _returnvalue) NewMaxSpeed (`KismetMathLibrary.SafeDivide` _movespeed 30.0)) _returnvalue))))))

(event `self.Change Movemnt Speed`
  (params (NewMovementSpeed :type "Float (double-precision)"))
  (bind _returnvalue (`self.GetAdvMovementComponent`))
  (set `CharacterMovementComponent.MaxWalkSpeed` NewMovementSpeed _returnvalue))

(event `/Game/Interfaces/BPI_AbilityInterface.Start Ability Sprint`
  (bind _returnvalue (`self.GetAdvMovementComponent`))
  (`Controller.SetIgnoreLookInput` (`self.GetController`) false)
  (set `self.bUseControllerRotationYaw` false)
  (set `CharacterMovementComponent.bOrientRotationToMovement` true _returnvalue)
  (`self.Change Movemnt Speed` (* (`CharacterMovementComponent.MaxWalkSpeed` _returnvalue) 0.77)))

(event `/Game/Interfaces/BPI_AbilityInterface.EndAbilitySprint`
  (bind _returnvalue (`self.GetAdvMovementComponent`))
  (set `self.bUseControllerRotationYaw` true)
  (set `CharacterMovementComponent.bOrientRotationToMovement` false _returnvalue))

(event `/Game/Interfaces/BPI_AbilityInterface.OverlapInAbilitySprint`
  (bind _returnvalue (`self.GetAdvMovementComponent`))
  (`KismetSystemLibrary.PrintString` (`KismetStringLibrary.Conv_DoubleToString` (`CharacterMovementComponent.MaxWalkSpeed` _returnvalue)))
  (`KismetSystemLibrary.PrintString` (`KismetStringLibrary.Conv_DoubleToString` (`KismetMathLibrary.VSize` (`MovementComponent.Velocity` _returnvalue)))))

(fn `UserConstructionScript`)