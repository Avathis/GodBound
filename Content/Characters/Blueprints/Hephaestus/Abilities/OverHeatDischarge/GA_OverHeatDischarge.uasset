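; Hephaestus's OverHeat Discharge gameplay ability, a hold-and-release area attack centred on the avatar.
; It plays a wind-up montage until input release, then a discharge montage that outlives the ability.
; A discharge gameplay event triggers a debug-drawn sphere overlap, applying a placeholder-named damage effect to enemy characters.
; EndAbility runs inside the hit loop or on discharge montage completion; cancelling the wind-up cancels the ability.
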(event `self.K2_ActivateAbility`
  (bind _returnvalue (`Actor.K2_GetActorLocation` (`self.GetAvatarActorFromActorInfo`)))
  (`self.K2_CommitAbility`)
  (`AbilityTask_PlayMontageAndWait.CreatePlayMontageAndWaitProxy` "None" "/Game/Characters/Blueprints/Hephaestus/Abilities/OverHeatDischarge/Ability_OverHeatDischarge2_Montage.Ability_OverHeatDischarge2_Montage" 1.0 "None"
    (:`then`
      (`AbilityTask_WaitInputRelease.WaitInputRelease` false
        (:`OnRelease`
          (`AbilityTask_PlayMontageAndWait.CreatePlayMontageAndWaitProxy` "None" "/Game/Characters/Blueprints/Hephaestus/Abilities/OverHeatDischarge/Ability_OverHeatDischarge_Montage.Ability_OverHeatDischarge_Montage" 1.0 "Start" false
            (:`then`
              (`AbilityTask_WaitGameplayEvent.WaitGameplayEvent` (struct :`TagName` "Abilities.Fire.OverHeat.Discharge") null
                (:`EventReceived`
                  (`KismetSystemLibrary.DrawDebugSphere` _returnvalue 250.0 12 (struct :`R` 1.0 :`G` 1.0 :`B` 1.0 :`A` 1.0) 2.0)
                  (bind _outactors (`KismetSystemLibrary.SphereOverlapActors` _returnvalue 250.0 (`|MakeArray` (enumliteral `EObjectTypeQuery` "ObjectTypeQuery3"))))
                  (for _array_element _outactors
                    (bind _asgb_enemy_character (cast `GB_EnemyCharacter` _array_element))
                    (`AbilitySystemComponent.BP_ApplyGameplayEffectToSelf` :`self` (`GB_Character.AbilitySystemComponent` _asgb_enemy_character) :`GameplayEffectClass` "/Game/Effects/BP_DAMAGE_REMOVEAFTER.BP_DAMAGE_REMOVEAFTER_C")
                    (`self.K2_EndAbility`)))))
            (:`OnCompleted`
              (`self.K2_EndAbility`))))))
    (:`OnCancelled`
      (`self.K2_CancelAbility`))))