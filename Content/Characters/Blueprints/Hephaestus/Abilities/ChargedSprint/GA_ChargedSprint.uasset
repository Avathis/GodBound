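; Hephaestus' Charged Sprint gameplay ability, which applies its effect, switches to charge-sprint movement and gradually builds speed through interface messages.
; Each overlap compares velocity to max walk speed, ending the charge when too slow or sharply slowed, and docking speed for moderate losses.
; Surviving overlaps resume acceleration immediately and re-arm detection after a short delay.
; Ending restores walking and removes the effect; input release is not wired to end it.
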(event `self.K2_ActivateAbility`
  (bind _returnvalue (`self.GetAvatarActorFromActorInfo`))
  (bind (_owneractor _avataractor _playercontroller _abilitysystemcomponent _skeletalmeshcomponent _animinstance _movementcomponent) (break `GameplayAbilityActorInfo` (`self.GetActorInfo`)))
  (`self.K2_CommitAbility`)
  (bind _returnvalue_2 (`self.BP_ApplyGameplayEffectToOwner` "/Game/Characters/Blueprints/Hephaestus/Abilities/ChargedSprint/GE_ChargedSprint.GE_ChargedSprint_C"))
  (`AbilityTask_WaitInputRelease.WaitInputRelease` false
    (:`then`
      (if (`KismetSystemLibrary.DoesImplementInterface` _returnvalue "/Game/Interfaces/BPI_MovementInterface.BPI_MovementInterface_C")
        (message `/Game/Interfaces/BPI_AbilityInterface.Start Ability Sprint` _returnvalue)
        (message `/Game/Interfaces/BPI_MovementInterface.Change Movement Type` _returnvalue "EMS_HephaestusChargeSprint")
        (if (`KismetSystemLibrary.DoesImplementInterface` _returnvalue "/Game/Interfaces/BPI_AbilityInterface.BPI_AbilityInterface_C")
          (message `/Game/Interfaces/BPI_AbilityInterface.GraduallyAddSpeed` _returnvalue 1400.0)
          (`AbilityTask_WaitOverlap.WaitForOverlap` :!label _label
            (:`OnOverlap`
              (bind _returnvalue_3 (`GB_Character.GetAdvMovementComponent` (cast `GB_PlayableCharacter` _owneractor :!pure true)))
              (bind _returnvalue_4 (`KismetMathLibrary.VSize` (`MovementComponent.Velocity` _returnvalue_3)))
              (if (< _returnvalue_4 300.0)
                (`self.K2_EndAbility`)
                (else
                  ;[1 1 1] CompleteStop
                  (if (> (- (`CharacterMovementComponent.MaxWalkSpeed` _returnvalue_3) _returnvalue_4) 600.0)
                    (`self.K2_EndAbility`)
                    (else
                      ;[1 1 1] SlowDown
                      (if (> (- (`CharacterMovementComponent.MaxWalkSpeed` _returnvalue_3) (`KismetMathLibrary.VSize` (`MovementComponent.Velocity` _returnvalue_3))) 300.0)
                        (message `/Game/Interfaces/BPI_AbilityInterface.AddSpeed` _owneractor -300.0))
                      (`AbilityTask_WaitDelay.WaitDelay` 0.1
                        (:`then`
                          (message `/Game/Interfaces/BPI_AbilityInterface.GraduallyAddSpeed` _owneractor 1400.0))
                        (:`OnFinish`
                          (goto _label))))))))))))))

(event `self.K2_OnEndAbility`
  (params (bWasCancelled :type Boolean))
  (bind _returnvalue (`self.GetAvatarActorFromActorInfo`))
  (message `/Game/Interfaces/BPI_MovementInterface.Change Movement Type` _returnvalue "EMS_Walking")
  (message `/Game/Interfaces/BPI_AbilityInterface.EndAbilitySprint` _returnvalue)
  (`self.BP_RemoveGameplayEffectFromOwnerWithHandle` (stale `self.K2_ActivateAbility` _returnvalue_2)))