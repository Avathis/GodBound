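; Gameplay ability for Hephaestus's Empower Stance, which applies an empowered effect to its owner during a stance montage.
; It commits, plays the montage at half speed and waits for the Abilities.Fire.Empowered event to apply the effect and debug-print owned tags.
; It then ends on the next matching ability activation or whenever the montage finishes, blends out or is interrupted, without stopping the montage itself.
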(event `self.K2_ActivateAbility`
  (`self.K2_CommitAbility`)
  (`AbilityTask_PlayMontageAndWait.CreatePlayMontageAndWaitProxy` "None" "/Game/Characters/Blueprints/Hephaestus/Abilities/EmpowerStance/Aibility_EmpowerStanceMontage.Aibility_EmpowerStanceMontage" 0.5 "None" false
    (:`then`
      (`AbilityTask_WaitGameplayEvent.WaitGameplayEvent` (struct :`TagName` "Abilities.Fire.Empowered") null
        (:`EventReceived`
          (`self.BP_ApplyGameplayEffectToOwner` "/Game/Characters/Blueprints/Hephaestus/Abilities/EmpowerStance/GE_HephaestusEmpowered.GE_HephaestusEmpowered_C")
          (`KismetSystemLibrary.PrintString` (`BlueprintGameplayTagLibrary.GetDebugStringFromGameplayTagContainer` (`GameplayTagAssetInterface.GetOwnedGameplayTags` (`AbilitySystemBlueprintLibrary.GetAbilitySystemComponent` (`self.GetAvatarActorFromActorInfo`)))))
          (`AbilityTask_WaitAbilityActivate.WaitForAbilityActivateWithTagRequirements` (struct)
            (:`OnActivate`
              (`self.K2_EndAbility`))))))
    (:`OnCompleted`
      (`self.K2_EndAbility` :!label _label))
    (:`OnBlendOut`
      (goto _label))
    (:`OnInterrupted`
      (goto _label))
    (:`OnCancelled`
      (goto _label))))