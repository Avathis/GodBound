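; Gameplay ability for Hephaestus's Pyr throw, currently a debug prototype that spawns no projectile.
; On activation it waits for confirm or cancel input, with only confirm handled.
; Confirm commits the ability, runs a camera hit trace on the GB_PlayableCharacter avatar, draws a debug line from the hand socket to the hit location, then ends.
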(event `self.K2_ActivateAbility`
  (`KismetSystemLibrary.PrintString` "Waiting")
  (`AbilityTask_WaitConfirmCancel.WaitConfirmCancel`
    (:`OnConfirm`
      (bind _asgb_playable_character (cast `GB_PlayableCharacter` (`self.GetAvatarActorFromActorInfo`)))
      (`self.K2_CommitAbility`)
      (bind _returnvalue (`GB_PlayableCharacter.HitTraceFromCamera` _asgb_playable_character 8000.0))
      (`KismetSystemLibrary.DrawDebugLine` (`SceneComponent.GetSocketLocation` (`Character.Mesh` _asgb_playable_character) "HandSocket") (`.Location` (`GameplayStatics.BreakHitResult` _returnvalue)) (struct) 10.0 1.0)
      (`KismetSystemLibrary.PrintString` "YAY")
      (`self.K2_EndAbility`))))