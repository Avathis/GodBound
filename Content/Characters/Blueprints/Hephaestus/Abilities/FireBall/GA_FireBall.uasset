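; GA_FireBall is Hephaestus's fireball gameplay ability, which commits and applies an overheat effect to the owner.
; It spawns a gravity-free BP_FireBall1 at the character's hand socket, attaches it and plays the throw montage.
; On the release gameplay event it detaches the ball, enables gravity and launches it along a suggested toss velocity toward the camera trace point.
; Debug drawing and printing remain, and montage blend-out or interruption ends the ability.
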(event `self.K2_ActivateAbility`
  (`self.K2_CommitAbility`)
  (`self.BP_ApplyGameplayEffectToOwner` "/Game/Effects/Utility/BP_OverHeatEffect.BP_OverHeatEffect_C")
  (bind _asbp_character_base (cast `/Game/Characters/BP_CharacterBase` (`.OwnerActor` (break `GameplayAbilityActorInfo` (`self.GetActorInfo`))))
    (:`then`
      (bind _mesh (`Character.Mesh` _asbp_character_base))
      (bind _returnvalue (`SceneComponent.GetSocketLocation` _mesh "HandSocket"))
      (bind (_asynctaskproxy _spawnedactor) (`GameplayTask_SpawnActor.SpawnActor` null _returnvalue (`SceneComponent.GetSocketRotation` _mesh "HandSocket") "/Game/Actors/Projectiles/BP_FireBall1.BP_FireBall1_C" false null)
        (:`Success`
          (bind _asbp_fire_ball_1 (cast `/Game/Actors/Projectiles/BP_FireBall1` _spawnedactor))
          (`PrimitiveComponent.SetEnableGravity` (`Projectile.StaticMesh` _asbp_fire_ball_1) false)
          (`KismetSystemLibrary.DrawDebugSphere` _returnvalue 10.0 12 (struct :`R` 1.0 :`B` 0.035882 :`A` 1.0) 10.0 2.6)
          (`Actor.K2_AttachToComponent` _spawnedactor (`Character.Mesh` _asbp_character_base) "HandSocket" "KeepWorld" "KeepWorld" "KeepWorld" true)
          (`AbilityTask_PlayMontageAndWait.CreatePlayMontageAndWaitProxy` "None" "/Game/Characters/Blueprints/Hephaestus/Abilities/FireBall/FireBall_Montage.FireBall_Montage"
            (:`then`
              (`AbilityTask_WaitGameplayEvent.WaitGameplayEvent` (struct :`TagName` "Damage.Fire.Fireball.Release") null
                (:`EventReceived`
                  (bind _returnvalue_2 (`GB_Character.TraceFromCamera` _asbp_character_base))
                  (bind _returnvalue_3 (`SceneComponent.GetSocketLocation` (`Character.Mesh` _asbp_character_base) "HandSocket"))
                  (`KismetSystemLibrary.DrawDebugLine` _returnvalue_3 _returnvalue_2 (struct :`R` 1.0 :`B` 0.078579 :`A` 1.0) 5.0)
                  (`Actor.K2_DetachFromActor` _asbp_fire_ball_1 "KeepWorld" "KeepWorld" "KeepWorld")
                  (bind _staticmesh (`Projectile.StaticMesh` _asbp_fire_ball_1))
                  (`PrimitiveComponent.SetEnableGravity` _staticmesh true)
                  (`PrimitiveComponent.SetEnableGravity` (`Projectile.StaticMesh` _asbp_fire_ball_1) true)
                  (bind _tossvelocity (`GameplayStatics.BlueprintSuggestProjectileVelocity` _returnvalue_3 _returnvalue_2 1500.0 0.0 "DoNotTrace" 32.0))
                  (`KismetSystemLibrary.PrintString` "Hello" true true (struct :`R` 1.0 :`G` 0.007958 :`A` 1.0))
                  (`PrimitiveComponent.SetAllPhysicsLinearVelocity` _staticmesh _tossvelocity true))))
            (:`OnBlendOut`
              (`self.K2_EndAbility` :!label _label))
            (:`OnInterrupted`
              (goto _label))
            (:`OnCancelled`
              (goto _label))))))
    (:`CastFailed`
      (`self.K2_CancelAbility`))))