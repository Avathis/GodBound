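; Gameplay ability for Zeus's lightning bolt, a hold-to-channel attack with placeholder damage and debug-line visuals.
; A montage's release event triggers a camera trace that damages the enemy hit.
; While input is held, an additive-named montage repeats, and each re-release event multi-traces from that enemy to the left hand, damaging enemies along the line.
; Releasing input or losing the target ends the ability.
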(event `self.K2_ActivateAbility`
  (`self.K2_CommitAbility`)
  (`AbilityTask_PlayMontageAndWait.CreatePlayMontageAndWaitProxy` "None" "/Game/Characters/Blueprints/ZEUS/Abilities/LightningBolt/Ability_LightningBoltTest.Ability_LightningBoltTest"
    (:`then`
      (`AbilityTask_WaitGameplayEvent.WaitGameplayEvent` (struct :`TagName` "Abilities.Lightning.Bolt.Release") null true
        (:`EventReceived`
          (bind _asgb_playable_character (cast `GB_PlayableCharacter` (`self.GetAvatarActorFromActorInfo`)))
          (bind _returnvalue (`GB_PlayableCharacter.HitTraceFromCamera` _asgb_playable_character 4000.0))
          (bind (_bblockinghit _binitialoverlap _time _distance _location _impactpoint _normal _impactnormal _physmat _hitactor) (`GameplayStatics.BreakHitResult` _returnvalue))
          (if _bblockinghit
            (bind _returnvalue_2 (`SceneComponent.GetSocketLocation` (`Character.Mesh` _asgb_playable_character) "LeftHandSocket"))
            (`KismetSystemLibrary.DrawDebugLine` _returnvalue_2 _location (struct :`R` 1.0 :`B` 0.853391 :`A` 1.0) 5.0 1.0)
            (`/Engine/EditorBlueprintResources/StandardMacros.IsValid` _hitactor
              (:`Is Valid`
                (bind _asgb_enemy_character (cast `GB_EnemyCharacter` _hitactor))
                (`AbilitySystemComponent.BP_ApplyGameplayEffectToSelf` :`self` (`GB_Character.AbilitySystemComponent` _asgb_enemy_character) :`GameplayEffectClass` "/Game/Effects/BP_DAMAGE_REMOVEAFTER.BP_DAMAGE_REMOVEAFTER_C")
                (`AbilityTask_WaitInputRelease.WaitInputRelease` false
                  (:`then`
                    (`/Engine/EditorBlueprintResources/StandardMacros.IsValid` _asgb_enemy_character :!label _label
                      (:`Is Valid`
                        (`AbilityTask_PlayMontageAndWait.CreatePlayMontageAndWaitProxy` "None" "/Game/Characters/Blueprints/ZEUS/Abilities/LightningBolt/Ability_LightningBoltTestAdd.Ability_LightningBoltTestAdd"
                          (:`then`
                            (`AbilityTask_WaitGameplayEvent.WaitGameplayEvent` (struct :`TagName` "Abilities.Lightning.Bolt.ReRelease") null
                              (:`EventReceived`
                                (bind _outhits (`KismetSystemLibrary.LineTraceMultiForObjects` (`Actor.K2_GetActorLocation` _asgb_enemy_character) _returnvalue_2 (`|MakeArray` (enumliteral `EObjectTypeQuery` "ObjectTypeQuery3"))))
                                (for _array_element _outhits
                                  (bind (_bblockinghit_2 _binitialoverlap_2 _time_2 _distance_2 _location_2 _impactpoint_2 _normal_2 _impactnormal_2 _physmat_2 _hitactor_2) (`GameplayStatics.BreakHitResult` _array_element))
                                  (`KismetSystemLibrary.DrawDebugLine` _location_2 _returnvalue_2 (struct :`R` 1.0 :`B` 0.109699 :`A` 1.0) 1.0)
                                  (bind _asgb_enemy_character_2 (cast `GB_EnemyCharacter` _hitactor_2))
                                  (`AbilitySystemComponent.BP_ApplyGameplayEffectToSelf` :`self` (`GB_Character.AbilitySystemComponent` _asgb_enemy_character_2) :`GameplayEffectClass` "/Game/Effects/BP_DAMAGE_REMOVEAFTER.BP_DAMAGE_REMOVEAFTER_C")))))
                          (:`OnCompleted`
                            (goto _label))))
                      (:`Is Not Valid`
                        (`self.K2_EndAbility`))))
                  (:`OnRelease`
                    (`self.K2_EndAbility`)))))
            (else
              (`self.K2_EndAbility`))))))
    (:`OnCompleted`
      (`self.K2_EndAbility`))))