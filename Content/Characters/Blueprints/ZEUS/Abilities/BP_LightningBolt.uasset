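; Zeus's Lightning Bolt gameplay ability, which damages targets supplied by a gameplay event during an attack montage.
; On activation it commits, plays the placeholder TestingPunch montage and waits for a single Lightning-tagged event, then applies BP_DamageEffect to that event's target data.
; The ability ends when the montage completes, blends out, is interrupted or is cancelled.
; Event-sending and debug print nodes are left unconnected, so the Lightning event must come from outside this graph.
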(event `self.K2_ActivateAbility`
  (`self.K2_CommitAbility`)
  (`AbilityTask_PlayMontageAndWait.CreatePlayMontageAndWaitProxy` "None" "/Game/Characters/Blueprints/TempCharacter/Animations/TestingPunch.TestingPunch"
    (:`then`
      (bind (_asynctaskproxy _payload) (`AbilityTask_WaitGameplayEvent.WaitGameplayEvent` (struct :`TagName` "Lightning") null true)
        (:`EventReceived`
          (`self.BP_ApplyGameplayEffectToTarget` (`.TargetData` (break `GameplayEventData` _payload)) "/Game/Effects/BP_DamageEffect.BP_DamageEffect_C"))))
    (:`OnCompleted`
      (`self.K2_EndAbility` :!label _label))
    (:`OnBlendOut`
      (goto _label))
    (:`OnInterrupted`
      (goto _label))
    (:`OnCancelled`
      (goto _label))))