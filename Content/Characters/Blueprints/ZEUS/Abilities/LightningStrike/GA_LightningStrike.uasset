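; Gameplay ability for Zeus's Lightning Strike, an area attack that damages enemies around a point traced from the camera.
; It plays the strike montage and waits for a release gameplay event before resolving the hit.
; A pawn sphere overlap at the traced point, shown with a debug sphere, applies a damage effect through each enemy character's ability system component.
; The ability ends when the montage completes, blends out or is interrupted or cancelled.
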(event `self.K2_ActivateAbility`
  (`AbilityTask_PlayMontageAndWait.CreatePlayMontageAndWaitProxy` "None" "/Game/Characters/Blueprints/ZEUS/Abilities/LightningStrike/LightningStrike_Montage.LightningStrike_Montage"
    (:`then`
      (`AbilityTask_WaitGameplayEvent.WaitGameplayEvent` (struct :`TagName` "Abilities.Lightning.Strik.Release") null
        (:`EventReceived`
          (bind _asgb_character (cast `GB_Character` (`self.GetAvatarActorFromActorInfo`)))
          (bind _returnvalue (`GB_Character.TraceFromCamera` _asgb_character))
          (`KismetSystemLibrary.DrawDebugSphere` _returnvalue 150.0 12 (struct :`R` 1.0 :`G` 1.0 :`B` 1.0 :`A` 1.0) 10.0 2.0)
          (bind _outactors (`KismetSystemLibrary.SphereOverlapActors` _returnvalue 150.0 (`|MakeArray` (enumliteral `EObjectTypeQuery` "ObjectTypeQuery3"))))
          (for _array_element _outactors
            (bind _asgb_enemy_character (cast `GB_EnemyCharacter` _array_element))
            (`AbilitySystemComponent.BP_ApplyGameplayEffectToSelf` :`self` (`AbilitySystemBlueprintLibrary.GetAbilitySystemComponent` _asgb_enemy_character) :`GameplayEffectClass` "/Game/Effects/BP_DAMAGE_REMOVEAFTER.BP_DAMAGE_REMOVEAFTER_C")))))
    (:`OnCompleted`
      (`self.K2_EndAbility` :!label _label))
    (:`OnBlendOut`
      (goto _label))
    (:`OnInterrupted`
      (goto _label))
    (:`OnCancelled`
      (goto _label))))