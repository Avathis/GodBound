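; Gameplay Ability that makes a playable character sprint while the input is held.
; On activation it lazily caches the avatar's GB_CharacterMovementComponent, ending the ability if either cast fails.
; It then starts a WaitInputRelease task and sets the movement state to Sprinting.
; Releasing the input ends the ability, and OnEndAbility sets the state back to Walking.
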(event `self.K2_ActivateAbility`
  (`KismetSystemLibrary.PrintString` "sprinting")
  (`/Engine/EditorBlueprintResources/StandardMacros.IsValid` (`self.PlayerMovementComponent`)
    (:`Is Valid`
      (`AbilityTask_WaitInputRelease.WaitInputRelease` true :!label _label
        (:`then`
          (`GB_CharacterMovementComponent.ChangeMovementState` (`self.PlayerMovementComponent`) "EMS_Sprinting"))
        (:`OnRelease`
          (`self.K2_EndAbility`))))
    (:`Is Not Valid`
      (bind _asgb_playable_character (cast `GB_PlayableCharacter` (`self.GetAvatarActorFromActorInfo`))
        (:`then`
          (bind _asgb_character_movement_component (cast `GB_CharacterMovementComponent` (`Pawn.GetMovementComponent` _asgb_playable_character))
            (:`then`
              (set `self.PlayerMovementComponent` _asgb_character_movement_component)
              (goto _label))
            (:`CastFailed`
              (`KismetSystemLibrary.PrintString` "Second cast failerd")
              (`self.K2_EndAbility`))))
        (:`CastFailed`
          (`KismetSystemLibrary.PrintString` "CastFailed")
          (`self.K2_EndAbility`))))))

(event `self.K2_OnEndAbility`
  (params (bWasCancelled :type Boolean))
  (`GB_CharacterMovementComponent.ChangeMovementState` (`self.PlayerMovementComponent`) "EMS_Walking"))