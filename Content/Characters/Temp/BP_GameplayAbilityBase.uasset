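; Gameplay Ability Blueprint in a Temp folder that fires a debug beam from the playable character and is set up to apply a gameplay effect to a target.
; After committing, it sends the beam's valid result to the owner as a gameplay event's Target.
; It only then starts waiting for a Lightning event to apply the effect from its TargetData.
; EndAbility follows without waiting for that event.
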(event `self.K2_ActivateAbility`
  (bind (_owneractor _avataractor) (break `GameplayAbilityActorInfo` (`self.GetActorInfo`)))
  (`self.K2_CommitAbility`)
  (bind _returnvalue (`PlayableCharacterBase.FireDebugBeam` (cast `/Game/Characters/Temp/MyPlayableCharacterBase` _avataractor :!pure true)))
  (`/Engine/EditorBlueprintResources/StandardMacros.IsValid` _returnvalue
    (:`Is Valid`
      (`AbilitySystemBlueprintLibrary.SendGameplayEventToActor` _owneractor (struct) (make `GameplayEventData` (struct) null _returnvalue))
      (`KismetSystemLibrary.PrintString` "Event sent")
      (bind (_asynctaskproxy _payload) (`AbilityTask_WaitGameplayEvent.WaitGameplayEvent` (struct :`TagName` "Lightning") null)
        (:`then`
          _)
        (:`EventReceived`
          (`self.BP_ApplyGameplayEffectToTarget` (`.TargetData` (break `GameplayEventData` _payload))))))
    (:`Is Not Valid`
      _))
  (`self.K2_EndAbility`))