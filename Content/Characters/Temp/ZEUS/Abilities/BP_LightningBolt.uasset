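; Gameplay ability for the ZEUS character's lightning bolt, currently using a TestingPunch montage and debug prints.
; On activation it commits, plays the montage and immediately starts listening for a Lightning gameplay event.
; A received event applies a gameplay effect to the target data in its payload.
; The ability ends when the montage completes, blends out, is interrupted or is cancelled; the event-sending nodes here are unwired.
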(event `self.K2_ActivateAbility`
  (`self.K2_CommitAbility`)
  (`AbilityTask_PlayMontageAndWait.CreatePlayMontageAndWaitProxy` "None" "/Game/Characters/Temp/TempCharacter/Animations/TestingPunch.TestingPunch"
    (:`then`
      (bind (_asynctaskproxy _payload) (`AbilityTask_WaitGameplayEvent.WaitGameplayEvent` (struct :`TagName` "Lightning") null)
        (:`EventReceived`
          (`self.BP_ApplyGameplayEffectToTarget` (`.TargetData` (break `GameplayEventData` _payload)))
          (`KismetSystemLibrary.PrintString` "EffectApply"))))
    (:`OnCompleted`
      (`self.K2_EndAbility` :!label _label))
    (:`OnBlendOut`
      (goto _label))
    (:`OnInterrupted`
      (goto _label))
    (:`OnCancelled`
      (goto _label))))