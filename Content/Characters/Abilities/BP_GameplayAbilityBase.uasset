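; Gameplay Ability Blueprint, named as a base, that spawns a ThirdPersonCharacter at the avatar's transform when activated.
; Activation calls commit without checking its result, spawns the character, draws a temporary red debug line, then ends the ability immediately.
; The line runs from the avatar's location to the sum of that location and its forward vector, with the whole sum scaled up.
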(event `self.K2_ActivateAbility`
  (bind (_owneractor _avataractor) (break `GameplayAbilityActorInfo` (`self.GetActorInfo`)))
  (bind _returnvalue (`Actor.K2_GetActorLocation` _avataractor))
  (`self.K2_CommitAbility`)
  (`|SpawnActorFromClass` "/Game/ThirdPersonCPP/Blueprints/ThirdPersonCharacter.ThirdPersonCharacter_C" (`Actor.GetTransform` _avataractor) "Undefined" "OverrideRootScale" null null)
  (`KismetSystemLibrary.DrawDebugLine` _returnvalue (* (+ _returnvalue (`KismetMathLibrary.GetForwardVector` (`Actor.K2_GetActorRotation` _avataractor))) (`KismetMathLibrary.MakeVector` 10.0 10.0 10.0)) (struct :`R` 0.973958 :`A` 1.0) 5.0 1.0)
  (`self.K2_EndAbility`))