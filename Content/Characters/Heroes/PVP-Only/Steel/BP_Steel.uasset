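; BP_Steel is the character Blueprint for Steel, a PVP-only hero built on the Gameplay Ability System.
; BeginPlay grants Steel's input-tagged abilities plus a test ability that the K key activates.
; An ability-montage event switches rotation between controller yaw and movement direction.
; The B key toggles blended view-target switches between the gameplay camera and a sequence-driven child-actor camera, playing or stopping its sequence.
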(event `self.ReceiveBeginPlay`
  (`self.GrantAbility` "/Game/Characters/Heroes/PVP-Only/Steel/Abilities/Jump/GA_SteelJump.GA_SteelJump_C" 0 0 (struct :`TagName` "Input.Jump"))
  (`self.GrantAbility` "/Game/Characters/Heroes/PVP-Only/Steel/Abilities/Primary/GA_SteelPrimary.GA_SteelPrimary_C" 0 0 (struct :`TagName` "Input.Primary"))
  (`self.GrantAbility` "/Game/Characters/Heroes/PVP-Only/Steel/Abilities/Secondary/GA_SteelSecondary.GA_SteelSecondary_C" 0 0 (struct :`TagName` "Input.Ability.1"))
  (`self.GrantAbility` "/Game/Characters/Heroes/PVP-Only/Steel/Abilities/ShieldPullOut/GA_ShieldMode.GA_ShieldMode_C" 0 0 (struct :`TagName` "Input.Secondary"))
  (`self.GrantAbility` "/Game/Characters/Heroes/PVP-Only/Steel/Abilities/ShieldCharge/GA_CowCatcher.GA_CowCatcher_C" 0 0 (struct :`TagName` "Input.Ability.2"))
  (`self.GrantAbility` "/Game/Characters/Heroes/PVP-Only/Steel/Abilities/GroundSmash/GA_SteelGroundSmash.GA_SteelGroundSmash_C" 0 0 (struct :`TagName` "Input.Ability.5"))
  (`AbilitySystemComponent.K2_GiveAbility` (`self.AbilitySystemComponent`) "/Game/Characters/Heroes/PVP-Only/Revenant/Abilities/TestingAbilityforNotifyError.TestingAbilityforNotifyError_C" 0 1))

(event `self.ReceiveTick`
  (params (DeltaSeconds :type "Float (single-precision)")))

(event `self.SetInAbilityMontage`
  (params (bInMontage :type Boolean))
  (set `self.bUseControllerRotationYaw` bInMontage)
  (set `CharacterMovementComponent.bOrientRotationToMovement` (not bInMontage) (`self.CharacterMovement`)))

(event `Key|B`
  (params (Key :type "Key Structure"))
  (:`Pressed`
    (bind _isa (`/Engine/EditorBlueprintResources/StandardMacros.FlipFlop`)
      (:`A`
        _)
      (:`B`
        _))
    (`self.SetCameraAnimationMode` _isa)))

(event `self.SetCameraAnimationMode`
  (params (bIsInAnimationMode :type Boolean))
  (bind _returnvalue (`GameplayStatics.GetPlayerController` 0))
  (bind _actorsequence (`self.ActorSequence`))
  (if bIsInAnimationMode
    (`PlayerController.SetViewTargetWithBlend` _returnvalue (`ChildActorComponent.ChildActor` (`self.SequenceChild`)) 1.0 "VTBlend_Linear" 0.0 false)
    (`ActorSequenceComponent.PlaySequence` _actorsequence)
    (else
      (`PlayerController.SetViewTargetWithBlend` _returnvalue (`ChildActorComponent.ChildActor` (`self.CameraChild`)) 1.0 "VTBlend_Cubic" 1.0 false)
      (`ActorSequenceComponent.StopSequence` _actorsequence))))

(event `Key|K`
  (params (Key :type "Key Structure"))
  (:`Pressed`
    (`AbilitySystemComponent.TryActivateAbilityByClass` (`self.AbilitySystemComponent`) "/Game/Characters/Heroes/PVP-Only/Revenant/Abilities/TestingAbilityforNotifyError.TestingAbilityforNotifyError_C" true)))

(fn `GetExecuteTargetAnimation`
  (returns (NewParam :type "AnimMontage Object Reference"))
  (return null))

(fn `GetExecutionEffect`
  (returns (NewParam :type "GameplayEffect Class Reference"))
  (return null))

(fn `GetShouldTurnInPlace`
  (returns (ShouldTurnInPlace :type Boolean))
  (return false))

(fn `UserConstructionScript`)