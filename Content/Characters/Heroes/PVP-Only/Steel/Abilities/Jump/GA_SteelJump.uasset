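; Gameplay ability for Steel's charged jump: holding input builds the jump, and release plus a jump event launches it.
; It runs a "Jumping" ability state with a gameplay effect, removed by tag when the state or ability ends.
; Hold time sets the clamped distance, height and duration of a root motion jump force along actor rotation.
; The ability ends on finish, landing or a change to Falling; an unused projectile-arc launch remains.
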(event `self.K2_ActivateAbility`
  (bind (_owneractor _avataractor) (break `GameplayAbilityActorInfo` (`self.GetActorInfo`)))
  (`self.K2_CommitAbility`)
  (`AbilityTask_StartAbilityState.StartAbilityState` "Jumping"
    (:`then`
      (`self.BP_ApplyGameplayEffectToOwner` "/Game/Characters/Heroes/PVP-Only/Steel/Abilities/Jump/GE_SteelJumping.GE_SteelJumping_C")
      (`AbilityTask_WaitMovementModeChange.CreateWaitMovementModeChange` "MOVE_Falling"
        (:`then`
          (bind (_asynctaskproxy _timeheld) (`AbilityTask_WaitInputRelease.WaitInputRelease` true)
            (:`OnRelease`
              (`self.EndAbilityState` "Jumping")
              (`AbilityAsync_WaitGameplayEvent.WaitGameplayEventToActor` _avataractor (struct :`TagName` "Abilities.Steel.Jump") true
                (:`EventReceived`
                  (bind _returnvalue (`KismetMathLibrary.FClamp` (* _timeheld 500.0) 500.0 3000.0))
                  (`AbilityTask_ApplyRootMotionJumpForce.ApplyRootMotionJumpForce` "None" (`Actor.K2_GetActorRotation` _avataractor) _returnvalue _returnvalue (`KismetMathLibrary.FClamp` _timeheld 2.0 3.0) 0.0 true "MaintainLastRootMotionVelocity"
                    (:`then`
                      (`AbilityTask_WaitInputPress.WaitInputPress` false))
                    (:`OnFinish`
                      (`self.K2_EndAbility` :!label _label))
                    (:`OnLanded`
                      (goto _label))))))))
        (:`OnChange`
          (`self.K2_EndAbility`))))
    (:`OnStateEnded`
      (`self.BP_RemoveGameplayEffectFromOwnerWithAssetTags` (struct :`GameplayTags` (struct :`(TagName` "Abilities.Steel.Jump"))) :!label _label_2))
    (:`OnStateInterrupted`
      (goto _label_2))))

(event `self.K2_OnEndAbility`
  (params (bWasCancelled :type Boolean))
  (`KismetSystemLibrary.PrintString` "ENDED \n")
  (`self.BP_RemoveGameplayEffectFromOwnerWithAssetTags` (struct :`GameplayTags` (struct :`(TagName` "Abilities.Steel.Jump")))))