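; BP_Revenant is the character Blueprint for Revenant, a PVP-only hero built on the Gameplay Ability System.
; InitializeAbilities, on authority only, applies the primary ammo effect at max stack count, then grants jump, primary, reload, Obliterate and Mark abilities bound to input tags.
; Ability5 input grants an alternate test primary without an authority check.
; A disconnected copy of the grant chain never runs.
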(event `self.ReceiveBeginPlay`)

(event `self.ReceiveTick`
  (params (DeltaSeconds :type "Float (single-precision)")))

(event `self.InitializeAbilities`
  (bind _abilitysystemcomponent (`self.AbilitySystemComponent`))
  (`/Engine/EditorBlueprintResources/ActorMacros.Switch Has Authority`
    (:`Authority`
      (bind _returnvalue (`AbilitySystemBlueprintLibrary.SetStackCountToMax` (`AbilitySystemComponent.MakeOutgoingSpec` :`self` _abilitysystemcomponent :`GameplayEffectClass` "/Game/Characters/Heroes/PVP-Only/Revenant/Abilities/Primary/GE_PrimaryAmmoCount.GE_PrimaryAmmoCount_C")))
      (`AbilitySystemComponent.BP_ApplyGameplayEffectSpecToSelf` _abilitysystemcomponent _returnvalue)
      (`self.GrantAbility` "/Game/Characters/Heroes/Hephaestus/Abilities/Jump/GA_Jump.GA_Jump_C" 0 0 (struct :`TagName` "Input.Jump"))
      (`self.GrantAbility` "/Game/Characters/Heroes/PVP-Only/Revenant/Abilities/Primary/GA_RevenantPrimaryTagTest.GA_RevenantPrimaryTagTest_C" 0 0 (struct :`TagName` "Input.Primary"))
      (`self.GrantAbility` "/Game/Characters/Heroes/PVP-Only/Revenant/Abilities/Reload/GA_RevenantReload.GA_RevenantReload_C" 0 0 (struct :`TagName` "Input.Secondary"))
      (`self.GrantAbility` "/Game/Characters/Heroes/PVP-Only/Revenant/Abilities/Obliterate/GA_RevenantObliterate.GA_RevenantObliterate_C" 0 0 (struct :`TagName` "Input.Ability.1"))
      (`self.GrantAbility` "/Game/Characters/Heroes/PVP-Only/Revenant/Abilities/Mark/GA_RevenantMark.GA_RevenantMark_C" 0 0 (struct :`TagName` "Input.Ability.2")))))

(event `EnhancedInput|/Game/Player/Input/IA_Ability5`
  (params (ActionValue :type Boolean) (ElapsedSeconds :type "Float (double-precision)") (TriggeredSeconds :type "Float (double-precision)") (InputAction :type "InputAction Object Reference" :default "/Game/Player/Input/IA_Ability5.IA_Ability5"))
  (:`Started`
    (`self.GrantAbility` "/Game/Characters/Heroes/PVP-Only/Revenant/Abilities/Primary/GA_RevenantPrimaryTest.GA_RevenantPrimaryTest_C" 0 0 (struct :`TagName` "Input.Primary"))))

(fn `UserConstructionScript`)