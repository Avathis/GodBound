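; Homing test projectile for the Revenant hero's Mark ability that applies a mark gameplay effect to a single target.
; The construction script points the projectile movement's homing at the root component of a valid Target.
; When the sphere hitbox overlaps that Target, the owner's ability system applies GE_RevenantMark to it and the projectile destroys itself, ignoring all other actors.
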(event `self.ReceiveBeginPlay`
  (add `PrimitiveComponent.OnComponentBeginOverlap` (`self.SphereHitBox`) (`|CreateDelegate` :!event `OnOverlapMark`)))

(event `OnOverlapMark`
  (params (OverlappedComponent :type "PrimitiveComponent Object Reference") (OtherActor :type "Actor Object Reference") (OtherComp :type "PrimitiveComponent Object Reference") (OtherBodyIndex :type Integer) (bFromSweep :type Boolean) (SweepResult :type "HitResult Structure (by ref)"))
  (bind _target (`self.Target`))
  (bind _returnvalue (`AbilitySystemBlueprintLibrary.GetAbilitySystemComponent` (`self.GetOwner`)))
  (if (== OtherActor _target)
    (`AbilitySystemComponent.BP_ApplyGameplayEffectSpecToTarget` _returnvalue (`AbilitySystemComponent.MakeOutgoingSpec` :`self` _returnvalue :`GameplayEffectClass` "/Game/Characters/Heroes/PVP-Only/Revenant/Abilities/Mark/GE_RevenantMark.GE_RevenantMark_C") (`AbilitySystemBlueprintLibrary.GetAbilitySystemComponent` _target))
    (`self.K2_DestroyActor`)))

(fn `UserConstructionScript`
  (bind _target (`self.Target`))
  (`/Engine/EditorBlueprintResources/StandardMacros.IsValid` _target
    (:`Is Valid`
      (set `ProjectileMovementComponent.HomingTargetComponent` (`Actor.RootComponent` _target) (`self.ProjectileMovementComponent`)))))