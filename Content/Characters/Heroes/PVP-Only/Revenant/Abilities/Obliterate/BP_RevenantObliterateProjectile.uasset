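; Homing projectile for Revenant's Obliterate ability that affects only its assigned HomeTarget.
; Construction launches it in a random, upward-biased cone around the initial direction and sets the target's root as the projectile movement's homing component.
; The overlap handler applies GE_RevenantPrimary through the owner's ability system, sends a hit-react gameplay event to the target, then destroys the projectile.
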(event `self.ReceiveBeginPlay`
  (add `PrimitiveComponent.OnComponentBeginOverlap` (`self.Sphere`) (`|CreateDelegate` :!event `OnOverlap`)))

(event `self.ReceiveActorBeginOverlap`
  (params (OtherActor :type "Actor Object Reference")))

(event `OnComponentBeginOverlap_Event`
  (params (OverlappedComponent :type "PrimitiveComponent Object Reference") (OtherActor :type "Actor Object Reference") (OtherComp :type "PrimitiveComponent Object Reference") (OtherBodyIndex :type Integer) (bFromSweep :type Boolean) (SweepResult :type "HitResult Structure (by ref)")))

(event `OnOverlap`
  (params (OverlappedComponent :type "PrimitiveComponent Object Reference") (OtherActor :type "Actor Object Reference") (OtherComp :type "PrimitiveComponent Object Reference") (OtherBodyIndex :type Integer) (bFromSweep :type Boolean) (SweepResult :type "HitResult Structure (by ref)"))
  (bind (_bblockinghit _binitialoverlap _time _distance _location _impactpoint _normal _impactnormal _physmat _hitactor _hitcomponent _hitbonename _bonename _hititem _elementindex _faceindex) (`GameplayStatics.BreakHitResult` SweepResult))
  (bind _hometarget (`self.HomeTarget`))
  (bind _returnvalue (`AbilitySystemBlueprintLibrary.GetAbilitySystemComponent` (`self.GetOwner`)))
  (if (== OtherActor _hometarget)
    (`AbilitySystemComponent.BP_ApplyGameplayEffectSpecToTarget` _returnvalue (`AbilitySystemComponent.MakeOutgoingSpec` :`self` _returnvalue :`GameplayEffectClass` "/Game/Characters/Heroes/PVP-Only/Revenant/Abilities/Primary/GE_RevenantPrimary.GE_RevenantPrimary_C") (`AbilitySystemBlueprintLibrary.GetAbilitySystemComponent` _hometarget))
    (`AbilitySystemBlueprintLibrary.SendGameplayEventToActor` (`self.HomeTarget`) (struct :`TagName` "Abilities.Hit.React") (make `GameplayEventData` (struct) null null null null (struct) (struct) (struct) 0.0 (`AbilitySystemBlueprintLibrary.AbilityTargetDataFromHitResult` (`GameplayStatics.MakeHitResult` _bblockinghit _binitialoverlap _time _distance _location _impactpoint _normal _impactnormal _physmat _hitactor _hitcomponent _hitbonename _bonename _hititem _elementindex _faceindex (`self.K2_GetActorLocation` _hometarget) (`self.K2_GetActorLocation` OtherActor)))))
    (`self.K2_DestroyActor`)))

(fn `SetHomingTarget`
  (params (NewParam :type "Actor Object Reference"))
  (set `ProjectileMovementComponent.HomingTargetComponent` (`Actor.RootComponent` NewParam) (`self.ProjectileMovement`)))

(fn `SetTimer`)

(fn `UserConstructionScript`
  (bind _hometarget (`self.HomeTarget`))
  (bind _projectilemovement (`self.ProjectileMovement`))
  (set `MovementComponent.Velocity` (`KismetMathLibrary.RandomUnitVectorInConeInDegreesFromStream` (`KismetMathLibrary.MakeVector` (.x (`self.InitialDirectionFV`)) (.y (`self.InitialDirectionFV`)) 4.0) 60.0 (`KismetMathLibrary.MakeRandomStream` (`KismetMathLibrary.RandomInteger` 360))) _projectilemovement)
  (`/Engine/EditorBlueprintResources/StandardMacros.IsValid` _hometarget
    (:`Is Valid`
      (set `ProjectileMovementComponent.HomingTargetComponent` (`Actor.RootComponent` _hometarget) _projectilemovement))))