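; Grux hero character Blueprint that grants primary attack, Roar and jump abilities through gameplay tags.
; Two melee trace components on the mesh forward each new hit as an Abilities.Primary.Hit gameplay event to itself.
; Start/end events for both sides drive only MeleeTraceRight with differing flags, and a K key toggle also tests it.
; Ability montages switch rotation from movement-oriented to controller yaw.
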(event `self.ReceiveBeginPlay`
  (bind _mesh (`self.Mesh`))
  (`GB_MeleeTraceComponent.SetupMeleeTrace` (`self.MeleeTraceRight`) _mesh)
  (`GB_MeleeTraceComponent.SetupMeleeTrace` (`self.MeleeTraceLeft`) _mesh))

(event `self.ReceiveTick`
  (params (DeltaSeconds :type "Float (single-precision)")))

(event `self.InitializeAbilities`
  (`self.GrantAbility` "/Game/Characters/Heroes/PVP-Only/Grux/Abilities/Primary/GA_GruxPrimary.GA_GruxPrimary_C" 0 0 (struct :`TagName` "Input.Primary"))
  (`self.GrantAbility` "/Game/Characters/Heroes/PVP-Only/Grux/Abilities/Ultimate/GA_Roar.GA_Roar_C" 0 0 (struct :`TagName` "Input.Secondary"))
  (`self.GrantAbility` "/Game/Characters/Heroes/Hephaestus/Abilities/Jump/GA_Jump.GA_Jump_C" 0 0 (struct :`TagName` "Input.Jump")))

(event `Key|K`
  (params (Key :type "Key Structure"))
  (bind _meleetraceright (`self.MeleeTraceRight`))
  (:`Pressed`
    (`/Engine/EditorBlueprintResources/StandardMacros.FlipFlop`
      (:`A`
        (`GB_MeleeTraceComponent.StartTrace` _meleetraceright false))
      (:`B`
        (`GB_MeleeTraceComponent.EndTrace` _meleetraceright false)))))

(event `self.MeleeTraceRight.OnItemAdded`
  (params (LastItem :type "HitResult Structure"))
  (`AbilitySystemBlueprintLibrary.SendGameplayEventToActor` self (struct :`TagName` "Abilities.Primary.Hit") (make `GameplayEventData` (struct) self null null null (struct) (struct) (struct) 0.0 (`AbilitySystemBlueprintLibrary.AbilityTargetDataFromHitResult` LastItem))))

(event `self.MeleeTraceLeft.OnItemAdded`
  (params (LastItem :type "HitResult Structure"))
  (`AbilitySystemBlueprintLibrary.SendGameplayEventToActor` self (struct :`TagName` "Abilities.Primary.Hit") (make `GameplayEventData` (struct) self null null null (struct) (struct) (struct) 0.0 (`AbilitySystemBlueprintLibrary.AbilityTargetDataFromHitResult` LastItem))))

(event `/Game/Characters/Heroes/BI_AbilitiesGeneral.StartMeleeTraceRight`
  (`GB_MeleeTraceComponent.StartTrace` (`self.MeleeTraceRight`) true))

(event `/Game/Characters/Heroes/BI_AbilitiesGeneral.EndMeleeTraceRight`
  (`GB_MeleeTraceComponent.EndTrace` (`self.MeleeTraceRight`) true))

(event `/Game/Characters/Heroes/BI_AbilitiesGeneral.StartMeleeTraceLeft`
  (`GB_MeleeTraceComponent.StartTrace` (`self.MeleeTraceRight`) false))

(event `/Game/Characters/Heroes/BI_AbilitiesGeneral.EndMeleeTraceLeft`
  (`GB_MeleeTraceComponent.EndTrace` (`self.MeleeTraceRight`) false))

(event `/Game/Characters/Heroes/BI_AbilitiesGeneral.SetInAbilityMontage`
  (params (bInMontage :type Boolean))
  (set `self.bUseControllerRotationYaw` bInMontage)
  (set `CharacterMovementComponent.bOrientRotationToMovement` (not bInMontage) (`self.CharacterMovement`)))

(fn `GetExecuteTargetAnimation`
  (returns (NewParam :type "AnimMontage Object Reference"))
  (return null))

(fn `GetExecutionEffect`
  (returns (NewParam :type "GameplayEffect Class Reference"))
  (return null))

(fn `GetShouldTurnInPlace`
  (returns (ShouldTurnInPlace :type Boolean))
  (return false))

(fn `IsDead`
  (returns (ReturnValue :type Boolean))
  (bind _returnvalue (`parent.IsDead`))
  (return _returnvalue))

(fn `UserConstructionScript`)