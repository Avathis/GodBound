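; Tesla's Alternating Current gameplay ability: a timed channeled beam that damages characters along a line to a confirmed target.
; Cast montages and target data tasks pick the first character, with range extended while OverCharged, then optionally a second near it.
; A looping timer line-traces from Tesla to the first, or between both once linked, applying SetByCaller damage effects and ending when range breaks.
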(event `self.K2_ActivateAbility`
  (bind (_locationtype _literaltransform _sourceactor _sourcecomponent _sourceability _sourcesocketname) (break `GameplayAbilityTargetingLocationInfo` (`self.MakeTargetLocationInfoFromOwnerActor`)))
  (bind (_locationtype_2 _literaltransform_2 _sourceactor_2 _sourcecomponent_2 _sourceability_2 _sourcesocketname_2) (break `GameplayAbilityTargetingLocationInfo` (`self.MakeTargetLocationInfoFromOwnerActor`)))
  (`AbilityTask_PlayMontageAndWait.CreatePlayMontageAndWaitProxy` "None" "/Game/Characters/Heroes/Tesla/Animation/Abilities/Montage_Tesla_ACCastStart.Montage_Tesla_ACCastStart"
    (:`then`
      (bind _returnvalue (`AbilitySystemComponent.GetActiveEffectsWithAllTags` (`self.GetAbilitySystemComponentFromActorInfo`) (struct :`GameplayTags` (struct :`(TagName` "Abilities.Tesla.State.OverCharged")))))
      (if (`KismetArrayLibrary.Array_IsNotEmpty` _returnvalue)
        (set `self.FinalMaxRange` (+ (`self.FinalMaxRange`) (`self.OverchargeRangeAdditive`)))
        (else
          (set `self.FinalMaxRange` (`self.MaxRangeBase`))))
      (bind (_asynctaskproxy _data) (`AbilityTask_WaitTargetData.WaitTargetData` "None" "UserConfirmed" "/Game/Characters/Heroes/Tesla/Abilities/EscapeTheBigEd/GB_TeslaTeleportTrace.GB_TeslaTeleportTrace_C" 50.0 (`self.FinalMaxRange`) (struct :`Name` "PVP_TargetPlayer") true 6 1 true false false (make `GameplayAbilityTargetingLocationInfo` _locationtype _literaltransform _sourceactor _sourcecomponent _sourceability _sourcesocketname) (struct) null (struct) true)
        (:`ValidData`
          (bind _asgb_playable_character (cast `GB_PlayableCharacter` (`.HitActor` (`GameplayStatics.BreakHitResult` (`AbilitySystemBlueprintLibrary.GetHitResultFromTargetData` _data))))
            (:`then`
              (set `self.FirstEnemyCharacter` _asgb_playable_character)
              (`AbilityTask_PlayMontageAndWait.CreatePlayMontageAndWaitProxy` "None" "/Game/Characters/Heroes/Tesla/Animation/Abilities/Montage_Tesla_ACStart.Montage_Tesla_ACStart" 2.0
                (:`OnBlendOut`
                  (`KismetSystemLibrary.K2_SetTimer` null "DealDamagePeriodic" 0.2 true)
                  (`AbilityTask_PlayMontageAndWait.CreatePlayMontageAndWaitProxy` "None" "/Game/Characters/Heroes/Tesla/Animation/Abilities/Montage_Tesla_ACLoop.Montage_Tesla_ACLoop" 0.5
                    (:`then`
                      (bind (_asynctaskproxy_2 _data_2) (`AbilityTask_WaitTargetData.WaitTargetData` "None" "UserConfirmed" "/Game/Characters/Heroes/Tesla/Abilities/EscapeTheBigEd/GB_TeslaTeleportTrace.GB_TeslaTeleportTrace_C" 50.0 (+ (`self.MaxRangeBase`) (`self.MaxRangeDetached`)) (struct :`Name` "PVP_TargetPlayer") true 6 1 false false false (make `GameplayAbilityTargetingLocationInfo` _locationtype_2 _literaltransform_2 _sourceactor_2 _sourcecomponent_2 _sourceability_2 _sourcesocketname_2) (struct) null (struct) true)
                        (:`then`
                          (`AbilityTask_WaitDelay.WaitDelay` 3.0
                            (:`OnFinish`
                              (`self.K2_EndAbility`))))
                        (:`ValidData`
                          (if true
                            (bind _asgb_playable_character_2 (cast `GB_PlayableCharacter` (`.HitActor` (`GameplayStatics.BreakHitResult` (`AbilitySystemBlueprintLibrary.GetHitResultFromTargetData` _data_2))))
                              (:`then`
                                (if (not (> (`KismetMathLibrary.Vector_Distance` (`Actor.K2_GetActorLocation` _asgb_playable_character_2) (`Actor.K2_GetActorLocation` (`self.FirstEnemyCharacter`))) 500.0))
                                  (set `self.SecondEnemyCharacter` _asgb_playable_character_2)))
                              (:`CastFailed`
                                (`self.K2_CancelAbility`)))))))))))
            (:`CastFailed`
              (`self.K2_CancelAbility`))))))
    (:`OnBlendOut`
      (`AbilityTask_PlayMontageAndWait.CreatePlayMontageAndWaitProxy` "None" "/Game/Characters/Heroes/Tesla/Animation/Abilities/Montage_Tesla_ACCast.Montage_Tesla_ACCast"))))

(event `self.K2_OnEndAbility`
  (params (bWasCancelled :type Boolean))
  (set `self.FirstEnemyCharacter` null)
  (set `self.SecondEnemyCharacter` null))

(fn `DealDamagePeriodic`
  (bind _returnvalue (`self.GetAvatarActorFromActorInfo`))
  (bind _returnvalue_2 (`Actor.K2_GetActorLocation` (`self.FirstEnemyCharacter`)))
  (bind _returnvalue_3 (`Actor.K2_GetActorLocation` (`self.SecondEnemyCharacter`)))
  (bind _returnvalue_4 (`Actor.K2_GetActorLocation` _returnvalue))
  (bind _returnvalue_5 (`Actor.K2_GetActorLocation` (`self.FirstEnemyCharacter`)))
  (`/Engine/EditorBlueprintResources/StandardMacros.IsValid` (`self.SecondEnemyCharacter`)
    (:`Is Valid`
      (`KismetSystemLibrary.PrintString` "Second one is valid")
      (if (> (`KismetMathLibrary.Vector_Distance` _returnvalue_2 _returnvalue_3) (`self.MaxRangeDetached`))
        (`self.K2_EndAbility`)
        (else
          (bind _outhits (`KismetSystemLibrary.LineTraceMulti` :`Start` _returnvalue_2 :`End` _returnvalue_3 :`TraceChannel` "TraceTypeQuery1" :`DrawDebugType` "ForDuration"))
          (for _array_element _outhits
            (bind _asgb_playable_character (cast `GB_PlayableCharacter` (`.HitActor` (`GameplayStatics.BreakHitResult` _array_element)))
              (:`then`
                (if (not (`Pawn.IsLocallyControlled` _asgb_playable_character))
                  (bind _returnvalue_6 (`AbilitySystemBlueprintLibrary.AssignTagSetByCallerMagnitude` (`AbilitySystemComponent.MakeOutgoingSpec` :`self` (`self.GetAbilitySystemComponentFromActorInfo`) :`GameplayEffectClass` (`self.DamageEffectClass`)) (struct :`TagName` "Damage") (`self.Damage`)))
                  (`self.K2_ApplyGameplayEffectSpecToTarget` _returnvalue_6 (`AbilitySystemBlueprintLibrary.AbilityTargetDataFromHitResult` _array_element))
                  (`KismetSystemLibrary.PrintString` "Hello")))
              (:`CastFailed`
                (`self.K2_EndAbility`)))))))
    (:`Is Not Valid`
      (if (> (`KismetMathLibrary.Vector_Distance` _returnvalue_5 _returnvalue_4) (`self.FinalMaxRange`))
        (`self.K2_EndAbility`)
        (else
          (bind _outhits_2 (`KismetSystemLibrary.LineTraceMulti` _returnvalue_4 _returnvalue_5 "TraceTypeQuery1" false (`|MakeArray` _returnvalue) "Persistent"))
          (for _array_element_2 _outhits_2
            (bind _returnvalue_7 (`AbilitySystemBlueprintLibrary.AssignTagSetByCallerMagnitude` (`AbilitySystemComponent.MakeOutgoingSpec` :`self` (`self.GetAbilitySystemComponentFromActorInfo`) :`GameplayEffectClass` (`self.DamageEffectClass`)) (struct :`TagName` "Damage") (`self.Damage`)))
            (`self.K2_ApplyGameplayEffectSpecToTarget` _returnvalue_7 (`AbilitySystemBlueprintLibrary.AbilityTargetDataFromHitResult` _array_element_2))))))))