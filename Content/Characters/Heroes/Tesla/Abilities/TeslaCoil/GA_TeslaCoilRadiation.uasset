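; Gameplay ability run by Tesla's deployed coil that deals periodic radiation damage to characters around it.
; On activation it commits and starts a looping timer that scans the actors overlapping the coil's sphere component.
; Each GB_Character other than the coil's Instigator receives a damage effect with a SetByCaller magnitude.
; The spec is made by the coil's ability system component but applied through the Instigator's.
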(event `self.K2_ActivateAbility`
  (`self.K2_CommitAbility`)
  (`KismetSystemLibrary.K2_SetTimerDelegate` (delegate `PeriodicDamage`) 1.0 true))

(event `PeriodicDamage`
  (bind _instigator (`Actor.Instigator` (`self.GetAvatarActorFromActorInfo`)))
  (bind _asbp_tesla_coil (cast `/Game/Characters/Heroes/Tesla/Abilities/TeslaCoil/BP_TeslaCoil` (`self.GetAvatarActorFromActorInfo`)))
  (for _array_element (`PrimitiveComponent.GetOverlappingActors` (`GB_GASActor.SphereComponent` _asbp_tesla_coil) null)
    (if (and (`KismetMathLibrary.ClassIsChildOf` (`GameplayStatics.GetObjectClass` _array_element) "/Script/GodBound.GB_Character") (!= _array_element _instigator))
      (bind _returnvalue (`AbilitySystemBlueprintLibrary.AssignTagSetByCallerMagnitude` (`AbilitySystemComponent.MakeOutgoingSpec` :`self` (`self.GetAbilitySystemComponentFromActorInfo`) :`GameplayEffectClass` (`self.TeslaCoilRadiationDamage`)) (struct :`TagName` "Damage") 50.0))
      (`AbilitySystemComponent.BP_ApplyGameplayEffectSpecToTarget` (`AbilitySystemBlueprintLibrary.GetAbilitySystemComponent` _instigator) _returnvalue (`AbilitySystemBlueprintLibrary.GetAbilitySystemComponent` _array_element)))))