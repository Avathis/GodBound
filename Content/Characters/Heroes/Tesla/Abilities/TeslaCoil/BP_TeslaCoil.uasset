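; BP_TeslaCoil is the coil actor for the Tesla hero's ability, which overcharges its instigator while they overlap it.
; On BeginPlay it applies a radiation gameplay effect to itself through its own AbilitySystemComponent.
; When the instigating Tesla enters, it applies GE_TeslaOvercharged and stores the effect handle, which it uses to remove the effect when Tesla leaves.
; Both overlap events print debug strings.
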(event `self.ReceiveBeginPlay`
  (`AbilitySystemComponent.BP_ApplyGameplayEffectToSelf` :`self` (`self.AbilitySystemComponent`) :`GameplayEffectClass` "/Game/Characters/Heroes/Tesla/Abilities/TeslaCoil/GE_TeslaCoilRatiationEffect.GE_TeslaCoilRatiationEffect_C"))

(event `self.ReceiveActorBeginOverlap`
  (params (OtherActor :type "Actor Object Reference"))
  (if (== OtherActor (`self.GetInstigator`))
    (bind _asbp_tesla (cast `/Game/Characters/Heroes/Tesla/BP_Tesla` OtherActor))
    (set `self.Tesla` _asbp_tesla)
    (bind _returnvalue (`AbilitySystemComponent.BP_ApplyGameplayEffectToTarget` :`self` (`self.AbilitySystemComponent`) :`GameplayEffectClass` "/Game/Characters/Heroes/Tesla/Abilities/GE_TeslaOvercharged.GE_TeslaOvercharged_C" :`Target` (`GB_Character.AbilitySystemComponent` _asbp_tesla)))
    (bind _output_get (set `self.OverchargedGameplayEffect` _returnvalue))
    (`KismetSystemLibrary.PrintString` (`AbilitySystemBlueprintLibrary.GetActiveGameplayEffectDebugString` _output_get))))

(event `self.ReceiveActorEndOverlap`
  (params (OtherActor :type "Actor Object Reference"))
  (bind _tesla (`self.Tesla`))
  (if (== OtherActor _tesla)
    (`AbilitySystemComponent.RemoveActiveGameplayEffect` (`GB_Character.AbilitySystemComponent` _tesla) (`self.OverchargedGameplayEffect`) -1)
    (`KismetSystemLibrary.PrintString` "OverlapEndCoil")))

(fn `UserConstructionScript`)