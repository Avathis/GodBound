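; Gameplay ability that lets the Tesla hero choose a spot and place a Tesla coil there.
; It runs a short-range target actor with custom confirmation, forwarding confirm and cancel input to the ability system component.
; On valid target data it spawns the coil at the hit location with the pawn as instigator and passes it to the avatar.
; The ability ends after that handoff, a failed spawn or cancellation.
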(event `self.K2_ActivateAbility`
  (bind _returnvalue (`self.GetAbilitySystemComponentFromActorInfo`))
  (bind (_locationtype _literaltransform _sourceactor _sourcecomponent _sourceability _sourcesocketname) (break `GameplayAbilityTargetingLocationInfo` (`self.MakeTargetLocationInfoFromOwnerActor`)))
  (bind (_asynctaskproxy _data) (`AbilityTask_WaitTargetData.WaitTargetData` "None" "Custom" "/Game/Characters/Heroes/Tesla/Abilities/TeslaCoil/BP_TeslaCoilTargetActor.BP_TeslaCoilTargetActor_C" 30.0 30.0 200.0 (struct :`Name` "Destructible") true (make `GameplayAbilityTargetingLocationInfo` _locationtype _literaltransform _sourceactor _sourcecomponent _sourceability _sourcesocketname) (struct) null (struct) true)
    (:`then`
      (`AbilityTask_WaitConfirmCancel.WaitConfirmCancel`
        (:`OnConfirm`
          (`AbilitySystemComponent.TargetConfirm` _returnvalue))
        (:`OnCancel`
          (`AbilitySystemComponent.TargetCancel` _returnvalue))))
    (:`ValidData`
      (bind _aspawn (cast `Pawn` (`self.GetAvatarActorFromActorInfo`)))
      (bind (_asynctaskproxy_2 _spawnedactor) (`GameplayTask_SpawnActor.SpawnActor` null (`.Location` (`GameplayStatics.BreakHitResult` (`AbilitySystemBlueprintLibrary.GetHitResultFromTargetData` _data))) (struct) "/Game/Characters/Heroes/Tesla/Abilities/TeslaCoil/BP_TeslaCoil.BP_TeslaCoil_C" false _aspawn)
        (:`Success`
          (bind _asbp_tesla_coil (cast `/Game/Characters/Heroes/Tesla/Abilities/TeslaCoil/BP_TeslaCoil` _spawnedactor))
          (message `/Game/Characters/Heroes/Tesla/BP_TeslaInterface.SetTeslaCoil` (`self.GetAvatarActorFromActorInfo`) _asbp_tesla_coil)
          (`self.K2_EndAbility`))
        (:`DidNotSpawn`
          (`self.K2_EndAbility`))))
    (:`Cancelled`
      (`self.K2_EndAbility`))))