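; Tesla's ElectroMagnet ability, which pulls when the avatar has an OverCharged effect active and pushes otherwise, setting a signed strength and matching montage.
; When the montage blends out, an instant radius target actor gathers actors around Tesla.
; Each one except Tesla receives GE_ElectroMagnet with set-by-caller damage and the strength carried in the effect context.
; Debug spheres are still drawn, and the pull event wait has nothing connected.
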(event `self.K2_ActivateAbility`
  (bind (_locationtype _literaltransform _sourceactor _sourcecomponent _sourceability _sourcesocketname) (break `GameplayAbilityTargetingLocationInfo` (`self.MakeTargetLocationInfoFromOwnerActor`)))
  (`self.K2_CommitAbility`)
  (bind _returnvalue (`AbilitySystemComponent.GetActiveEffectsWithAllTags` (`AbilitySystemBlueprintLibrary.GetAbilitySystemComponent` (`self.GetAvatarActorFromActorInfo`)) (struct :`GameplayTags` (struct :`(TagName` "Abilities.Tesla.State.OverCharged")))))
  (if (`KismetArrayLibrary.Array_IsNotEmpty` _returnvalue)
    (set `self.PushPull` 500.0)
    (`AbilityTask_PlayMontageAndWait.CreatePlayMontageAndWaitProxy` "None" "/Game/Characters/Heroes/Tesla/Animation/Abilities/Montage_Tesla_ElectroMagnetPull.Montage_Tesla_ElectroMagnetPull"
      (:`then`
        (`AbilityAsync_WaitGameplayEvent.WaitGameplayEventToActor` (`self.GetAvatarActorFromActorInfo`) (struct :`TagName` "Abilities.Tesla.EM.Pull") true))
      (:`OnBlendOut`
        (bind (_asynctaskproxy _data) (`AbilityTask_WaitTargetData.WaitTargetData` "None" "Instant" "/Game/Characters/Heroes/Tesla/Abilities/ElectroMagnet/BP_ElectroMagnetTargetActor.BP_ElectroMagnetTargetActor_C" 700.0 (make `GameplayAbilityTargetingLocationInfo` _locationtype _literaltransform _sourceactor _sourcecomponent _sourceability _sourcesocketname) (struct) null (struct) true :!label _label)
          (:`ValidData`
            (`KismetSystemLibrary.DrawDebugSphere` (`Actor.K2_GetActorLocation` (`self.GetAvatarActorFromActorInfo`)) 500.0 12 (struct :`R` 1.0 :`G` 1.0 :`B` 1.0 :`A` 1.0) 5.0)
            (for _array_element (`AbilitySystemBlueprintLibrary.GetActorsFromTargetData` _data)
              (if (!= _array_element (`self.GetAvatarActorFromActorInfo`))
                (bind _returnvalue_2 (`AbilitySystemBlueprintLibrary.AssignTagSetByCallerMagnitude` (`self.MakeOutgoingGameplayEffectSpec` "/Game/Characters/Heroes/Tesla/Abilities/ElectroMagnet/GE_ElectroMagnet.GE_ElectroMagnet_C") (struct :`TagName` "Damage") 50.0))
                (bind _returnvalue_3 (`self.SetContextEffectStrength` (`self.PushPull`) _returnvalue_2))
                (`self.K2_ApplyGameplayEffectSpecToTarget` _returnvalue_3 (`AbilitySystemBlueprintLibrary.AbilityTargetDataFromActor` _array_element))
                (`KismetSystemLibrary.DrawDebugSphere` (`Actor.K2_GetActorLocation` _array_element) 50.0 12 (struct :`R` 1.0 :`G` 1.0 :`B` 1.0 :`A` 1.0) 5.0)))
            (`self.K2_EndAbility`))
          (:`Cancelled`
            (`self.K2_CancelAbility`)))))
    (else
      (set `self.PushPull` -500.0)
      (`AbilityTask_PlayMontageAndWait.CreatePlayMontageAndWaitProxy` "None" "/Game/Characters/Heroes/Tesla/Animation/Abilities/Montage_Tesla_ElectroMagnetPush.Montage_Tesla_ElectroMagnetPush"
        (:`OnBlendOut`
          (goto _label))))))