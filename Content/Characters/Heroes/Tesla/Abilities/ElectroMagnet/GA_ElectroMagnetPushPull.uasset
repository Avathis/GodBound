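; Gameplay ability for Tesla's ElectroMagnet that pushes or pulls its owner relative to the actor that caused the granting effect.
; On activation it reads that effect's strength: negative pushes away, zero or positive pulls in.
; A brief additive radial root motion force, shaped by a strength curve, applies the movement and keeps its final velocity.
; The finish callback only prints a debug string and never ends the ability.
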(event `self.K2_ActivateAbility`
  (`self.K2_CommitAbility`)
  (if (>= (`GB_AbilitySystemLibrary.GetEffectStrength` (`self.GetGrantedByEffectContext`)) 0.0)
    (set `self.bIsPush` false)
    (else
      (set `self.bIsPush` true)))
  (`AbilityTask_ApplyRootMotionRadialForce.ApplyRootMotionRadialForce` "None" (`Actor.K2_GetActorLocation` (`AbilitySystemBlueprintLibrary.EffectContextGetEffectCauser` (`self.GetGrantedByEffectContext`))) null 5000.0 0.1 700.0 (`self.bIsPush`) true false null "/Game/Characters/Heroes/Tesla/Abilities/ElectroMagnet/Curve_ElectroMagnet.Curve_ElectroMagnet" false (struct) "MaintainLastRootMotionVelocity"
    (:`OnFinish`
      (`KismetSystemLibrary.PrintString` "Hello"))))