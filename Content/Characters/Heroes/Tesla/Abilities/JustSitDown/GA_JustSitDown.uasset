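; Tesla's Just Sit Down gameplay ability, which spawns a temporary damage sphere at the effect causer of its granting effect.
; Characters already inside, except the avatar, receive a set-by-caller damage effect.
; Overlap handlers, named for Overclock, apply that same effect to entering actors with an ability system and remove it on exit.
; A short delay ends the ability, destroying the sphere.
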(event `self.K2_ActivateAbility`
  (bind _returnvalue (`AbilitySystemBlueprintLibrary.EffectContextGetEffectCauser` (`self.GetGrantedByEffectContext`)))
  (`/Engine/EditorBlueprintResources/StandardMacros.IsValid` _returnvalue
    (:`Is Valid`
      (`self.K2_CommitAbility`)
      (bind (_asynctaskproxy _spawnedactor) (`GameplayTask_SpawnActor.SpawnActor` null (`Actor.K2_GetActorLocation` _returnvalue) (struct) "/Game/Characters/Heroes/Tesla/Abilities/JustSitDown/BP_JustSitDownSphere.BP_JustSitDownSphere_C" false null)
        (:`Success`
          (bind _output_get (set `self.SpawnedJSDActor` _spawnedactor))
          (bind _output_get_2 (set `self.Overlapping Actors` (`Actor.GetOverlappingActors` _output_get "/Script/GodBound.GB_Character")))
          (`KismetArrayLibrary.Array_RemoveItem` _output_get_2 (`self.GetAvatarActorFromActorInfo`))
          (bind _returnvalue_2 (`AbilitySystemBlueprintLibrary.AssignTagSetByCallerMagnitude` (`AbilitySystemComponent.MakeOutgoingSpec` :`self` (`self.GetAbilitySystemComponentFromActorInfo`) :`GameplayEffectClass` (`self.Damage Effect`)) (struct :`TagName` "Damage") 50.0))
          (`self.K2_ApplyGameplayEffectSpecToTarget` _returnvalue_2 (`AbilitySystemBlueprintLibrary.AbilityTargetDataFromActorArray` (`self.Overlapping Actors`)))
          (add `Actor.OnActorBeginOverlap` _spawnedactor (delegate `ApplyOverclock`))
          (add `Actor.OnActorEndOverlap` _spawnedactor (delegate `RemoveOverclock`))
          (`Actor.SetOwner` _spawnedactor (`self.GetAvatarActorFromActorInfo`))
          (`GameplayTask_WaitDelay.TaskWaitDelay` null 3.0
            (:`OnFinish`
              (`KismetSystemLibrary.PrintString` "Hello")
              (`self.K2_EndAbility`))))))
    (:`Is Not Valid`
      (`self.K2_CancelAbility`))))

(event `self.K2_OnEndAbility`
  (params (bWasCancelled :type Boolean))
  (bind _spawnedjsdactor (`self.SpawnedJSDActor`))
  (`/Engine/EditorBlueprintResources/StandardMacros.IsValid` _spawnedjsdactor
    (:`Is Valid`
      (`Actor.K2_DestroyActor` _spawnedjsdactor)
      (set `self.SpawnedJSDActor` null))))

(event `ApplyOverclock`
  (params (OverlappedActor :type "Actor Object Reference") (OtherActor :type "Actor Object Reference"))
  (bind _returnvalue (`AbilitySystemBlueprintLibrary.GetAbilitySystemComponent` OtherActor))
  (bind _returnvalue_2 (`self.GetAbilitySystemComponentFromActorInfo`))
  (`/Engine/EditorBlueprintResources/StandardMacros.IsValid` _returnvalue
    (:`Is Valid`
      (bind _returnvalue_3 (`AbilitySystemBlueprintLibrary.AssignTagSetByCallerMagnitude` (`AbilitySystemComponent.MakeOutgoingSpec` :`self` _returnvalue_2 :`GameplayEffectClass` (`self.Damage Effect`)) (struct :`TagName` "Damage") 50.0))
      (`AbilitySystemComponent.BP_ApplyGameplayEffectSpecToTarget` _returnvalue_2 _returnvalue_3 _returnvalue)
      (`KismetSystemLibrary.PrintString` "Effect granted"))))

(event `RemoveOverclock`
  (params (OverlappedActor :type "Actor Object Reference") (OtherActor :type "Actor Object Reference"))
  (bind _returnvalue (`AbilitySystemBlueprintLibrary.GetAbilitySystemComponent` OtherActor))
  (`/Engine/EditorBlueprintResources/StandardMacros.IsValid` _returnvalue
    (:`Is Valid`
      (`AbilitySystemComponent.RemoveActiveGameplayEffectBySourceEffect` _returnvalue (`self.Damage Effect`) (`self.GetAbilitySystemComponentFromActorInfo`) -1))))