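; Gameplay ability for Tesla's EscapeTheBigEd, which teleports the hero to a targeted actor.
; It waits for user-confirmed target data from a GB_TeslaTeleportTrace target actor, then moves the avatar to the hit actor's location.
; Camera boom lag speed drops before the jump and is restored through SetCameraLagSmooth to soften the camera movement.
; The ability ends on a successful move or non-blocking hit, but cancellation or a failed move leaves it active.
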(event `self.K2_ActivateAbility`
  (bind (_locationtype _literaltransform _sourceactor _sourcecomponent _sourceability _sourcesocketname) (break `GameplayAbilityTargetingLocationInfo` (`self.MakeTargetLocationInfoFromOwnerActor`)))
  (bind (_asynctaskproxy _data) (`AbilityTask_WaitTargetData.WaitTargetData` "None" "UserConfirmed" "/Game/Characters/Heroes/Tesla/Abilities/EscapeTheBigEd/GB_TeslaTeleportTrace.GB_TeslaTeleportTrace_C" 100.0 3000.0 (struct :`Name` "TraceGASActor") true 1 1 false false false (make `GameplayAbilityTargetingLocationInfo` _locationtype _literaltransform _sourceactor _sourcecomponent _sourceability _sourcesocketname) (struct) null (`AbilitySystemBlueprintLibrary.MakeFilterHandle` (make `GameplayTargetDataFilter` null "TDFS_NoOthers" true) (`AbilitySystemBlueprintLibrary.EffectContextGetInstigatorActor` (`self.GetGrantedByEffectContext`))) true)
    (:`ValidData`
      (`KismetSystemLibrary.PrintString` "Hello")
      (bind (_bblockinghit _binitialoverlap _time _distance _location _impactpoint _normal _impactnormal _physmat _hitactor) (`GameplayStatics.BreakHitResult` (`AbilitySystemBlueprintLibrary.GetHitResultFromTargetData` _data)))
      (if _bblockinghit
        (bind _asbp_tesla (cast `/Game/Characters/Heroes/Tesla/BP_Tesla` (`self.GetAvatarActorFromActorInfo`)))
        (set `SpringArmComponent.CameraLagSpeed` 0.1 (`GB_Character.CameraBoom` _asbp_tesla))
        (bind (_sweephitresult _returnvalue) (`Actor.K2_SetActorLocation` (`self.GetAvatarActorFromActorInfo`) (`Actor.K2_GetActorLocation` _hitactor) false false))
        (if _returnvalue
          (`/Game/Characters/Heroes/Tesla/BP_TeslaInterface.SetCameraLagSmooth` _asbp_tesla 10.0)
          (`self.K2_EndAbility`))
        (else
          (`self.K2_EndAbility`))))
    (:`Cancelled`
      (`KismetSystemLibrary.PrintString` "NotHello"))))