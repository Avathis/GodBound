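; Tesla hero character Blueprint built on the Gameplay Ability System, granting the Place Tesla Coil and Alternating Current abilities on input codes.
; SetTeslaCoil takes ownership of each coil and keeps up to three in rolling slots, destroying the oldest when a fourth arrives.
; SetCameraLagSmooth drives camera boom lag speed through a timeline.
; Tick prints health for debugging, and other debug and attribute-effect nodes are left disconnected.
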(event `Key|H`
  (params (Key :type "Key Structure")))

(event `self.ReceiveBeginPlay`)

(event `self.ReceiveTick`
  (params (DeltaSeconds :type "Float (single-precision)"))
  (`/Engine/EditorBlueprintResources/StandardMacros.IsValid` (`self.AbilitySystemComponent`)
    (:`Is Valid`
      (`KismetSystemLibrary.PrintString` (`KismetStringLibrary.Conv_DoubleToString` (`self.GetHealth`))))))

(event `self.InitializeAbilities`
  (`self.GrantAbility` "/Game/Characters/Heroes/Tesla/Abilities/TeslaCoil/GA_PlaceTeslaCoil.GA_PlaceTeslaCoil_C" 0 7)
  (`self.GrantAbility` "/Game/Characters/Heroes/Tesla/Abilities/AlternatingCurrent/GA_AlternatingCurrent.GA_AlternatingCurrent_C" 0 8))

(event `/Game/Characters/Heroes/Tesla/BP_TeslaInterface.SetTeslaCoil`
  (params (NewParam :type "/Game/Characters/Heroes/Tesla/Abilities/TeslaCoil/BP_TeslaCoil Object Reference"))
  (`self.SetOwner` NewParam self)
  (`/Engine/EditorBlueprintResources/StandardMacros.IsValid` (`self.TeslaCoilJedan`)
    (:`Is Valid`
      (`/Engine/EditorBlueprintResources/StandardMacros.IsValid` (`self.TeslaCoilDve`)
        (:`Is Valid`
          (`/Engine/EditorBlueprintResources/StandardMacros.IsValid` (`self.TeslaCoilTri`)
            (:`Is Valid`
              (`self.K2_DestroyActor` (`self.TeslaCoilJedan`))
              (set `self.TeslaCoilJedan` (`self.TeslaCoilDve`))
              (set `self.TeslaCoilDve` (`self.TeslaCoilTri`))
              (set `self.TeslaCoilTri` NewParam))
            (:`Is Not Valid`
              (set `self.TeslaCoilTri` NewParam))))
        (:`Is Not Valid`
          (set `self.TeslaCoilDve` NewParam))))
    (:`Is Not Valid`
      (set `self.TeslaCoilJedan` NewParam))))

(event `/Game/Characters/Heroes/Tesla/BP_TeslaInterface.SetCameraLagSmooth`
  (params (CameraLag :type "Float (double-precision)"))
  (bind (_direction _adjustcameralag) (`Timeline|AdjustCameraLag` :!via `PlayFromStart`)
    (:`Update`
      (set `SpringArmComponent.CameraLagSpeed` _adjustcameralag (`self.CameraBoom`)))))

(fn `UserConstructionScript`)