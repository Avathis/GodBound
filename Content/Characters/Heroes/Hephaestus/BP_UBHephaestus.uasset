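; Playable Hephaestus hero character that grants its Gameplay Ability System kit and exposes hooks for movement, collision, sprint and health/overheat bar.
; Six arm meshes follow the main mesh pose, with timelines fading their fire-up material opacity unless the ArmsOfAshes tag is active.
; Finishers blend to a cinematic camera, play a sequence and send an Execution.Finished event when it stops.
; Death changes capsule collision and destroys the actor after a State.Dead event.
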(event `self.ReceiveBeginPlay`)

(event `self.ReceiveTick`
  (params (DeltaSeconds :type "Float (single-precision)")))

(event `self.InitializeAbilities`
  (`self.GrantAbility` "/Game/Characters/Heroes/Hephaestus/PVP-ABILITIES/AutoAttack/GA_HephaestusAutoAttack.GA_HephaestusAutoAttack_C" 0 6)
  (`self.GrantAbility` "/Game/Characters/Heroes/Hephaestus/PVP-ABILITIES/Charge/GA_Charge.GA_Charge_C" 0 7)
  (`self.GrantAbility` "/Game/Characters/Heroes/Hephaestus/PVP-ABILITIES/GroundPound/GA_GroundPound.GA_GroundPound_C" 0 9)
  (`self.GrantAbility` "/Game/Characters/Heroes/Hephaestus/PVP-ABILITIES/ArmsOfAshes/GA_ArmsOfAshes.GA_ArmsOfAshes_C" 0 10)
  (`self.GrantAbility` "/Game/Characters/Heroes/Hephaestus/PVP-ABILITIES/Parry/GA_Parry.GA_Parry_C" 0 11)
  (`self.GrantAbility` "/Game/Characters/Heroes/SharedAbilities/GA_Sprint.GA_Sprint_C" 0 3))

(event `/Game/Characters/Heroes/BI_AbilitiesGeneral.SetInAbilityMontage`
  (params (bInMontage :type Boolean))
  (set `self.bUseControllerRotationYaw` bInMontage)
  (set `CharacterMovementComponent.bOrientRotationToMovement` (not bInMontage) (`self.CharacterMovement`)))

(event `self.SetToOverlapPlayer`
  (params (OverlapPlayer :type Boolean))
  (bind _capsulecomponent (`self.CapsuleComponent`))
  (if OverlapPlayer
    (`PrimitiveComponent.SetCollisionResponseToChannel` _capsulecomponent "ECC_GameTraceChannel1" "ECR_Overlap")
    (else
      (`PrimitiveComponent.SetCollisionResponseToChannel` _capsulecomponent "ECC_GameTraceChannel1" "ECR_Block"))))

(event `/Game/Characters/Heroes/BI_AbilitiesGeneral.SetMovementRestricted`
  (params (MovementEnabled :type Boolean))
  (bind _charactermovement (`self.CharacterMovement`))
  (if MovementEnabled
    (`CharacterMovementComponent.SetMovementMode` _charactermovement "MOVE_Walking" 0)
    (`PrimitiveComponent.SetEnableGravity` (`self.CapsuleComponent`) true)
    (else
      (`CharacterMovementComponent.DisableMovement` _charactermovement))))

(event `/Game/Characters/Heroes/BI_AbilitiesGeneral.SetCanManuallyMove`
  (params (CanManuallyMove :type Boolean))
  (set `self.bCanManuallyMove` CanManuallyMove))

(event `self.FireUpArms`
  (params (bShouldFireUp :type Boolean))
  (`self.FireUpLeftArm` bShouldFireUp)
  (`self.FireUpRightArm` bShouldFireUp))

(event `self.FireUpLeftArm`
  (params (bShouldFireUp :type Boolean))
  (if (not (`GameplayTagAssetInterface.HasMatchingGameplayTag` (`self.AbilitySystemComponent`) (struct :`TagName` "Abilities.Hephaestus.F.ArmsOfAshes")))
    (if bShouldFireUp
      (bind (_direction _newtrack_0) (`Timeline|Timeline_0` :!label _label)
        (:`Update`
          (`MeshComponent.SetScalarParameterValueOnMaterials` (`self.LeftArmMIddle`) "Opacity" _newtrack_0)
          (`MeshComponent.SetScalarParameterValueOnMaterials` (`self.LeftArm`) "Opacity" _newtrack_0)
          (`MeshComponent.SetScalarParameterValueOnMaterials` (`self.LeftArmUpper`) "Opacity" _newtrack_0)))
      (else
        (goto _label :!via `ReverseFromEnd`)))))

(event `self.FireUpRightArm`
  (params (bShouldFireUp :type Boolean))
  (if (not (`GameplayTagAssetInterface.HasMatchingGameplayTag` (`self.AbilitySystemComponent`) (struct :`TagName` "Abilities.Hephaestus.F.ArmsOfAshes")))
    (if bShouldFireUp
      (bind (_direction _newtrack_0) (`Timeline|Timeline_1` :!label _label_2)
        (:`Update`
          (`MeshComponent.SetScalarParameterValueOnMaterials` (`self.RightArmUpper`) "Opacity" _newtrack_0)
          (`MeshComponent.SetScalarParameterValueOnMaterials` (`self.RightArmMiddle`) "Opacity" _newtrack_0)
          (`MeshComponent.SetScalarParameterValueOnMaterials` (`self.RightArm`) "Opacity" _newtrack_0)))
      (else
        (goto _label_2 :!via `ReverseFromEnd`)))))

(event `self.ResetCameraPosition`
  (`SceneComponent.ResetRelativeTransform` (`self.Camera`)))

(event `self.PlaySeqeunceTesting`
  (bind _camerasequence (`self.CameraSequence`))
  (bind _playercontroller (`self.PlayerController`))
  (bind _sequenceplayer (`ActorSequenceComponent.SequencePlayer` _camerasequence))
  (`/Engine/EditorBlueprintResources/StandardMacros.IsValid` _playercontroller :!label _label_3
    (:`Is Valid`
      (`PlayerController.SetViewTargetWithBlend` _playercontroller (`ChildActorComponent.ChildActor` (`self.SequenceCameraChild`)) 0.5 "VTBlend_Cubic" 0.0 false)
      (set `self.bCanManuallyLookAround` false)
      (`/Engine/EditorBlueprintResources/StandardMacros.IsValid` _camerasequence
        (:`Is Valid`
          (`MovieSceneSequencePlayer.Play` _sequenceplayer)
          (add `MovieSceneSequencePlayer.OnStop` _sequenceplayer (delegate `OnFinished_Event`))
          (`AbilityAsync_WaitGameplayEvent.WaitGameplayEventToActor` null (struct :`TagName` "Abilities.Execution.Cancelled")
            (:`then`
              (`KismetSystemLibrary.Delay` 3.5))
            (:`EventReceived`
              _))
          (`MovieSceneSequencePlayer.GoToEndAndStop` _sequenceplayer))))))

(event `/Game/Characters/Heroes/BI_AbilitiesGeneral.ExecuteFinisher`
  (goto _label_3))

(event `Key|K`
  (params (Key :type "Key Structure")))

(event `OnStopExecution`)

(event `self.InitializeHealthBarAttributes`
  (bind _uihealthbar (`self.UIHealthBar`))
  (`/Engine/EditorBlueprintResources/StandardMacros.IsValid` _uihealthbar
    (:`Is Valid`
      (bind _returnvalue (`self.GetHealthPercentage`))
      (`GB_HealthWidget.SetHealthPercentage` _uihealthbar _returnvalue)
      (bind _returnvalue_2 (`self.GetOverHeatPercentage`))
      (`KismetSystemLibrary.PrintString` (`KismetStringLibrary.Conv_DoubleToString` _returnvalue_2))
      (`GB_HealthWidget.SetOverHeatPercentage` _uihealthbar _returnvalue_2))))

(event `OnFinished_Event`
  (`PlayerController.SetViewTargetWithBlend` (`self.PlayerController`) (`ChildActorComponent.ChildActor` (`self.CameraChild`)) 0.5 "VTBlend_Cubic" 0.0 false)
  (set `self.bCanManuallyLookAround` true)
  (`AbilitySystemBlueprintLibrary.SendGameplayEventToActor` self (struct :`TagName` "Abilities.Execution.Finished")))

(event `/Game/Characters/Heroes/BI_AbilitiesGeneral.StartSprint`
  (params (bShouldSprint :type Boolean))
  (bind _charactermovementcomponent (`self.CharacterMovementComponent`))
  (if bShouldSprint
    (`GB_CharacterMovementComponent.StartSprinting` _charactermovementcomponent)
    (else
      (`GB_CharacterMovementComponent.StopSprinting` _charactermovementcomponent))))

(event `self.ShowHealthBar`
  (set `Widget.Visibility` "Visible" (`WidgetComponent.GetWidget` (`self.UIHealthBarComponent`)))
  (`KismetSystemLibrary.K2_SetTimerDelegate` (delegate `HideHealthBar`) 5.0))

(event `HideHealthBar`
  (set `Widget.Visibility` "Hidden" (`WidgetComponent.GetWidget` (`self.UIHealthBarComponent`))))

(event `/Game/Characters/Heroes/BI_AbilitiesGeneral.GetUp`)

(event `/Game/Characters/Heroes/BI_AbilitiesGeneral.TurnToTarget`
  (params (ActorToTurnTo :type "Actor Object Reference"))
  (bind (_returnvalue_roll _returnvalue_pitch _returnvalue_yaw) (`KismetMathLibrary.BreakRotator` (`self.K2_GetActorRotation`)))
  (bind (_returnvalue_roll_2 _returnvalue_pitch_2 _returnvalue_yaw_2) (`KismetMathLibrary.BreakRotator` (`KismetMathLibrary.FindLookAtRotation` (`self.K2_GetActorLocation`) (`self.K2_GetActorLocation` ActorToTurnTo))))
  (`Timeline|Timeline` :!via `PlayFromStart`
    (:`Update`
      (`self.K2_SetActorRotation` (`KismetMathLibrary.MakeRotator` _returnvalue_roll _returnvalue_pitch (`KismetMathLibrary.FInterpTo` _returnvalue_yaw _returnvalue_yaw_2 (`GameplayStatics.GetWorldDeltaSeconds`) 5.0))))))

(event `/Game/Characters/Heroes/BI_AbilitiesGeneral.SwitchToCinematicCamera`
  (params (bToCinematic :type Boolean))
  (bind _playercontroller (`self.PlayerController`))
  (if bToCinematic
    (`/Engine/EditorBlueprintResources/StandardMacros.IsValid` _playercontroller
      (:`Is Valid`
        (`PlayerController.SetViewTargetWithBlend` _playercontroller (`ChildActorComponent.ChildActor` (`self.SequenceCameraChild`)) 0.5 "VTBlend_Cubic" 0.0 false)))
    (else
      (`/Engine/EditorBlueprintResources/StandardMacros.IsValid` _playercontroller
        (:`Is Valid`
          (`PlayerController.SetViewTargetWithBlend` _playercontroller (`ChildActorComponent.ChildActor` (`self.CameraChild`)) 0.5 "VTBlend_Cubic" 0.0 false))))))

(event `PlayMontageOnAll`
  (params (AnimMontage :type "AnimMontage Object Reference"))
  (`self.Die`)
  (`|PlayMontage` (`self.Mesh`) (`self.ExecutionTargetAnimation`)))

(event `/Game/Characters/Heroes/BI_AbilitiesGeneral.PlayMontageMC`
  (params (MontageToPlay :type "AnimMontage Object Reference"))
  (`self.PlayMontageOnAll` MontageToPlay))

(event `self.Die`
  (`PrimitiveComponent.SetCollisionObjectType` (`self.CapsuleComponent`) "ECC_Pawn")
  (`PrimitiveComponent.SetCollisionResponseToChannel` (`self.CapsuleComponent`) "ECC_GameTraceChannel1" "ECR_Ignore")
  (`AbilityAsync_WaitGameplayEvent.WaitGameplayEventToActor` null (struct :`TagName` "State.Dead")
    (:`EventReceived`
      (`KismetSystemLibrary.Delay` 3.0)
      (`self.K2_DestroyActor` self))))

(fn `GetExecuteTargetAnimation`
  (returns (NewParam :type "AnimMontage Object Reference"))
  (bind _executiontargetanimation (`self.ExecutionTargetAnimation`))
  (`/Engine/EditorBlueprintResources/StandardMacros.IsValid` _executiontargetanimation
    (:`Is Valid`
      (`KismetSystemLibrary.PrintString` "ANIMATION REALLY VALID"))
    (:`Is Not Valid`
      (`KismetSystemLibrary.PrintString` "Animation Not valid in the first place")))
  (return _executiontargetanimation))

(fn `GetExecutionEffect`
  (returns (NewParam :type "GameplayEffect Class Reference"))
  (return (`self.ExecutionEffect`)))

(fn `UserConstructionScript`
  (`SkinnedMeshComponent.SetLeaderPoseComponent` (`self.RightArm`) (`self.Mesh`) false false)
  (`SkinnedMeshComponent.SetLeaderPoseComponent` (`self.LeftArm`) (`self.Mesh`) false false)
  (`SkinnedMeshComponent.SetLeaderPoseComponent` (`self.LeftArmMIddle`) (`self.Mesh`) false false)
  (`SkinnedMeshComponent.SetLeaderPoseComponent` (`self.RightArmMiddle`) (`self.Mesh`) false false)
  (`SkinnedMeshComponent.SetLeaderPoseComponent` (`self.LeftArmUpper`) (`self.Mesh`) false false)
  (`SkinnedMeshComponent.SetLeaderPoseComponent` (`self.RightArmUpper`) (`self.Mesh`) false false))