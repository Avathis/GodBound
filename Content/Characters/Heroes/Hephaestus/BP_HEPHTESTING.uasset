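; BP_HEPHTESTING is a test Blueprint of the Hephaestus hero that switches GAS ability sets by combat mode.
; ChangeCombatSet unequips the current set, grants the one mapped to the new mode and triggers OverHeatActivate for mode F.
; Interface events forward combat entry and exit, while speed events adjust the advanced movement component's MaxWalkSpeed.
; ChangeMovementType is empty; manual ability grants and movement-state gameplay effect logic remain disconnected.
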(event `self.ReceiveBeginPlay`)

(event `self.ReceiveActorBeginOverlap`
  (params (OtherActor :type "Actor Object Reference")))

(event `self.ReceiveTick`
  (params (DeltaSeconds :type "Float (single-precision)")))

(event `/Game/Interfaces/BPI_MovementInterface.Change Movement Type`
  (params (NewMovmentType :type "EMovementState Enum" :default "EMS_Idle")))

(event `/Game/Interfaces/BPI_AbilityInterface.ChangeCombatSet`
  (params (NewParam :type "EHephaestusSet Enum" :default "EHS_OOC"))
  (`self.UnequipAbilitySet` (`self.CurrentAbilitySet`))
  (bind _output_get (set `self.CombatSet` NewParam))
  (bind _returnvalue (`self.ChangeAbilitySet` (`self.AbilitySystemComponent`) (`BlueprintMapLibrary.Map_Find` (`self.AbilitySetsInMode`) _output_get) self (`self.CurrentAbilitySet`)))
  (set `self.CurrentAbilitySet` _returnvalue)
  (switch `EHephaestusSet` _output_get
    (:`EHS_F`
      (`self.OverHeatActivate`))))

(event `/Game/Interfaces/BPI_AbilityInterface.ExitCombatI`
  (`self.ExitCombat`))

(event `/Game/Interfaces/BPI_AbilityInterface.EnterCombatI`
  (`self.EnterCombat`))

(event `/Game/Interfaces/BPI_AbilityInterface.AddSpeed`
  (params (AddedSpeed :type "Float (double-precision)"))
  (bind _returnvalue (`self.GetAdvMovementComponent`))
  (`/Game/Interfaces/BPI_MovementInterface.Change Movemnt Speed` (+ (`CharacterMovementComponent.MaxWalkSpeed` _returnvalue) AddedSpeed)))

(event `/Game/Interfaces/BPI_MovementInterface.Change Movemnt Speed`
  (params (NewMovementSpeed :type "Float (double-precision)"))
  (bind _returnvalue (`self.GetAdvMovementComponent`))
  (set `CharacterMovementComponent.MaxWalkSpeed` NewMovementSpeed _returnvalue))

(fn `GetCombatMode`
  (returns (NewParam :type "EHephaestusSet Enum"))
  (return (`self.CombatSet`)))

(fn `UserConstructionScript`)