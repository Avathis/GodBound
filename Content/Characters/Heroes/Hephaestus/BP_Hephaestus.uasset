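; Hephaestus hero character Blueprint that grants sprint, jump and fireball abilities through the Gameplay Ability System and starts out of combat.
; Combat set changes enter or exit combat, apply the matching gameplay effect and reset movement to walking.
; Movement changes apply walk or run effects per combat set.
; Speed helpers include a timeline ramp that stops outside charge sprint, while ability-sprint events switch rotation to follow movement and back.
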(event `self.ReceiveBeginPlay`
  (bind _abilitysystemcomponent (`self.AbilitySystemComponent`))
  (`self.GrantAbility` "/Game/Characters/Heroes/SharedAbilities/GA_Sprint.GA_Sprint_C" 1 3)
  (`self.GrantAbility` "/Game/Characters/Heroes/Hephaestus/Abilities/Jump/GA_Heph_Jump.GA_Heph_Jump_C" 0 4)
  (`self.GrantAbility` "/Game/Characters/Heroes/Hephaestus/Abilities/FireBall/GA_FireBall.GA_FireBall_C" 0 7)
  (`AbilitySystemComponent.BP_ApplyGameplayEffectToSelf` :`self` _abilitysystemcomponent :`GameplayEffectClass` "/Game/Characters/Heroes/Hephaestus/Abilities/EnterExitCombat/GE_OutOfCombat.GE_OutOfCombat_C")
  (`AbilitySystemComponent.BP_ApplyGameplayEffectToSelf` :`self` _abilitysystemcomponent :`GameplayEffectClass` "/Game/Effects/GE_M_Walk.GE_M_Walk_C"))

(event `self.ReceiveTick`
  (params (DeltaSeconds :type "Float (single-precision)")))

(event `self.Change Movement Type`
  (params (NewMovmentType :type "EMovementState Enum" :default "EMS_Idle"))
  (bind _abilitysystemcomponent (`self.AbilitySystemComponent`))
  (bind _combatset (`self.CombatSet`))
  (if (`|EnumInequality` NewMovmentType "EMS_Idle")
    (bind _returnvalue (`self.GetAdvMovementComponent`))
    (`GB_CharacterMovementComponent.ChangeMovementState` _returnvalue NewMovmentType)
    (else
      (bind _returnvalue_2 (`self.GetAdvMovementComponent`))
      (`GB_CharacterMovementComponent.ChangeMovementState` _returnvalue_2 (`GB_CharacterMovementComponent.MovementType` _returnvalue_2))))
  (bind _returnvalue_3 (`self.GetAdvMovementComponent`))
  (switch `EMovementState` (`GB_CharacterMovementComponent.MovementType` _returnvalue_3)
    (:`EMS_Walking`
      (switch `EHephaestusSet` _combatset
        (:`EHS_OOC`
          (`AbilitySystemComponent.BP_ApplyGameplayEffectToSelf` :`self` _abilitysystemcomponent :`GameplayEffectClass` "/Game/Effects/GE_OOC_Walk.GE_OOC_Walk_C"))
        (:`EHS_M`
          (`AbilitySystemComponent.BP_ApplyGameplayEffectToSelf` :`self` _abilitysystemcomponent :`GameplayEffectClass` "/Game/Effects/GE_M_Walk.GE_M_Walk_C"))))
    (:`EMS_Sprinting`
      (switch `EHephaestusSet` _combatset
        (:`EHS_OOC`
          (`AbilitySystemComponent.BP_ApplyGameplayEffectToSelf` :`self` _abilitysystemcomponent :`GameplayEffectClass` "/Game/Effects/GE_OOC_Run.GE_OOC_Run_C"))
        (:`EHS_M`
          (`AbilitySystemComponent.BP_ApplyGameplayEffectToSelf` :`self` _abilitysystemcomponent :`GameplayEffectClass` "/Game/Effects/GE_M_Run.GE_M_Run_C"))))))

(event `/Game/Interfaces/BPI_AbilityInterface.ChangeCombatSet`
  (params (NewParam :type "EHephaestusSet Enum" :default "EHS_OOC"))
  (bind _abilitysystemcomponent (`self.AbilitySystemComponent`))
  (bind _output_get (set `self.CombatSet` NewParam))
  (switch `EHephaestusSet` _output_get
    (:`EHS_OOC`
      (`/Game/Interfaces/BPI_AbilityInterface.ExitCombatI`)
      (`AbilitySystemComponent.BP_ApplyGameplayEffectToSelf` :`self` _abilitysystemcomponent :`GameplayEffectClass` "/Game/Characters/Heroes/Hephaestus/Abilities/EnterExitCombat/GE_OutOfCombat.GE_OutOfCombat_C"))
    (:`EHS_M`
      (`self.EnterCombat`)
      (`AbilitySystemComponent.BP_ApplyGameplayEffectToSelf` :`self` _abilitysystemcomponent :`GameplayEffectClass` "/Game/Characters/Heroes/Hephaestus/Abilities/EnterExitCombat/GE_IC_M.GE_IC_M_C")))
  (`self.Change Movement Type` "EMS_Walking"))

(event `/Game/Interfaces/BPI_AbilityInterface.ExitCombatI`
  (`self.ExitCombat`))

(event `/Game/Interfaces/BPI_AbilityInterface.EnterCombatI`
  (`self.EnterCombat`))

(event `/Game/Interfaces/BPI_AbilityInterface.AddSpeed`
  (params (AddedSpeed :type "Float (double-precision)"))
  (bind _returnvalue (`self.GetAdvMovementComponent`))
  (`self.Change Movemnt Speed` (+ (`CharacterMovementComponent.MaxWalkSpeed` _returnvalue) AddedSpeed)))

(event `/Game/Interfaces/BPI_AbilityInterface.GraduallyAddSpeed`
  (params (NewMaxSpeed :type "Float (double-precision)"))
  (bind (_direction _movespeed) (`Timeline|ChargedSpeedTL` :!via `PlayFromStart` :!label _label)
    (:`Update`
      (bind _returnvalue (`self.GetAdvMovementComponent`))
      (bind _returnvalue_2 (`GB_CharacterMovementComponent.GetMovementType` _returnvalue))
      (if (`|EnumInequality` _returnvalue_2 "EMS_HephaestusChargeSprint")
        (goto _label :!via `Stop`)
        (else
          (set `CharacterMovementComponent.MaxWalkSpeed` (`KismetMathLibrary.Lerp` (`CharacterMovementComponent.MaxWalkSpeed` _returnvalue) NewMaxSpeed (`KismetMathLibrary.SafeDivide` _movespeed 30.0)) _returnvalue))))))

(event `self.Change Movemnt Speed`
  (params (NewMovementSpeed :type "Float (double-precision)"))
  (bind _returnvalue (`self.GetAdvMovementComponent`))
  (set `CharacterMovementComponent.MaxWalkSpeed` NewMovementSpeed _returnvalue))

(event `/Game/Interfaces/BPI_AbilityInterface.Start Ability Sprint`
  (bind _returnvalue (`self.GetAdvMovementComponent`))
  (`Controller.SetIgnoreLookInput` (`self.GetController`) false)
  (set `self.bUseControllerRotationYaw` false)
  (set `CharacterMovementComponent.bOrientRotationToMovement` true _returnvalue)
  (`self.Change Movemnt Speed` (* (`CharacterMovementComponent.MaxWalkSpeed` _returnvalue) 0.77)))

(event `/Game/Interfaces/BPI_AbilityInterface.EndAbilitySprint`
  (bind _returnvalue (`self.GetAdvMovementComponent`))
  (set `self.bUseControllerRotationYaw` true)
  (set `CharacterMovementComponent.bOrientRotationToMovement` false _returnvalue))

(event `/Game/Interfaces/BPI_AbilityInterface.OverlapInAbilitySprint`
  (bind _returnvalue (`self.GetAdvMovementComponent`))
  (`KismetSystemLibrary.PrintString` (`KismetStringLibrary.Conv_DoubleToString` (`CharacterMovementComponent.MaxWalkSpeed` _returnvalue)))
  (`KismetSystemLibrary.PrintString` (`KismetStringLibrary.Conv_DoubleToString` (`KismetMathLibrary.VSize` (`MovementComponent.Velocity` _returnvalue)))))

(fn `UserConstructionScript`)