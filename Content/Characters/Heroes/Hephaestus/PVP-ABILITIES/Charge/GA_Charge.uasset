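; Gameplay ability for Hephaestus's PvP Charge, a short forward rush that damages actors it hits.
; An instant melee target trace must find an actor before the ability commits, plays the montage and attaches an overlap hitbox to the avatar.
; A montage gameplay event triggers root-motion movement to the trace end at current height, with player overlap enabled.
; Hitbox overlaps apply SetByCaller damage, and ending the ability destroys the hitbox and restores movement.
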(event `self.K2_ActivateAbility`
  (bind _returnvalue (`self.GetAvatarActorFromActorInfo`))
  (bind _returnvalue_2 (`self.GetAvatarActorFromActorInfo`))
  (bind (_locationtype _literaltransform _sourceactor _sourcecomponent _sourceability _sourcesocketname) (break `GameplayAbilityTargetingLocationInfo` (`self.MakeTargetLocationInfoFromOwnerActor`)))
  (`KismetSystemLibrary.PrintString` "HelloCharge")
  (bind (_asynctaskproxy _data) (`AbilityTask_WaitTargetData.WaitTargetData` "None" "Instant" "/Game/Characters/Heroes/Hephaestus/PVP-ABILITIES/AutoAttack/BP_Hephaestus_MeleeTA.BP_Hephaestus_MeleeTA_C" 100.0 600.0 (struct :`Name` "PVP_TargetPlayer") true 1 1 false false false (make `GameplayAbilityTargetingLocationInfo` _locationtype _literaltransform _sourceactor _sourcecomponent _sourceability _sourcesocketname) (struct) null (struct) true)
    (:`ValidData`
      (if (`AbilitySystemBlueprintLibrary.TargetDataHasActor` _data)
        (`self.K2_CommitAbility`)
        (`AbilityTask_PlayMontageAndWait.CreatePlayMontageAndWaitProxy` "None" "/Game/Characters/Heroes/Hephaestus/PVP-ABILITIES/Charge/Hephaestus_Charge.Hephaestus_Charge"
          (:`then`
            (`AbilityAsync_WaitGameplayEvent.WaitGameplayEventToActor` _returnvalue_2 (struct :`TagName` "Abilities.Hephaestus.F.Charge") true
              (:`then`
                (bind (_asynctaskproxy_2 _spawnedactor) (`GameplayTask_SpawnActor.SpawnActor` null (`Actor.K2_GetActorLocation` _returnvalue) (struct) "/Game/Characters/Heroes/Hephaestus/PVP-ABILITIES/Charge/BP_ChargeHitBox.BP_ChargeHitBox_C" false (cast `Pawn` _returnvalue :!pure true))
                  (:`Success`
                    (set `self.Hitbox` _spawnedactor)
                    (add `Actor.OnActorBeginOverlap` _spawnedactor (delegate `ChargeOverlap`))
                    (`Actor.K2_AttachToActor` _spawnedactor _returnvalue_2 "None" "SnapToTarget" "SnapToTarget" "SnapToTarget" true))))
              (:`EventReceived`
                (message `/Game/Characters/Heroes/Hephaestus/BI_UBHephaestusInterface.SetToOverlapPlayer` (`self.GetAvatarActorFromActorInfo`) true)
                (bind (_x _y) (`KismetMathLibrary.BreakVector3f` (`.TraceEnd` (`GameplayStatics.BreakHitResult` (`AbilitySystemBlueprintLibrary.GetHitResultFromTargetData` _data)))))
                (`AbilityTask_ApplyRootMotionMoveToForce.ApplyRootMotionMoveToForce` "None" (`KismetMathLibrary.MakeVector` _x _y (`.Z` (`KismetMathLibrary.BreakVector3f` (`Actor.K2_GetActorLocation` (`self.GetAvatarActorFromActorInfo`))))) 0.2 false "MOVE_Walking" false null "SetVelocity"
                  (:`OnTimedOut`
                    _)
                  (:`OnTimedOutAndDestinationReached`
                    _))
                (message `/Game/Characters/Heroes/Hephaestus/BI_UBHephaestusInterface.SetToOverlapPlayer` (`self.GetAvatarActorFromActorInfo`) false))))
          (:`OnCompleted`
            (`self.K2_EndAbility` :!label _label))
          (:`OnBlendOut`
            (goto _label))
          (:`OnInterrupted`
            (goto _label))
          (:`OnCancelled`
            (goto _label)))
        (else
          (`self.K2_CancelAbility`))))))

(event `self.K2_OnEndAbility`
  (params (bWasCancelled :type Boolean))
  (bind _returnvalue (`self.GetAvatarActorFromActorInfo`))
  (bind _hitbox (`self.Hitbox`))
  (`/Engine/EditorBlueprintResources/StandardMacros.IsValid` _hitbox
    (:`Is Valid`
      (`Actor.K2_DestroyActor` _hitbox))
    (:`Is Not Valid`
      _))
  (message `/Game/Characters/Heroes/Hephaestus/BI_UBHephaestusInterface.SetToOverlapPlayer` _returnvalue false)
  (message `/Game/Characters/Heroes/BI_AbilitiesGeneral.SetCanManuallyMove` _returnvalue true))

(event `ChargeOverlap`
  (params (OverlappedActor :type "Actor Object Reference") (OtherActor :type "Actor Object Reference"))
  (if (not (== OtherActor (`self.GetAvatarActorFromActorInfo`)))
    (bind _returnvalue (`AbilitySystemBlueprintLibrary.AssignTagSetByCallerMagnitude` (`self.MakeOutgoingGameplayEffectSpec` (`self.ChargeDamageEffect`) (`KismetMathLibrary.Conv_IntToDouble` (`self.GetAbilityLevel`))) (struct :`TagName` "Damage") 50.0))
    (`self.K2_ApplyGameplayEffectSpecToTarget` _returnvalue (`AbilitySystemBlueprintLibrary.AbilityTargetDataFromActor` OtherActor))
    (`KismetSystemLibrary.PrintString` (`KismetSystemLibrary.GetObjectName` OtherActor))))