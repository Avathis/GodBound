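; Hephaestus's hold-to-charge dash Gameplay Ability, which locks manual movement while charging.
; Releasing input, or reaching the hold time cap, attaches a BP_ChargeHitBox and launches him forward with root motion, scaling distance by hold time.
; An overlap or the end of the move leads to Hit, a sphere overlap ahead applying hold-scaled damage with a linked knockback effect.
; Ending the ability restores movement and cleans up the hitbox.
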(event `self.K2_ActivateAbility`
  (bind _returnvalue (`self.GetAvatarActorFromActorInfo`))
  (bind _returnvalue_2 (`self.GetAvatarActorFromActorInfo`))
  (bind _async_input_task (`self.Async Input Task`))
  (bind (_owneractor _avataractor _playercontroller) (break `GameplayAbilityActorInfo` (`self.GetActorInfo`)))
  (message `/Game/Characters/Heroes/BI_AbilitiesGeneral.SetCanManuallyMove` (`self.GetAvatarActorFromActorInfo`) false)
  (message `/Game/Characters/Heroes/BI_AbilitiesGeneral.SetShouldTurnInPlace` (`self.GetAvatarActorFromActorInfo`) true)
  (`self.K2_CommitAbility`)
  (bind _returnvalue_3 (`self.BP_ApplyGameplayEffectToOwner` "/Game/Characters/Heroes/Hephaestus/PVP-ABILITIES/Charge/Experimental/GE_HoldingCharge.GE_HoldingCharge_C"))
  (set `self.HoldingGE` _returnvalue_3)
  (bind _asynctaskproxy (`GameplayTask_WaitDelay.TaskWaitDelay` null 2.0)
    (:`then`
      (set `self.Async Wait Task` _asynctaskproxy)
      (bind (_asynctaskproxy_2 _timeheld) (`AbilityTask_WaitInputRelease.WaitInputRelease` true)
        (:`then`
          (set `self.Async Input Task` _asynctaskproxy_2)
          (`AbilityTask_PlayMontageAndWait.CreatePlayMontageAndWaitProxy` "None" "/Game/Characters/SharedAnimations/MeleeAnimations/FighterAnimations/Attacks/Heph_Charge_Start.Heph_Charge_Start" 0.9 "Default"))
        (:`OnRelease`
          (set `self.InputHeldTime` _timeheld)
          (`GameplayTask.EndTask` (`self.Async Wait Task`))
          (bind (_asynctaskproxy_3 _spawnedactor) (`GameplayTask_SpawnActor.SpawnActor` null (`Actor.K2_GetActorLocation` _returnvalue_2) (`Actor.K2_GetActorRotation` _returnvalue_2) "/Game/Characters/Heroes/Hephaestus/PVP-ABILITIES/Charge/BP_ChargeHitBox.BP_ChargeHitBox_C" false null :!label _label)
            (:`then`
              (`self.BP_RemoveGameplayEffectFromOwnerWithHandle` (`self.HoldingGE`))
              (`PlayerController.ClientStopCameraShake` _playercontroller "/Game/Characters/Heroes/Hephaestus/PVP-ABILITIES/Charge/Experimental/CS_HoldingCharge.CS_HoldingCharge_C" false)
              (`PlayerController.ClientStopCameraShake` _playercontroller "/Game/Characters/Heroes/Hephaestus/PVP-ABILITIES/Charge/Experimental/CS_ChargeCamera.CS_ChargeCamera_C" false))
            (:`Success`
              (set `self.HitBox` _spawnedactor)
              (add `Actor.OnActorBeginOverlap` _spawnedactor (delegate `OnHitBoxOverlap`))
              (`Actor.K2_AttachToActor` _spawnedactor (`self.GetAvatarActorFromActorInfo`) "None" "SnapToTarget" "SnapToTarget" "KeepWorld" true)
              (`AbilityTask_PlayMontageAndWait.CreatePlayMontageAndWaitProxy` "None" "/Game/Characters/SharedAnimations/MeleeAnimations/FighterAnimations/Attacks/Heph_Charge_Loop.Heph_Charge_Loop" 1.0 "Launch"
                (:`then`
                  (bind _asynctaskproxy_4 (`AbilityTask_ApplyRootMotionMoveToForce.ApplyRootMotionMoveToForce` "None" (+ (* (`Actor.GetActorForwardVector` _returnvalue) (`KismetMathLibrary.Conv_DoubleToVector` (`KismetMathLibrary.FMax` (* (`self.InputHeldTime`) 1000.0) 600.0))) (`Actor.K2_GetActorLocation` _returnvalue)) 0.3 false "MOVE_None" false null "SetVelocity")
                    (:`then`
                      (set `self.Async RootMotion Task` _asynctaskproxy_4)
                      (`AbilityTask_WaitOverlap.WaitForOverlap`
                        (:`OnOverlap`
                          (`AbilityTask_PlayMontageAndWait.CreatePlayMontageAndWaitProxy` "None" "/Game/Characters/SharedAnimations/MeleeAnimations/FighterAnimations/Attacks/Heph_Charge_End.Heph_Charge_End" 1.0 "Hit" false
                            (:`then`
                              (`self.Hit` (`self.InputHeldTime`)))))))
                    (:`OnTimedOut`
                      (`AbilityTask_PlayMontageAndWait.CreatePlayMontageAndWaitProxy` "None" "/Game/Characters/SharedAnimations/MeleeAnimations/FighterAnimations/Attacks/Heph_Charge_End.Heph_Charge_End" 1.0 "Hit" false :!label _label_2
                        (:`then`
                          (`self.Hit` (`self.InputHeldTime`)))))
                    (:`OnTimedOutAndDestinationReached`
                      (goto _label_2))))))
            (:`DidNotSpawn`
              (`self.K2_CancelAbility`))))))
    (:`OnFinish`
      (`/Engine/EditorBlueprintResources/StandardMacros.IsValid` _async_input_task
        (:`Is Valid`
          (`GameplayTask.EndTask` _async_input_task))
        (:`Is Not Valid`
          _))
      (set `self.InputHeldTime` 2.0)
      (goto _label))))

(event `self.K2_OnEndAbility`
  (params (bWasCancelled :type Boolean))
  (bind _hitbox (`self.HitBox`))
  (bind (_owneractor _avataractor _playercontroller) (break `GameplayAbilityActorInfo` (`self.GetActorInfo`)))
  (message `/Game/Characters/Heroes/BI_AbilitiesGeneral.SetCanManuallyMove` (`self.GetAvatarActorFromActorInfo`) true)
  (message `/Game/Characters/Heroes/BI_AbilitiesGeneral.SetShouldTurnInPlace` (`self.GetAvatarActorFromActorInfo`) false)
  (`/Engine/EditorBlueprintResources/StandardMacros.IsValid` _hitbox
    (:`Is Valid`
      (`Actor.K2_DestroyActor` _hitbox)
      (`self.BP_RemoveGameplayEffectFromOwnerWithHandle` (`self.HoldingGE`))
      (`PlayerController.ClientStopCameraShake` _playercontroller "/Game/Characters/Heroes/Hephaestus/PVP-ABILITIES/Charge/Experimental/CS_ChargeCamera.CS_ChargeCamera_C" false)
      (`PlayerController.ClientStopCameraShake` _playercontroller "/Game/Characters/Heroes/Hephaestus/PVP-ABILITIES/Charge/Experimental/CS_HoldingCharge.CS_HoldingCharge_C" false))))

(event `OnHitBoxOverlap`
  (params (OverlappedActor :type "Actor Object Reference") (OtherActor :type "Actor Object Reference"))
  (bind _async_rootmotion_task (`self.Async RootMotion Task`))
  (if (!= OtherActor (`self.GetAvatarActorFromActorInfo`))
    (`/Engine/EditorBlueprintResources/StandardMacros.IsValid` _async_rootmotion_task
      (:`Is Valid`
        (`GameplayTask.EndTask` _async_rootmotion_task))
      (:`Is Not Valid`
        _))
    (if (`KismetMathLibrary.ClassIsChildOf` (`GameplayStatics.GetObjectClass` OtherActor) "/Script/GodBound.GB_Character")
      (`AbilityTask_PlayMontageAndWait.CreatePlayMontageAndWaitProxy` "None" "/Game/Characters/SharedAnimations/MeleeAnimations/FighterAnimations/Attacks/Heph_Charge_End.Heph_Charge_End" 1.0 "None" false
        (:`then`
          (`self.Hit` (`self.InputHeldTime`)))))))

(fn `Hit`
  (params (TimeHeld :type "Float (double-precision)"))
  (bind _returnvalue (`self.GetAvatarActorFromActorInfo`))
  (bind _outactors (`KismetSystemLibrary.SphereOverlapActors` (+ (* (`Actor.GetActorForwardVector` _returnvalue) (`KismetMathLibrary.Conv_DoubleToVector` 100.0)) (`Actor.K2_GetActorLocation` _returnvalue)) 100.0 (`|MakeArray` "ObjectTypeQuery7" "ObjectTypeQuery6" :!type "EObjectTypeQuery Enum") null (`|MakeArray` (`self.GetAvatarActorFromActorInfo`))))
  (bind _returnvalue_2 (`AbilitySystemBlueprintLibrary.AssignTagSetByCallerMagnitude` (`self.MakeOutgoingGameplayEffectSpec` "/Game/Characters/Heroes/Hephaestus/PVP-ABILITIES/Charge/Experimental/GE_ChargeKnockDamage.GE_ChargeKnockDamage_C") (struct :`TagName` "Damage") (* TimeHeld (`self.Damage`))))
  (bind _returnvalue_3 (`self.SetContextEffectStrength` (`KismetMathLibrary.FMax` (* (`self.KnockBackValue`) TimeHeld) 1000.0) (`self.MakeOutgoingGameplayEffectSpec` "/Game/Characters/Heroes/Hephaestus/PVP-ABILITIES/Charge/Experimental/GE_ChargeKnockBack.GE_ChargeKnockBack_C")))
  (bind _returnvalue_4 (`AbilitySystemBlueprintLibrary.AddLinkedGameplayEffectSpec` _returnvalue_2 _returnvalue_3))
  (`self.K2_ApplyGameplayEffectSpecToTarget` _returnvalue_4 (`AbilitySystemBlueprintLibrary.AbilityTargetDataFromActorArray` _outactors))
  (`self.K2_ExecuteGameplayCue` (struct :`TagName` "GameplayCue.Hephaestus.Charge.Hit"))
  (`self.K2_EndAbility`))