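; Gameplay ability for Hephaestus's Ground Pound that knocks back the character it is granted to.
; An additive root motion radial force pushes away from a point just below the granting effect's causer, with strength read from that effect and scaled by a distance falloff curve.
; A debug sphere draws the radius on activation.
; The ability ends when the force finishes, then removes the effect that granted it.
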(event `self.K2_ActivateAbility`
  (bind _returnvalue (`self.GetGrantedByEffectContext`))
  (bind (_x _y _z) (`KismetMathLibrary.BreakVector3f` (`Actor.K2_GetActorLocation` (`AbilitySystemBlueprintLibrary.EffectContextGetEffectCauser` _returnvalue))))
  (bind _returnvalue_2 (`KismetMathLibrary.MakeVector` _x _y (- _z 100.0)))
  (`self.K2_CommitAbility`)
  (`KismetSystemLibrary.DrawDebugSphere` _returnvalue_2 500.0 12 (struct :`R` 1.0 :`G` 1.0 :`B` 1.0 :`A` 1.0) 1.0)
  (`AbilityTask_ApplyRootMotionRadialForce.ApplyRootMotionRadialForce` "None" _returnvalue_2 null (`GB_AbilitySystemLibrary.GetEffectStrength` _returnvalue) 0.5 500.0 true true false "/Game/Characters/Heroes/Hephaestus/PVP-ABILITIES/GroundPound/Curve_GroundPoundImpactKnockBack.Curve_GroundPoundImpactKnockBack" null false (struct) "MaintainLastRootMotionVelocity"
    (:`OnFinish`
      (`self.K2_EndAbility`))))

(event `self.K2_OnEndAbility`
  (params (bWasCancelled :type Boolean))
  (`self.RemoveGrantedByEffect`))