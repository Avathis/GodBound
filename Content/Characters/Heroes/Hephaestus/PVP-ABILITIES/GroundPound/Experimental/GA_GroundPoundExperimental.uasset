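; Experimental Hephaestus ground pound ability: a forward lunge and knock-up uppercut into the air, then an aimed dive onto a targeted spot.
; A montage event triggers the uppercut and rise, then a target actor waits briefly for confirmation.
; During the dive, an attached hitbox grabs overlapped characters onto the foot socket.
; Landing applies linked impact and set-by-caller damage specs in a radius; ability end releases victims and removes grab effects.
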(event `self.K2_ActivateAbility`
  (bind _returnvalue (`self.GetAvatarActorFromActorInfo`))
  (bind _returnvalue_2 (`self.GetAvatarActorFromActorInfo`))
  (bind _returnvalue_3 (`self.GetAvatarActorFromActorInfo`))
  (bind _returnvalue_4 (`self.GetAvatarActorFromActorInfo`))
  (bind (_locationtype _literaltransform _sourceactor _sourcecomponent _sourceability _sourcesocketname) (break `GameplayAbilityTargetingLocationInfo` (`self.MakeTargetLocationInfoFromOwnerActor`)))
  (bind _returnvalue_5 (`Actor.K2_GetActorLocation` _returnvalue_2))
  (`self.K2_CommitAbility`)
  (message `/Game/Characters/Heroes/Hephaestus/BI_UBHephaestusInterface.SetToOverlapPlayer` _returnvalue_4 true)
  (`AbilityTask_ApplyRootMotionMoveToForce.ApplyRootMotionMoveToForce` "None" (+ (* (`Actor.GetActorForwardVector` _returnvalue_4) (`KismetMathLibrary.Conv_DoubleToVector` 200.0)) (`Actor.K2_GetActorLocation` _returnvalue_4)) 0.44 false "MOVE_None" false null "MaintainLastRootMotionVelocity"
    (:`then`
      (`AbilityTask_PlayMontageAndWait.CreatePlayMontageAndWaitProxy` "None" "/Game/Characters/SharedAnimations/MeleeAnimations/FighterAnimations/Attacks/Montage_Hephaestus_UpAndDOwn.Montage_Hephaestus_UpAndDOwn" 1.0 "None" true 0.0
        (:`then`
          (`AbilityTask_WaitGameplayEvent.WaitGameplayEvent` (struct :`TagName` "Abilities.Hephaestus.F.Jump") null true
            (:`EventReceived`
              (`self.K2_ExecuteGameplayCue` (struct :`TagName` "GameplayCue.Hephaestus.GroundPound.UpperCut"))
              (bind _outactors (`KismetSystemLibrary.SphereOverlapActors` _returnvalue_5 200.0 (`|MakeArray` "ObjectTypeQuery7" "ObjectTypeQuery8" :!type "EObjectTypeQuery Enum") null (`|MakeArray` _returnvalue_2)))
              (`self.BP_ApplyGameplayEffectToTarget` (`AbilitySystemBlueprintLibrary.AbilityTargetDataFromActorArray` _outactors) "/Game/Characters/Heroes/SharedAbilities/GE_KnockUp_UAD.GE_KnockUp_UAD_C")
              (`AbilityTask_ApplyRootMotionConstantForce.ApplyRootMotionConstantForce` "None" (`KismetMathLibrary.Conv_RotatorToVector` (`KismetMathLibrary.FindLookAtRotation` _returnvalue_5 (+ (* (`Actor.GetActorForwardVector` _returnvalue_2) (`KismetMathLibrary.Conv_DoubleToVector` 200.0)) _returnvalue_5 (0.0 0.0 500.0)))) 1200.0 0.5 true null "MaintainLastRootMotionVelocity"
                (:`OnFinish`
                  (bind (_asynctaskproxy _data) (`AbilityTask_WaitTargetData.WaitTargetData` "None" "UserConfirmed" "/Game/Actors/TargetActors/BP_HephaestusUAD_TA.BP_HephaestusUAD_TA_C" 0.0 0.0 1000.0 (struct :`Name` "TargetActorGroundLocation") true (make `GameplayAbilityTargetingLocationInfo` _locationtype _literaltransform _sourceactor _sourcecomponent _sourceability _sourcesocketname) (struct) null (struct) true)
                    (:`then`
                      (`AbilityTask_PlayMontageAndWait.CreatePlayMontageAndWaitProxy` "None" "/Game/Characters/SharedAnimations/MeleeAnimations/FighterAnimations/Attacks/Attack_Air_to_Floor_01_Start_Seq_Retargeted_Montage.Attack_Air_to_Floor_01_Start_Seq_Retargeted_Montage" 0.2
                        (:`then`
                          (`GameplayTask_WaitDelay.TaskWaitDelay` null 1.5
                            (:`OnFinish`
                              (`/Engine/EditorBlueprintResources/StandardMacros.IsValid` _asynctaskproxy
                                (:`Is Valid`
                                  (`GameplayTask.EndTask` _asynctaskproxy)
                                  (`self.K2_EndAbility`))))))))
                    (:`ValidData`
                      (`PlayerController.ClientStopCameraShake` (`.PlayerController` (break `GameplayAbilityActorInfo` (`self.GetActorInfo`))) "/Game/Characters/Heroes/Hephaestus/PVP-ABILITIES/GroundPound/Experimental/CS_GroundPoundExp.CS_GroundPoundExp_C" false)
                      (bind (_asynctaskproxy_2 _spawnedactor) (`GameplayTask_SpawnActor.SpawnActor` null (`Actor.K2_GetActorLocation` _returnvalue) (`Actor.K2_GetActorRotation` _returnvalue) "/Game/Characters/Heroes/Hephaestus/PVP-ABILITIES/GroundPound/Experimental/BP_GroundPoundHitbox.BP_GroundPoundHitbox_C" false null)
                        (:`Success`
                          (bind _output_get (set `self.HitBox` _spawnedactor))
                          (add `Actor.OnActorBeginOverlap` _output_get (delegate `OnActorBeginOverlap_Event`))
                          (`Actor.K2_AttachToActor` _output_get (`self.GetAvatarActorFromActorInfo`) "None" "KeepWorld" "KeepWorld" "KeepWorld" true)
                          (`self.K2_ExecuteGameplayCue` (struct :`TagName` "GameplayCue.Hephaestus.GroundPound.Repel"))
                          (`AbilityTask_ApplyRootMotionMoveToForce.ApplyRootMotionMoveToForce` "None" (`.Location` (`GameplayStatics.BreakHitResult` (`AbilitySystemBlueprintLibrary.GetHitResultFromTargetData` _data))) 0.3 false "MOVE_Falling" false null "SetVelocity"
                            (:`then`
                              (`AbilityTask_PlayMontageAndWait.CreatePlayMontageAndWaitProxy` "None" "/Game/Characters/SharedAnimations/MeleeAnimations/FighterAnimations/Attacks/Attack_Air_to_Floor_01_Loop_Seq_Retargeted_Montage.Attack_Air_to_Floor_01_Loop_Seq_Retargeted_Montage" 0.01))
                            (:`OnTimedOut`
                              (`AbilityTask_PlayMontageAndWait.CreatePlayMontageAndWaitProxy` "None" "/Game/Characters/SharedAnimations/MeleeAnimations/FighterAnimations/Attacks/Attack_Air_to_Floor_01_End_Seq_Retargeted_Montage.Attack_Air_to_Floor_01_End_Seq_Retargeted_Montage" 1.5 "None" false :!label _label
                                (:`then`
                                  (bind _outactors_2 (`KismetSystemLibrary.SphereOverlapActors` (`Actor.K2_GetActorLocation` _returnvalue_3) 300.0 (`|MakeArray` "ObjectTypeQuery7" "ObjectTypeQuery10" "ObjectTypeQuery8" :!type "EObjectTypeQuery Enum") "/Script/GodBound.GB_Character" (`|MakeArray` _returnvalue_3)))
                                  (bind _returnvalue_6 (`self.SetContextEffectStrength` 2000.0 (`self.MakeOutgoingGameplayEffectSpec` "/Game/Characters/Heroes/Hephaestus/PVP-ABILITIES/GroundPound/GE_GroundPoundImpactDamage.GE_GroundPoundImpactDamage_C")))
                                  (bind _returnvalue_7 (`AbilitySystemBlueprintLibrary.AssignTagSetByCallerMagnitude` (`self.MakeOutgoingGameplayEffectSpec` "/Game/Characters/Heroes/Hephaestus/PVP-ABILITIES/GroundPound/GE_GroundPoundDamage.GE_GroundPoundDamage_C") (struct :`TagName` "Damage") 250.0))
                                  (bind _returnvalue_8 (`AbilitySystemBlueprintLibrary.AddLinkedGameplayEffectSpec` _returnvalue_6 _returnvalue_7))
                                  (`self.K2_ApplyGameplayEffectSpecToTarget` _returnvalue_8 (`AbilitySystemBlueprintLibrary.AbilityTargetDataFromActorArray` _outactors_2))
                                  (`self.K2_ExecuteGameplayCue` (struct :`TagName` "GameplayCue.Hephaestus.GroundPound.Impact.Exp"))
                                  (`GameplayTask_WaitDelay.TaskWaitDelay` null 0.05
                                    (:`OnFinish`
                                      (`KismetSystemLibrary.PrintString` "Effects Working")
                                      (`self.K2_EndAbility`))))))
                            (:`OnTimedOutAndDestinationReached`
                              (goto _label))))
                        (:`DidNotSpawn`
                          (`self.K2_CancelAbility`))))
                    (:`Cancelled`
                      (`self.K2_EndAbility`))))))))
        (:`OnCancelled`
          (`self.K2_CancelAbility`))))))

(event `self.K2_OnEndAbility`
  (params (bWasCancelled :type Boolean))
  (bind _attachedactors (`self.AttachedActors`))
  (bind _hitbox (`self.HitBox`))
  (`PlayerController.ClientStopCameraShake` (`.PlayerController` (break `GameplayAbilityActorInfo` (`self.GetActorInfo`))) "/Game/Characters/Heroes/Hephaestus/PVP-ABILITIES/GroundPound/Experimental/CS_GroundPoundExp.CS_GroundPoundExp_C" false)
  (`/Engine/EditorBlueprintResources/StandardMacros.IsValid` _hitbox
    (:`Is Valid`
      (`Actor.K2_DestroyActor` _hitbox)
      (set `self.HitBox` null))
    (:`Is Not Valid`
      _))
  (message `/Game/Characters/Heroes/Hephaestus/BI_UBHephaestusInterface.SetToOverlapPlayer` (`self.GetAvatarActorFromActorInfo`) false)
  (for _array_element (`self.AttachedEffects`)
    (`self.BP_RemoveGameplayEffectFromOwnerWithHandle` _array_element))
  (if (`KismetArrayLibrary.Array_IsNotEmpty` _attachedactors)
    (for _array_element_2 _attachedactors
      (`KismetSystemLibrary.PrintString` (`KismetSystemLibrary.GetObjectName` _array_element_2))
      (message `/Game/Characters/Heroes/Hephaestus/BI_UBHephaestusInterface.SetToOverlapPlayer` _array_element_2 false)
      (`Actor.K2_DetachFromActor` _array_element_2 "KeepWorld" "KeepWorld" "KeepWorld"))
    (`KismetArrayLibrary.Array_Clear` _attachedactors)))

(event `OnActorBeginOverlap_Event`
  (params (OverlappedActor :type "Actor Object Reference") (OtherActor :type "Actor Object Reference"))
  (bind _returnvalue (`self.GetAvatarActorFromActorInfo`))
  (`KismetSystemLibrary.PrintString` "Overlapped")
  (if (!= OtherActor _returnvalue)
    (if (not (`KismetArrayLibrary.Array_Contains` (`self.AttachedActors`) OtherActor))
      (`KismetArrayLibrary.Array_Add` (`self.AttachedActors`) OtherActor)
      (if (`KismetMathLibrary.ClassIsChildOf` (`GameplayStatics.GetObjectClass` OtherActor) "/Script/GodBound.GB_Character")
        (message `/Game/Characters/Heroes/Hephaestus/BI_UBHephaestusInterface.SetToOverlapPlayer` OtherActor true)
        (bind _returnvalue_2 (`self.BP_ApplyGameplayEffectToTarget` (`AbilitySystemBlueprintLibrary.AbilityTargetDataFromActor` OtherActor) "/Game/Characters/Heroes/GeneralEffects/Debuffs/GE_Grabbed.GE_Grabbed_C"))
        (`KismetArrayLibrary.Array_Append` (`self.AttachedEffects`) _returnvalue_2)
        (`Actor.K2_AttachToActor` OtherActor _returnvalue "Foot_L_Kick" "KeepWorld" "KeepWorld" "KeepWorld" true)))))