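; GA_GroundPound is Hephaestus's PvP ground-pound ability: a targeted dash, leap and slam.
; Instant trace targeting drives a root-motion dash, then a gameplay event during the montage spawns a hitbox.
; Overlapped characters take damage and an attach effect as Hephaestus makes a root-motion jump, whose finish triggers radial impact damage and a GameplayCue.
; The ability ends early without a target or hitbox overlap, and cleanup restores movement, camera and collision state.
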(event `self.K2_ActivateAbility`
  (bind _returnvalue (`self.GetAvatarActorFromActorInfo`))
  (bind _returnvalue_2 (`self.GetAvatarActorFromActorInfo`))
  (bind _returnvalue_3 (`self.GetAvatarActorFromActorInfo`))
  (bind (_locationtype _literaltransform _sourceactor _sourcecomponent _sourceability _sourcesocketname) (break `GameplayAbilityTargetingLocationInfo` (`self.MakeTargetLocationInfoFromOwnerActor`)))
  (`self.K2_CommitAbility`)
  (bind _returnvalue_4 (`CameraAnimationCameraModifier.PlayCameraAnimation` (`CameraAnimationCameraModifier.GetCameraAnimationCameraModifierFromPlayerController` (`.PlayerController` (break `GameplayAbilityActorInfo` (`self.GetActorInfo`)))) "/Game/Characters/Heroes/Hephaestus/PVP-ABILITIES/GroundPound/GroundPoundCameraSequence.GroundPoundCameraSequence" (make `CameraAnimationParams` 1.3 1.0 "Linear" 0.0 "Linear" 0.5 false false 0.3)))
  (set `self.CameraAnimation` _returnvalue_4)
  (message `/Game/Characters/Heroes/BI_AbilitiesGeneral.SetInAbilityMontage` _returnvalue true)
  (message `/Game/Characters/Heroes/BI_AbilitiesGeneral.SetCanManuallyMove` _returnvalue false)
  (bind (_asynctaskproxy _data) (`AbilityTask_WaitTargetData.WaitTargetData` "None" "Instant" "/Game/Characters/Heroes/Hephaestus/PVP-ABILITIES/GroundPound/BP_TAGroundPoundTrace.BP_TAGroundPoundTrace_C" 100.0 400.0 (struct :`Name` "PVP_TargetPlayer") true 1 1 false false false (make `GameplayAbilityTargetingLocationInfo` _locationtype _literaltransform _sourceactor _sourcecomponent _sourceability _sourcesocketname) (struct) null)
    (:`ValidData`
      (message `/Game/Characters/Heroes/Hephaestus/BI_UBHephaestusInterface.SetToOverlapPlayer` (`self.GetAvatarActorFromActorInfo`) true)
      (if (`AbilitySystemBlueprintLibrary.TargetDataHasActor` _data)
        (`AbilityTask_ApplyRootMotionMoveToActorForce.ApplyRootMotionMoveToTargetDataActorForce` "None" _data 0 0 (0.0 0.0 0.0) "AlignFromTargetToSource" 0.5 null "/Game/Characters/Heroes/Hephaestus/PVP-ABILITIES/GroundPound/Curve_GroundPoundAirTime.Curve_GroundPoundAirTime" false "MOVE_None" false null "/Game/Characters/Heroes/Hephaestus/PVP-ABILITIES/GroundPound/Curve_GroundPoundDash.Curve_GroundPoundDash" "SetVelocity"
          (:`then`
            (message `/Game/Characters/Heroes/BI_AbilitiesGeneral.SetInAbilityMontage` (`self.GetAvatarActorFromActorInfo`) false)
            (`AbilityTask_PlayMontageAndWait.CreatePlayMontageAndWaitProxy` "None" "/Game/Characters/SharedAnimations/MeleeAnimations/FighterAnimations/Attacks/Montage_Hephaestus_UpAndDOwn.Montage_Hephaestus_UpAndDOwn"
              (:`then`
                (`AbilityAsync_WaitGameplayEvent.WaitGameplayEventToActor` (`self.GetAvatarActorFromActorInfo`) (struct :`TagName` "Abilities.Hephaestus.F.Jump") true
                  (:`EventReceived`
                    (bind (_asynctaskproxy_2 _spawnedactor) (`GameplayTask_SpawnActor.SpawnActor` null (+ (`Actor.K2_GetActorLocation` _returnvalue_2) (* (`Actor.GetActorForwardVector` _returnvalue_2) (`KismetMathLibrary.Conv_DoubleToVector` 75.0))) (`Actor.K2_GetActorRotation` _returnvalue_2) (`self.HitBoxClass`) false (cast `GB_Character` _returnvalue_2 :!pure true))
                      (:`Success`
                        (set `self.Actor` _spawnedactor)
                        (bind _overlappingactors (`Actor.GetOverlappingActors` _spawnedactor "/Script/GodBound.GB_Character"))
                        (if (`KismetArrayLibrary.Array_IsNotEmpty` _overlappingactors)
                          (bind _returnvalue_5 (`AbilitySystemBlueprintLibrary.AssignTagSetByCallerMagnitude` (`self.MakeOutgoingGameplayEffectSpec` "/Game/Characters/Heroes/Hephaestus/PVP-ABILITIES/GroundPound/GE_GroundPoundDamage.GE_GroundPoundDamage_C") (struct :`TagName` "Damage") 40.0))
                          (bind _returnvalue_6 (`AbilitySystemBlueprintLibrary.AddLinkedGameplayEffectSpec` (`self.MakeOutgoingGameplayEffectSpec` "/Game/Characters/Heroes/Hephaestus/PVP-ABILITIES/GroundPound/GE_GroundPoundAttached.GE_GroundPoundAttached_C") _returnvalue_5))
                          (bind _returnvalue_7 (`self.K2_ApplyGameplayEffectSpecToTarget` _returnvalue_6 (`AbilitySystemBlueprintLibrary.AbilityTargetDataFromActorArray` _overlappingactors)))
                          (set `self.ActiveKnockUpEffect` _returnvalue_7)
                          (bind _asynctaskproxy_3 (`AbilityTask_ApplyRootMotionJumpForce.ApplyRootMotionJumpForce` "None" (`Actor.K2_GetActorRotation` (`self.GetAvatarActorFromActorInfo`)) 1000.0 500.0 2.0 0.0 true "MaintainLastRootMotionVelocity")
                            (:`OnFinish`
                              (`GameplayTask.EndTask` _asynctaskproxy_3)
                              (for _array_element (`self.ActiveKnockUpEffect`)
                                (`self.BP_RemoveGameplayEffectFromOwnerWithHandle` _array_element))
                              (bind _outactors (`KismetSystemLibrary.SphereOverlapActors` (`Actor.K2_GetActorLocation` _returnvalue_3) 300.0 (`|MakeArray` "ObjectTypeQuery7" "ObjectTypeQuery10" :!type "EObjectTypeQuery Enum") "/Script/GodBound.GB_Character" (`|MakeArray` _returnvalue_3)))
                              (bind _returnvalue_8 (`self.SetContextEffectStrength` 2000.0 (`self.MakeOutgoingGameplayEffectSpec` "/Game/Characters/Heroes/Hephaestus/PVP-ABILITIES/GroundPound/GE_GroundPoundImpactDamage.GE_GroundPoundImpactDamage_C")))
                              (bind _returnvalue_9 (`AbilitySystemBlueprintLibrary.AssignTagSetByCallerMagnitude` (`self.MakeOutgoingGameplayEffectSpec` "/Game/Characters/Heroes/Hephaestus/PVP-ABILITIES/GroundPound/GE_GroundPoundDamage.GE_GroundPoundDamage_C") (struct :`TagName` "Damage") 250.0))
                              (bind _returnvalue_10 (`AbilitySystemBlueprintLibrary.AddLinkedGameplayEffectSpec` _returnvalue_8 _returnvalue_9))
                              (`self.K2_ApplyGameplayEffectSpecToTarget` _returnvalue_10 (`AbilitySystemBlueprintLibrary.AbilityTargetDataFromActorArray` _outactors))
                              (`self.K2_ExecuteGameplayCueWithParams` (struct :`TagName` "GameplayCue.Hephaestus.GroundPound.Impact") (`AbilitySystemBlueprintLibrary.MakeGameplayCueParameters` 50.0)))
                            (:`OnLanded`
                              (`AbilityTask_PlayMontageAndWait.CreatePlayMontageAndWaitProxy` "None" "/Game/Characters/SharedAnimations/MeleeAnimations/FighterAnimations/Attacks/Attack_Air_to_Floor_01_End_Seq_Retargeted_Montage.Attack_Air_to_Floor_01_End_Seq_Retargeted_Montage"
                                (:`OnCompleted`
                                  _)
                                (:`OnBlendOut`
                                  _)
                                (:`OnInterrupted`
                                  _)
                                (:`OnCancelled`
                                  _))
                              (`self.K2_EndAbility`)))
                          (else
                            (`self.K2_EndAbility`))))))))
              (:`OnBlendOut`
                (`AbilityTask_PlayMontageAndWait.CreatePlayMontageAndWaitProxy` "None" "/Game/Characters/SharedAnimations/MeleeAnimations/FighterAnimations/Attacks/Attack_Air_to_Floor_01_Start_Seq_Retargeted_Montage.Attack_Air_to_Floor_01_Start_Seq_Retargeted_Montage" 0.2
                  (:`OnBlendOut`
                    (`AbilityTask_PlayMontageAndWait.CreatePlayMontageAndWaitProxy` "None" "/Game/Characters/SharedAnimations/MeleeAnimations/FighterAnimations/Attacks/Attack_Air_to_Floor_01_Loop_Seq_Retargeted_Montage.Attack_Air_to_Floor_01_Loop_Seq_Retargeted_Montage"))))
              (:`OnInterrupted`
                (`self.K2_CancelAbility` :!label _label))
              (:`OnCancelled`
                (goto _label)))))
        (else
          (`self.K2_EndAbility`))))))

(event `self.K2_OnEndAbility`
  (params (bWasCancelled :type Boolean))
  (bind _returnvalue (`self.GetAvatarActorFromActorInfo`))
  (bind _actor (`self.Actor`))
  (bind (_owneractor _avataractor _playercontroller) (break `GameplayAbilityActorInfo` (`self.GetActorInfo`)))
  (bind _returnvalue_2 (`CameraAnimationCameraModifier.GetCameraAnimationCameraModifierFromPlayerController` _playercontroller))
  (if (`KismetSystemLibrary.IsValid` (`PlayerController.PlayerCameraManager` _playercontroller))
    (if (`KismetSystemLibrary.IsValid` _returnvalue_2)
      (`CameraAnimationCameraModifier.StopAllCameraAnimations` _returnvalue_2 false)))
  (message `/Game/Characters/Heroes/Hephaestus/BI_UBHephaestusInterface.SetToOverlapPlayer` _returnvalue false)
  (message `/Game/Characters/Heroes/BI_AbilitiesGeneral.SetInAbilityMontage` _returnvalue true)
  (message `/Game/Characters/Heroes/BI_AbilitiesGeneral.SetCanManuallyMove` _returnvalue true)
  (`/Engine/EditorBlueprintResources/StandardMacros.IsValid` _actor
    (:`Is Valid`
      (`Actor.K2_DestroyActor` _actor)
      (set `self.Actor` null))))