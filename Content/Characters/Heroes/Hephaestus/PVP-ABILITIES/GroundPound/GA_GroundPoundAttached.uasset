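; Gameplay ability for Hephaestus's GroundPound that applies a knock-up to its owner, apparently the character hit, when granted by a gameplay effect.
; On activation, a root motion jump force launches the owner along the effect causer's rotation until landing.
; Slowed heavy-hit start and loop montages chain on blend out.
; Ending removes the granting effect, but the EndAbility calls are unwired, so the ability never ends itself.
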(event `self.K2_ActivateAbility`
  (`KismetSystemLibrary.PrintString` "KnockUPACTIVE")
  (`AbilityTask_ApplyRootMotionJumpForce.ApplyRootMotionJumpForce` "None" (`Actor.K2_GetActorRotation` (`AbilitySystemBlueprintLibrary.EffectContextGetEffectCauser` (`self.GetGrantedByEffectContext`))) 1000.0 500.0 2.0 0.0 true "MaintainLastRootMotionVelocity"
    (:`then`
      (`AbilityTask_PlayMontageAndWait.CreatePlayMontageAndWaitProxy` "None" "/Game/Characters/SharedAnimations/MeleeAnimations/FighterAnimations/Hit/Hit_Heavy_Start_Seq_Retargeted_Montage.Hit_Heavy_Start_Seq_Retargeted_Montage" 0.2
        (:`OnBlendOut`
          (`AbilityTask_PlayMontageAndWait.CreatePlayMontageAndWaitProxy` "None" "/Game/Characters/SharedAnimations/MeleeAnimations/FighterAnimations/Hit/Hit_Heavy_Loop_Seq_Retargeted_Montage.Hit_Heavy_Loop_Seq_Retargeted_Montage" 0.1))))))

(event `self.K2_OnEndAbility`
  (params (bWasCancelled :type Boolean))
  (`self.RemoveGrantedByEffect`)
  (`KismetSystemLibrary.PrintString` "KnockUP ENDED REALLY FAST \n"))