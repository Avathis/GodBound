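; Hephaestus's melee auto-attack Gameplay Ability, a five-stage montage punch combo chained by repeated attack activations.
; Each stage lunges with root motion toward an instantly traced target or straight ahead, then montage events trigger hand-socket sphere traces that apply damage.
; IntoCombo events check GetCanIntoCombo to continue immediately or await another activation, using nested async tasks.
; A combo effect lasts until the ability ends, which also restores movement.
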(event `self.K2_ActivateAbility`
  (bind _returnvalue (`self.GetAvatarActorFromActorInfo`))
  (bind _returnvalue_2 (`self.GetAvatarActorFromActorInfo`))
  (bind _returnvalue_3 (`self.GetAvatarActorFromActorInfo`))
  (bind _returnvalue_4 (`self.GetAvatarActorFromActorInfo`))
  (bind _returnvalue_5 (`self.GetAvatarActorFromActorInfo`))
  (bind _returnvalue_6 (`self.GetAvatarActorFromActorInfo`))
  (bind _returnvalue_7 (`self.GetAvatarActorFromActorInfo`))
  (bind _returnvalue_8 (`self.GetAvatarActorFromActorInfo`))
  (bind (_locationtype _literaltransform _sourceactor _sourcecomponent _sourceability _sourcesocketname) (break `GameplayAbilityTargetingLocationInfo` (`self.MakeTargetLocationInfoFromOwnerActor`)))
  (bind (_locationtype_2 _literaltransform_2 _sourceactor_2 _sourcecomponent_2 _sourceability_2 _sourcesocketname_2) (break `GameplayAbilityTargetingLocationInfo` (`self.MakeTargetLocationInfoFromOwnerActor`)))
  (bind (_locationtype_3 _literaltransform_3 _sourceactor_3 _sourcecomponent_3 _sourceability_3 _sourcesocketname_3) (break `GameplayAbilityTargetingLocationInfo` (`self.MakeTargetLocationInfoFromOwnerActor`)))
  (bind (_locationtype_4 _literaltransform_4 _sourceactor_4 _sourcecomponent_4 _sourceability_4 _sourcesocketname_4) (break `GameplayAbilityTargetingLocationInfo` (`self.MakeTargetLocationInfoFromOwnerActor`)))
  (bind (_locationtype_5 _literaltransform_5 _sourceactor_5 _sourcecomponent_5 _sourceability_5 _sourcesocketname_5) (break `GameplayAbilityTargetingLocationInfo` (`self.MakeTargetLocationInfoFromOwnerActor`)))
  (`self.K2_CommitAbility`)
  (bind _returnvalue_9 (`self.BP_ApplyGameplayEffectToOwner` "/Game/Characters/Heroes/Hephaestus/PVP-ABILITIES/AutoAttack/GE_HephIntoCombo.GE_HephIntoCombo_C"))
  (set `self.HephaestusComboGE` _returnvalue_9)
  (`AbilityTask_WaitAbilityActivate.WaitForAbilityActivate` (struct) (struct :`TagName` "Abilities.Hephaestus.F.AutoAttack")
    (:`then`
      ;[1 1 1] 1st Attack
      (message `/Game/Characters/Heroes/BI_AbilitiesGeneral.SetCanManuallyMove` (`self.GetAvatarActorFromActorInfo`) false)
      (bind (_asynctaskproxy _data) (`AbilityTask_WaitTargetData.WaitTargetData` "None" "Instant" (`self.TargetActorClass`) 50.0 200.0 (struct :`Name` "PVP_TargetPlayer") false 5 1 true false false (make `GameplayAbilityTargetingLocationInfo` _locationtype_5 _literaltransform_5 _sourceactor_5 _sourcecomponent_5 _sourceability_5 _sourcesocketname_5) (struct) null)
        (:`then`
          (`AbilityTask_PlayMontageAndWait.CreatePlayMontageAndWaitProxy` "None" (`self.Montage_1`) 0.8
            (:`then`
              (bind _asynctaskproxy_2 (`AbilityAsync_WaitGameplayEvent.WaitGameplayEventToActor` (`self.GetAvatarActorFromActorInfo`) (struct :`TagName` "Abilities.Hephaestus.OutOfCombo") true)
                (:`then`
                  (set `self.OutOfComboAction` _asynctaskproxy_2)
                  (`AbilityAsync_WaitGameplayEvent.WaitGameplayEventToActor` _returnvalue_2 (struct :`TagName` "Abilities.Hephaestus.F.AutoAttack.Left.Small") true
                    (:`then`
                      (`AbilityAsync_WaitGameplayEvent.WaitGameplayEventToActor` _returnvalue_2 (struct :`TagName` "Abilities.Hephaestus.F.AutoAttack.Right.Small") true
                        (:`then`
                          ;[1 1 1] 2nd Attack
                          (bind _asynctaskproxy_3 (`AbilityTask_WaitAbilityActivate.WaitForAbilityActivate` (struct :`TagName` "Abilities.Hephaestus.F.AutoAttack"))
                            (:`then`
                              (`AbilityAsync_WaitGameplayEvent.WaitGameplayEventToActor` (`self.GetAvatarActorFromActorInfo`) (struct :`TagName` "Abilities.IntoCombo") true false
                                (:`EventReceived`
                                  (message `/Game/Characters/Heroes/BI_AbilitiesGeneral.SetInAbilityMontage` (`self.GetAvatarActorFromActorInfo`) true)
                                  (`/Engine/EditorBlueprintResources/StandardMacros.IsValid` _asynctaskproxy_3
                                    (:`Is Valid`
                                      (`GameplayTask.EndTask` _asynctaskproxy_3))
                                    (:`Is Not Valid`
                                      _))
                                  (bind _cancombo (`self.GetCanIntoCombo`))
                                  (if (not _cancombo)
                                    (`AbilityTask_WaitAbilityActivate.WaitForAbilityActivate` (struct :`TagName` "Abilities.Hephaestus.F.AutoAttack")
                                      (:`OnActivate`
                                        _)))
                                  (bind (_asynctaskproxy_4 _data_2) (`AbilityTask_WaitTargetData.WaitTargetData` "None" "Instant" (`self.TargetActorClass`) 50.0 200.0 (struct :`Name` "PVP_TargetPlayer") true 1 1 false false false (make `GameplayAbilityTargetingLocationInfo` _locationtype_2 _literaltransform_2 _sourceactor_2 _sourcecomponent_2 _sourceability_2 _sourcesocketname_2) (struct) null)
                                    (:`then`
                                      (`AbilityTask_PlayMontageAndWait.CreatePlayMontageAndWaitProxy` "None" (`self.Montage_2`)
                                        (:`then`
                                          (bind _asynctaskproxy_5 (`AbilityAsync_WaitGameplayEvent.WaitGameplayEventToActor` (`self.GetAvatarActorFromActorInfo`) (struct :`TagName` "Abilities.Hephaestus.OutOfCombo") true)
                                            (:`then`
                                              (set `self.OutOfComboAction` _asynctaskproxy_5)
                                              (`AbilityAsync_WaitGameplayEvent.WaitGameplayEventToActor` (`self.GetAvatarActorFromActorInfo`) (struct :`TagName` "Abilities.Hephaestus.F.AutoAttack.Left.Big") true
                                                (:`then`
                                                  ;[1 1 1] 3rd Attack
                                                  (bind _asynctaskproxy_6 (`AbilityTask_WaitAbilityActivate.WaitForAbilityActivate` (struct :`TagName` "Abilities.Hephaestus.F.AutoAttack"))
                                                    (:`then`
                                                      (`AbilityAsync_WaitGameplayEvent.WaitGameplayEventToActor` (`self.GetAvatarActorFromActorInfo`) (struct :`TagName` "Abilities.IntoCombo") true false
                                                        (:`EventReceived`
                                                          (message `/Game/Characters/Heroes/BI_AbilitiesGeneral.SetInAbilityMontage` (`self.GetAvatarActorFromActorInfo`) true)
                                                          (`/Engine/EditorBlueprintResources/StandardMacros.IsValid` _asynctaskproxy_6
                                                            (:`Is Valid`
                                                              (`GameplayTask.EndTask` _asynctaskproxy_6))
                                                            (:`Is Not Valid`
                                                              _))
                                                          (bind _cancombo_2 (`self.GetCanIntoCombo`))
                                                          (if (not _cancombo_2)
                                                            (`AbilityTask_WaitAbilityActivate.WaitForAbilityActivate` (struct :`TagName` "Abilities.Hephaestus.F.AutoAttack")
                                                              (:`OnActivate`
                                                                _)))
                                                          (message `/Game/Characters/Heroes/BI_AbilitiesGeneral.SetCanManuallyMove` (`self.GetAvatarActorFromActorInfo`) false)
                                                          (bind (_asynctaskproxy_7 _data_3) (`AbilityTask_WaitTargetData.WaitTargetData` "None" "Instant" (`self.TargetActorClass`) 50.0 200.0 (struct :`Name` "PVP_TargetPlayer") true 1 1 false false false (make `GameplayAbilityTargetingLocationInfo` _locationtype_3 _literaltransform_3 _sourceactor_3 _sourcecomponent_3 _sourceability_3 _sourcesocketname_3) (struct) null)
                                                            (:`then`
                                                              (`AbilityTask_PlayMontageAndWait.CreatePlayMontageAndWaitProxy` "None" (`self.Montage_3`)
                                                                (:`then`
                                                                  (`AbilityAsync_WaitGameplayEvent.WaitGameplayEventToActor` (`self.GetAvatarActorFromActorInfo`) (struct :`TagName` "Abilities.Hephaestus.F.AutoAttack.Right.Big") true
                                                                    (:`then`
                                                                      ;[1 1 1] 4th Attack
                                                                      (bind _asynctaskproxy_8 (`AbilityTask_WaitAbilityActivate.WaitForAbilityActivate` (struct :`TagName` "Abilities.Hephaestus.F.AutoAttack"))
                                                                        (:`then`
                                                                          (`AbilityAsync_WaitGameplayEvent.WaitGameplayEventToActor` _returnvalue (struct :`TagName` "Abilities.IntoCombo") true false
                                                                            (:`EventReceived`
                                                                              (message `/Game/Characters/Heroes/BI_AbilitiesGeneral.SetInAbilityMontage` _returnvalue true)
                                                                              (`/Engine/EditorBlueprintResources/StandardMacros.IsValid` _asynctaskproxy_8
                                                                                (:`Is Valid`
                                                                                  (`GameplayTask.EndTask` _asynctaskproxy_8))
                                                                                (:`Is Not Valid`
                                                                                  _))
                                                                              (bind _cancombo_3 (`self.GetCanIntoCombo`))
                                                                              (if (not _cancombo_3)
                                                                                (`AbilityTask_WaitAbilityActivate.WaitForAbilityActivate` (struct :`TagName` "Abilities.Hephaestus.F.AutoAttack")
                                                                                  (:`OnActivate`
                                                                                    _)))
                                                                              (message `/Game/Characters/Heroes/BI_AbilitiesGeneral.SetCanManuallyMove` (`self.GetAvatarActorFromActorInfo`) false)
                                                                              (bind (_asynctaskproxy_9 _data_4) (`AbilityTask_WaitTargetData.WaitTargetData` "None" "Instant" (`self.TargetActorClass`) 50.0 200.0 (struct :`Name` "PVP_TargetPlayer") true 1 1 false false false (make `GameplayAbilityTargetingLocationInfo` _locationtype_4 _literaltransform_4 _sourceactor_4 _sourcecomponent_4 _sourceability_4 _sourcesocketname_4) (struct) null)
                                                                                (:`then`
                                                                                  (`AbilityTask_PlayMontageAndWait.CreatePlayMontageAndWaitProxy` "None" (`self.Montage_4`)
                                                                                    (:`then`
                                                                                      (`AbilityAsync_WaitGameplayEvent.WaitGameplayEventToActor` (`self.GetAvatarActorFromActorInfo`) (struct :`TagName` "Abilities.Hephaestus.F.AutoAttack.Left.Big") true
                                                                                        (:`then`
                                                                                          ;[1 1 1] 5th Attack
                                                                                          (bind _asynctaskproxy_10 (`AbilityTask_WaitAbilityActivate.WaitForAbilityActivate` (struct :`TagName` "Abilities.Hephaestus.F.AutoAttack"))
                                                                                            (:`then`
                                                                                              (`AbilityAsync_WaitGameplayEvent.WaitGameplayEventToActor` _returnvalue_7 (struct :`TagName` "Abilities.IntoCombo") true false
                                                                                                (:`EventReceived`
                                                                                                  (message `/Game/Characters/Heroes/BI_AbilitiesGeneral.SetInAbilityMontage` _returnvalue_7 true)
                                                                                                  (`/Engine/EditorBlueprintResources/StandardMacros.IsValid` _asynctaskproxy_10
                                                                                                    (:`Is Valid`
                                                                                                      (`GameplayTask.EndTask` _asynctaskproxy_10))
                                                                                                    (:`Is Not Valid`
                                                                                                      _))
                                                                                                  (bind _cancombo_4 (`self.GetCanIntoCombo`))
                                                                                                  (if (not _cancombo_4)
                                                                                                    (`AbilityTask_WaitAbilityActivate.WaitForAbilityActivate` (struct :`TagName` "Abilities.Hephaestus.F.AutoAttack")
                                                                                                      (:`OnActivate`
                                                                                                        _)))
                                                                                                  (bind (_asynctaskproxy_11 _data_5) (`AbilityTask_WaitTargetData.WaitTargetData` "None" "Instant" (`self.TargetActorClass`) 50.0 400.0 (struct :`Name` "PVP_TargetPlayer") true 1 1 false false false (make `GameplayAbilityTargetingLocationInfo` _locationtype _literaltransform _sourceactor _sourcecomponent _sourceability _sourcesocketname) (struct) null)
                                                                                                    (:`then`
                                                                                                      (`AbilityTask_PlayMontageAndWait.CreatePlayMontageAndWaitProxy` "None" (`self.Montage_5`)
                                                                                                        (:`then`
                                                                                                          (`AbilityAsync_WaitGameplayEvent.WaitGameplayEventToActor` (`self.GetAvatarActorFromActorInfo`) (struct :`TagName` "Abilities.Hephaestus.F.AutoAttack.Right.Big") true
                                                                                                            (:`EventReceived`
                                                                                                              (bind _newparam (`self.TraceForTargets` 50.0 50.0 "Hand_R_Punch"))
                                                                                                              (`self.ApplyDamageToTarget` _newparam 45.0))))
                                                                                                        (:`OnCompleted`
                                                                                                          (`self.K2_EndAbility` :!label _label))
                                                                                                        (:`OnBlendOut`
                                                                                                          (goto _label))
                                                                                                        (:`OnInterrupted`
                                                                                                          (goto _label))
                                                                                                        (:`OnCancelled`
                                                                                                          (goto _label))))
                                                                                                    (:`ValidData`
                                                                                                      (message `/Game/Characters/Heroes/BI_AbilitiesGeneral.SetInAbilityMontage` (`self.GetAvatarActorFromActorInfo`) false)
                                                                                                      (if (`AbilitySystemBlueprintLibrary.TargetDataHasActor` _data_5)
                                                                                                        (`AbilityTask_ApplyRootMotionMoveToActorForce.ApplyRootMotionMoveToTargetDataActorForce` "None" _data_5 0 0 (0.0 0.0 0.0) "AlignToWorldSpace" 0.2 null null false "MOVE_None" false null null "MaintainLastRootMotionVelocity" (0.0 0.0 0.0) 0.0 true)
                                                                                                        (else
                                                                                                          (`AbilityTask_ApplyRootMotionMoveToForce.ApplyRootMotionMoveToForce` "None" (+ (`Actor.K2_GetActorLocation` _returnvalue_4) (* (`Actor.GetActorForwardVector` _returnvalue_4) (`KismetMathLibrary.Conv_DoubleToVector` 200.0))) 0.2 false "MOVE_None" true null "MaintainLastRootMotionVelocity"))))))))
                                                                                            (:`OnActivate`
                                                                                              (`self.SetCombo`))))
                                                                                        (:`EventReceived`
                                                                                          (bind _newparam_2 (`self.TraceForTargets` 50.0 50.0 "Hand_L_Punch"))
                                                                                          (`self.ApplyDamageToTarget` _newparam_2 30.0))))
                                                                                    (:`OnCompleted`
                                                                                      (`self.K2_EndAbility` :!label _label_2))
                                                                                    (:`OnBlendOut`
                                                                                      (goto _label_2))
                                                                                    (:`OnCancelled`
                                                                                      (goto _label_2))))
                                                                                (:`ValidData`
                                                                                  (message `/Game/Characters/Heroes/BI_AbilitiesGeneral.SetInAbilityMontage` (`self.GetAvatarActorFromActorInfo`) false)
                                                                                  (if (`AbilitySystemBlueprintLibrary.TargetDataHasActor` _data_4)
                                                                                    (`AbilityTask_ApplyRootMotionMoveToActorForce.ApplyRootMotionMoveToTargetDataActorForce` "None" _data_4 0 0 (0.0 0.0 0.0) "AlignToWorldSpace" 0.2 null null false "MOVE_None" false null null "MaintainLastRootMotionVelocity" (0.0 0.0 0.0) 0.0 true)
                                                                                    (else
                                                                                      (`AbilityTask_ApplyRootMotionMoveToForce.ApplyRootMotionMoveToForce` "None" (+ (`Actor.K2_GetActorLocation` _returnvalue_8) (* (`Actor.GetActorForwardVector` _returnvalue_8) (`KismetMathLibrary.Conv_DoubleToVector` 200.0))) 0.2 false "MOVE_None" false null "MaintainLastRootMotionVelocity"))))))))
                                                                        (:`OnActivate`
                                                                          (`self.SetCombo`))))
                                                                    (:`EventReceived`
                                                                      (bind _newparam_3 (`self.TraceForTargets` 50.0 50.0 "Hand_R_Punch"))
                                                                      (`self.ApplyDamageToTarget` _newparam_3 35.0))))
                                                                (:`OnCompleted`
                                                                  (`self.K2_EndAbility` :!label _label_3))
                                                                (:`OnBlendOut`
                                                                  (goto _label_3))
                                                                (:`OnCancelled`
                                                                  (goto _label_3))))
                                                            (:`ValidData`
                                                              (message `/Game/Characters/Heroes/BI_AbilitiesGeneral.SetInAbilityMontage` (`self.GetAvatarActorFromActorInfo`) false)
                                                              (if (`AbilitySystemBlueprintLibrary.TargetDataHasActor` _data_3)
                                                                (`AbilityTask_ApplyRootMotionMoveToActorForce.ApplyRootMotionMoveToTargetDataActorForce` "None" _data_3 0 0 (0.0 0.0 0.0) "AlignToWorldSpace" 0.2 null null false "MOVE_None" false null null "MaintainLastRootMotionVelocity" (0.0 0.0 0.0) 0.0 true)
                                                                (else
                                                                  (`AbilityTask_ApplyRootMotionMoveToForce.ApplyRootMotionMoveToForce` "None" (+ (`Actor.K2_GetActorLocation` _returnvalue_6) (* (`Actor.GetActorForwardVector` _returnvalue_6) (`KismetMathLibrary.Conv_DoubleToVector` 200.0))) 0.2 false "MOVE_None" false null "MaintainLastRootMotionVelocity"))))))))
                                                    (:`OnActivate`
                                                      (`self.SetCombo`))))
                                                (:`EventReceived`
                                                  (bind _newparam_4 (`self.TraceForTargets` 50.0 50.0 "Hand_L_Punch"))
                                                  (`self.ApplyDamageToTarget` _newparam_4 30.0))))))
                                        (:`OnCompleted`
                                          (`self.K2_EndAbility` :!label _label_4))
                                        (:`OnBlendOut`
                                          (goto _label_4))
                                        (:`OnCancelled`
                                          (goto _label_4))))
                                    (:`ValidData`
                                      (message `/Game/Characters/Heroes/BI_AbilitiesGeneral.SetInAbilityMontage` (`self.GetAvatarActorFromActorInfo`) false)
                                      (if (`AbilitySystemBlueprintLibrary.TargetDataHasActor` _data_2)
                                        (`AbilityTask_ApplyRootMotionMoveToActorForce.ApplyRootMotionMoveToTargetDataActorForce` "None" _data_2 0 0 (0.0 0.0 0.0) "AlignToWorldSpace" 0.2 null null false "MOVE_None" false null null "MaintainLastRootMotionVelocity" (0.0 0.0 0.0) 0.0 true)
                                        (else
                                          (`AbilityTask_ApplyRootMotionMoveToForce.ApplyRootMotionMoveToForce` "None" (+ (`Actor.K2_GetActorLocation` _returnvalue_5) (* (`Actor.GetActorForwardVector` _returnvalue_5) (`KismetMathLibrary.Conv_DoubleToVector` 200.0))) 0.2 false "MOVE_None" false null "MaintainLastRootMotionVelocity"))))))))
                            (:`OnActivate`
                              (`self.SetCombo`))))
                        (:`EventReceived`
                          (bind (_newparam_5 _origin) (`self.TraceForTargets` 50.0 50.0 "Hand_R_Punch"))
                          (`self.ApplyDamageToTarget` _newparam_5 15.0 _origin))))
                    (:`EventReceived`
                      (bind (_newparam_6 _origin_2) (`self.TraceForTargets` 50.0 50.0 "Hand_L_Punch"))
                      (`self.ApplyDamageToTarget` _newparam_6 15.0 _origin_2))))))
            (:`OnCompleted`
              (`self.K2_EndAbility` :!label _label_5))
            (:`OnBlendOut`
              (goto _label_5))
            (:`OnCancelled`
              (goto _label_5))))
        (:`ValidData`
          (message `/Game/Characters/Heroes/BI_AbilitiesGeneral.SetInAbilityMontage` (`self.GetAvatarActorFromActorInfo`) false)
          (if (`AbilitySystemBlueprintLibrary.TargetDataHasActor` _data)
            (`AbilityTask_ApplyRootMotionMoveToActorForce.ApplyRootMotionMoveToTargetDataActorForce` "None" _data 0 0 (0.0 0.0 0.0) "AlignToWorldSpace" 0.2 null null false "MOVE_None" false null null "MaintainLastRootMotionVelocity" (0.0 0.0 0.0) 0.0 true)
            (else
              (`AbilityTask_ApplyRootMotionMoveToForce.ApplyRootMotionMoveToForce` "None" (+ (`Actor.K2_GetActorLocation` _returnvalue_3) (* (`Actor.GetActorForwardVector` _returnvalue_3) (`KismetMathLibrary.Conv_DoubleToVector` 250.0))) 0.3 false "MOVE_None" false null "MaintainLastRootMotionVelocity"))))))
    (:`OnActivate`
      (`AbilitySystemBlueprintLibrary.SendGameplayEventToActor` (`self.GetAvatarActorFromActorInfo`) (struct :`TagName` "Abilities.IntoCombo"))
      (`self.SetCombo`))))

(event `self.K2_OnEndAbility`
  (params (bWasCancelled :type Boolean))
  (bind _returnvalue (`self.GetAvatarActorFromActorInfo`))
  (`self.BP_RemoveGameplayEffectFromOwnerWithHandle` (`self.HephaestusComboGE`))
  (message `/Game/Characters/Heroes/BI_AbilitiesGeneral.SetInAbilityMontage` _returnvalue true)
  (message `/Game/Characters/Heroes/BI_AbilitiesGeneral.SetCanManuallyMove` _returnvalue true))

(fn `ApplyDamageToTarget`
  (params (TargetData :type "GameplayAbilityTargetDataHandle Structure") (Damage :type "Float (double-precision)") (Origin :type "Vector Structure"))
  (bind _returnvalue (`AbilitySystemBlueprintLibrary.AssignTagSetByCallerMagnitude` (`self.MakeOutgoingGameplayEffectSpec` (`self.DamageEffect`) (`KismetMathLibrary.Conv_IntToDouble` (`self.GetAbilityLevel`))) (struct :`TagName` "Damage") Damage))
  (bind _returnvalue_2 (`AbilitySystemBlueprintLibrary.GetEffectContext` _returnvalue))
  (`AbilitySystemBlueprintLibrary.EffectContextSetOrigin` _returnvalue_2 Origin)
  (`self.K2_ApplyGameplayEffectSpecToTarget` _returnvalue TargetData))

(fn `GetCanIntoCombo`
  (returns (CanCombo :type Boolean))
  (`self.ResetCombo`)
  (return (or (`self.bComboQ_A`) (`self.bComboQ_B`))))

(fn `ResetCombo`
  (set `self.bComboQ_A` (`self.bComboQ_B`))
  (set `self.bComboQ_B` false))

(fn `SetCombo`
  (if (`self.bComboQ_A`)
    (if (not (`self.bComboQ_B`))
      (set `self.bComboQ_B` true))
    (else
      (set `self.bComboQ_A` true))))

(fn `TraceForTargets`
  (params (Range :type "Float (double-precision)") (Radius :type "Float (double-precision)") (SocketName :type Name))
  (returns (NewParam :type "GameplayAbilityTargetDataHandle Structure") (Origin :type "Vector Structure"))
  (locals (TargetDataToPass :type "GameplayAbilityTargetDataHandle Structure"))
  (bind _returnvalue (`SceneComponent.GetSocketLocation` (`self.GetOwningComponentFromActorInfo`) SocketName))
  (bind _outhits (`KismetSystemLibrary.SphereTraceMultiForObjects` _returnvalue (+ _returnvalue (* (`Actor.GetActorForwardVector` (`self.GetAvatarActorFromActorInfo`)) (`KismetMathLibrary.Conv_DoubleToVector` Range))) Radius (`|MakeArray` "ObjectTypeQuery7" "ObjectTypeQuery10" :!type "EObjectTypeQuery Enum") false (`|MakeArray` (`self.GetAvatarActorFromActorInfo`)) "None" true (struct :`R` 1.0 :`A` 1.0) (struct :`G` 1.0 :`A` 1.0) 2.0))
  (for _array_element _outhits
    (bind _returnvalue_2 (`AbilitySystemBlueprintLibrary.AppendTargetDataHandle` (`local.TargetDataToPass`) (`AbilitySystemBlueprintLibrary.AbilityTargetDataFromHitResult` _array_element)))
    (set `local.TargetDataToPass` _returnvalue_2))
  (return (`local.TargetDataToPass`) _returnvalue))