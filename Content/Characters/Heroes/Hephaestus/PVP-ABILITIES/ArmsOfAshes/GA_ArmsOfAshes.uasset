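; Gameplay ability for Hephaestus's PVP Arms of Ashes, currently a debug prototype of melee targeting with no damage or effects.
; On activation, WaitTargetData runs the Hephaestus melee target actor, configured for a short, debug-drawn sphere trace from the owner, excluding self and awaiting user confirmation.
; Valid target data has each hit actor's name printed, then the ability ends; cancellation is unhandled.
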(event `self.K2_ActivateAbility`
  (bind (_locationtype _literaltransform _sourceactor _sourcecomponent _sourceability _sourcesocketname) (break `GameplayAbilityTargetingLocationInfo` (`self.MakeTargetLocationInfoFromOwnerActor`)))
  (bind (_asynctaskproxy _data) (`AbilityTask_WaitTargetData.WaitTargetData` "None" "UserConfirmed" "/Game/Characters/Heroes/Hephaestus/PVP-ABILITIES/AutoAttack/BP_Hephaestus_MeleeTA.BP_Hephaestus_MeleeTA_C" 50.0 100.0 (struct :`Name` "PVP_TargetPlayer") true 1 1 true false false (make `GameplayAbilityTargetingLocationInfo` _locationtype _literaltransform _sourceactor _sourcecomponent _sourceability _sourcesocketname) (struct) null (`AbilitySystemBlueprintLibrary.MakeFilterHandle` (make `GameplayTargetDataFilter` null "TDFS_NoSelf") (`self.GetAvatarActorFromActorInfo`)) true)
    (:`ValidData`
      (for _array_element (`AbilitySystemBlueprintLibrary.GetActorsFromTargetData` _data)
        (`KismetSystemLibrary.PrintString` (`KismetSystemLibrary.GetObjectName` _array_element)))
      (`self.K2_EndAbility`))))