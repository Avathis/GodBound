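; Gameplay ability for Hephaestus's parry, a held frontal block.
; On activation it applies the frontal parry effect, disables manual movement and plays the block montage.
; While active, each applied effect from a Damage-tagged source adds an overheat effect to the owner.
; Input release or a short timeout ends the ability, which restores movement and removes the parry effect.
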(event `self.K2_ActivateAbility`
  (`self.K2_CommitAbility`)
  (bind _returnvalue (`self.BP_ApplyGameplayEffectToOwner` "/Game/Characters/Heroes/Hephaestus/PVP-ABILITIES/Parry/GE_ParryFrontal.GE_ParryFrontal_C"))
  (bind _output_get (set `self.FronatlParryGE` _returnvalue))
  (`AbilityTask_WaitGameplayEffectRemoved.WaitForGameplayEffectRemoved` _output_get
    (:`then`
      (message `/Game/Characters/Heroes/BI_AbilitiesGeneral.SetCanManuallyMove` (`self.GetAvatarActorFromActorInfo`) false)
      (`AbilityTask_PlayMontageAndWait.CreatePlayMontageAndWaitProxy` "None" "/Game/Characters/SharedAnimations/MeleeAnimations/FighterAnimations/Locomotion/Walk/Combat/Montage_HephaestusBlock.Montage_HephaestusBlock"
        (:`then`
          (`AbilityTask_WaitGameplayEffectApplied_Self.WaitGameplayEffectAppliedToSelf` (struct) (make `GameplayTagRequirements` (struct :`GameplayTags` (struct :`(TagName` "Damage")))) (struct) false null true
            (:`then`
              (`AbilityTask_WaitInputRelease.WaitInputRelease` false
                (:`then`
                  (`GameplayTask_WaitDelay.TaskWaitDelay` null 1.5
                    (:`OnFinish`
                      (`self.K2_EndAbility`))))
                (:`OnRelease`
                  (`self.K2_EndAbility`))))
            (:`OnApplied`
              (`self.BP_ApplyGameplayEffectToOwner` "/Game/Characters/Heroes/Hephaestus/PVP-ABILITIES/Parry/GE_OverHeatAdditive.GE_OverHeatAdditive_C"))))))))

(event `self.K2_OnEndAbility`
  (params (bWasCancelled :type Boolean))
  (message `/Game/Characters/Heroes/BI_AbilitiesGeneral.SetCanManuallyMove` (`self.GetAvatarActorFromActorInfo`) true)
  (`self.BP_RemoveGameplayEffectFromOwnerWithHandle` (`self.FronatlParryGE`)))