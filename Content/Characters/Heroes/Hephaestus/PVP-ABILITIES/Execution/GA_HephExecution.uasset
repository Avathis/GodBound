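; Hephaestus execution gameplay ability, granted by a gameplay effect whose causer is the execution target.
; Root motion moves Hephaestus in front of the target, then he faces it and sends it an Abilities.Execution event.
; A cinematic camera animation plays alongside the execute montage until the montage ends or a Finished event arrives.
; Ending restores camera and montage state, removes the granting effect and signals Cancelled if cancelled.
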(event `self.K2_ActivateAbility`
  (bind _returnvalue (`self.GetAvatarActorFromActorInfo`))
  (bind (_owneractor _avataractor _playercontroller) (break `GameplayAbilityActorInfo` (`self.GetActorInfo`)))
  (bind _returnvalue_2 (`AbilitySystemBlueprintLibrary.EffectContextGetEffectCauser` (`self.GetGrantedByEffectContext`)))
  (`self.K2_CommitAbility`)
  (message `/Game/Characters/Heroes/BI_AbilitiesGeneral.SetInAbilityMontage` _returnvalue false)
  (`AbilityTask_ApplyRootMotionMoveToActorForce.ApplyRootMotionMoveToActorForce` "None" _returnvalue_2 (85.0 0.0 0.0) "AlignToTargetForward" 1.0 null null false "MOVE_None" true null null "SetVelocity"
    (:`OnFinished`
      (`Actor.K2_SetActorRotation` _returnvalue (`KismetMathLibrary.FindLookAtRotation` (`Actor.K2_GetActorLocation` _returnvalue) (`Actor.K2_GetActorLocation` _returnvalue_2)) false)
      (`AbilitySystemBlueprintLibrary.SendGameplayEventToActor` (`AbilitySystemBlueprintLibrary.EffectContextGetEffectCauser` (`self.GetGrantedByEffectContext`)) (struct :`TagName` "Abilities.Execution") (make `GameplayEventData` (struct) (`self.GetAvatarActorFromActorInfo`)))
      (message `/Game/Characters/Heroes/BI_AbilitiesGeneral.SwitchToCinematicCamera` _avataractor true)
      (`CameraAnimationCameraModifier.PlayCameraAnimation` (`CameraAnimationCameraModifier.GetCameraAnimationCameraModifierFromPlayerController` _playercontroller) "/Game/Characters/Heroes/Hephaestus/PVP-ABILITIES/Execution/CamS_HephaestusExecution.CamS_HephaestusExecution" (make `CameraAnimationParams` 1.0))
      (`AbilityTask_PlayMontageAndWait.CreatePlayMontageAndWaitProxy` "None" "/Game/Characters/Heroes/Hephaestus/PVP-ABILITIES/Execution/Hephaestus_Execute.Hephaestus_Execute"
        (:`then`
          (`AbilityAsync_WaitGameplayEvent.WaitGameplayEventToActor` _avataractor (struct :`TagName` "Abilities.Execution.Finished")
            (:`EventReceived`
              (`self.K2_EndAbility`))))
        (:`OnCompleted`
          (`self.K2_EndAbility` :!label _label))
        (:`OnBlendOut`
          (goto _label))
        (:`OnInterrupted`
          (goto _label))
        (:`OnCancelled`
          (goto _label))))))

(event `self.K2_OnEndAbility`
  (params (bWasCancelled :type Boolean))
  (bind _returnvalue (`self.GetAvatarActorFromActorInfo`))
  (if bWasCancelled
    (`AbilitySystemBlueprintLibrary.SendGameplayEventToActor` _returnvalue (struct :`TagName` "Abilities.Execution.Cancelled")))
  (message `/Game/Characters/Heroes/BI_AbilitiesGeneral.SetInAbilityMontage` _returnvalue true)
  (`self.RemoveGrantedByEffect`)
  (message `/Game/Characters/Heroes/BI_AbilitiesGeneral.SwitchToCinematicCamera` _returnvalue false)
  (`CameraAnimationCameraModifier.StopAllCameraAnimations` (`CameraAnimationCameraModifier.GetCameraAnimationCameraModifierFromPlayerController` (`.PlayerController` (break `GameplayAbilityActorInfo` (`self.GetActorInfo`)))) false))