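; Hephaestus's PowerJump gameplay ability, an unfinished prototype that launches the owner toward a hard-coded world location.
; On activation it commits, computes a suggested toss velocity with debug drawing, and uses it as the direction of a timed root motion constant force.
; The ability ends when that force finishes.
; Disconnected experiments remain, including a camera-trace-targeted jump force and move-to, radial and move-to-actor root motion forces.
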(event `self.K2_ActivateAbility`
  (`self.K2_CommitAbility`)
  (bind _tossvelocity (`GameplayStatics.BlueprintSuggestProjectileVelocity` (`Actor.K2_GetActorLocation` (`.OwnerActor` (break `GameplayAbilityActorInfo` (`self.GetActorInfo`)))) (`KismetMathLibrary.MakeVector` -1105.0 -565.0 213.0) 1200.0 0.0 "DoNotTrace" 0.0 false true))
  (`AbilityTask_ApplyRootMotionConstantForce.ApplyRootMotionConstantForce` "None" _tossvelocity 1200.0 1.0 false null "MaintainLastRootMotionVelocity"
    (:`OnFinish`
      (`self.K2_EndAbility`))))