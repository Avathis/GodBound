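; Test Gameplay Ability for Hephaestus's Power Jump, a targeted leap that deals area damage on impact.
; A player-confirmed placement target actor supplies target data, then the ability commits and launches the character along a suggested projectile arc to that point.
; The first overlap triggers a sphere query that applies a placeholder damage effect and ends the ability.
; Debug drawing and prints remain, and the no-controller branch never ends the ability.
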(event `self.K2_ActivateAbility`
  (bind (_locationtype _literaltransform _sourceactor _sourcecomponent _sourceability _sourcesocketname) (break `GameplayAbilityTargetingLocationInfo` (`self.MakeTargetLocationInfoFromOwnerActor`)))
  (`/Engine/EditorBlueprintResources/StandardMacros.IsValid` (`.PlayerController` (break `GameplayAbilityActorInfo` (`self.GetActorInfo`)))
    (:`Is Valid`
      (bind (_asynctaskproxy _data) (`AbilityTask_WaitTargetData.WaitTargetData` "None" "UserConfirmed" "/Game/Actors/TargetActors/BP_TestingActorPlacement.BP_TestingActorPlacement_C" null null 0.0 0.0 999999.0 (struct :`Name` "NoCollision") true (make `GameplayAbilityTargetingLocationInfo` _locationtype _literaltransform _sourceactor _sourcecomponent _sourceability _sourcesocketname) (struct) null (struct) true)
        (:`ValidData`
          (if true
            (bind _returnvalue (`self.K2_CommitAbility`))
            (if _returnvalue
              (bind (_bblockinghit _binitialoverlap _time _distance _location _impactpoint _normal _impactnormal _physmat _hitactor _hitcomponent _hitbonename _bonename _hititem _elementindex _faceindex _tracestart) (`GameplayStatics.BreakHitResult` (`AbilitySystemBlueprintLibrary.GetHitResultFromTargetData` _data)))
              (bind _outlaunchvelocity (`GameplayStatics.SuggestProjectileVelocity_CustomArc` _tracestart _location))
              (bind _asgb_playable_character (cast `GB_PlayableCharacter` (`self.GetOwningActorFromActorInfo`)))
              (`Character.LaunchCharacter` _asgb_playable_character _outlaunchvelocity true true)
              (`AbilityTask_WaitOverlap.WaitForOverlap`
                (:`OnOverlap`
                  (bind _returnvalue_2 (`Actor.K2_GetActorLocation` _asgb_playable_character))
                  (bind _outactors (`KismetSystemLibrary.SphereOverlapActors` _returnvalue_2 200.0 (`|MakeArray` "ObjectTypeQuery8" "ObjectTypeQuery6" :!type "EObjectTypeQuery Enum")))
                  (`KismetSystemLibrary.DrawDebugSphere` _returnvalue_2 200.0 12 (struct :`R` 1.0 :`G` 1.0 :`B` 1.0 :`A` 1.0) 5.0 1.0)
                  (`self.BP_ApplyGameplayEffectToTarget` (`AbilitySystemBlueprintLibrary.AbilityTargetDataFromActorArray` _outactors) "/Game/Effects/BP_DAMAGE_REMOVEAFTER.BP_DAMAGE_REMOVEAFTER_C")
                  (`self.K2_EndAbility`)
                  (`KismetSystemLibrary.PrintString` "Yes")))
              (else
                (`self.K2_CancelAbility` :!label _label)))
            (else
              (goto _label))))
        (:`Cancelled`
          (`KismetSystemLibrary.PrintString` "Hello")
          (goto _label))))
    (:`Is Not Valid`
      (`KismetSystemLibrary.PrintString` "No it is not"))))