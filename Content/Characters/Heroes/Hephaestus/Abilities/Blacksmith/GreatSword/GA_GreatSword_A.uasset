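; Gameplay ability for a Hephaestus Blacksmith greatsword slash that plays a slowed heavy-slash montage driven by gameplay events.
; Events spawn a sword on the right-hand socket, trigger debug-drawn sphere overlaps that apply damage, and destroy the sword.
; An ignore list prevents repeat hits.
; After despawn, an IntoCombo event grants a combo effect; ending the ability clears the list and removes LightSword Swing1-tagged effects.
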(event `self.K2_ActivateAbility`
  (bind (_owneractor _avataractor _playercontroller _abilitysystemcomponent _skeletalmeshcomponent) (break `GameplayAbilityActorInfo` (`self.GetActorInfo`)))
  (bind _returnvalue (`self.K2_CommitAbility`))
  (if _returnvalue
    (`AbilityTask_PlayMontageAndWait.CreatePlayMontageAndWaitProxy` "None" "/Game/Characters/Heroes/Hephaestus/Animations/Abilities/InPlace/Montage_Hephaestus_HeavySlashD.Montage_Hephaestus_HeavySlashD" 0.5
      (:`then`
        (`AbilityTask_WaitGameplayEvent.WaitGameplayEvent` (struct :`TagName` "Abilities.Blacksmith.SpawnWeapon") null
          (:`EventReceived`
            (bind (_asynctaskproxy _spawnedactor) (`GameplayTask_SpawnActor.SpawnActor` null (`SceneComponent.GetSocketLocation` _skeletalmeshcomponent "Hand_R_MeleeSocket") (`SceneComponent.GetSocketRotation` _skeletalmeshcomponent "Hand_R_MeleeSocket") "/Game/Actors/Weapons/BP_B_ReplaceableGSowrd.BP_B_ReplaceableGSowrd_C" false null)
              (:`Success`
                (bind _output_get (set `self.Spawned Sword` _spawnedactor))
                (`Actor.K2_AttachToComponent` _output_get _skeletalmeshcomponent "Hand_R_MeleeSocket" "SnapToTarget" "SnapToTarget" "SnapToTarget" false)
                (`AbilityTask_WaitGameplayEvent.WaitGameplayEvent` (struct :`TagName` "Abilities.Blacksmith.DespawnWeapon") null
                  (:`then`
                    (`AbilityTask_WaitGameplayEvent.WaitGameplayEvent` (struct :`TagName` "Abilities.Blacksmith.Slash.Trace") null
                      (:`EventReceived`
                        (bind _newparam (message `/Game/Interfaces/BPI_AbilityInterface.GetSceneComponentForTrace` (`self.Spawned Sword`)))
                        (bind _returnvalue_2 (`SceneComponent.K2_GetComponentLocation` _newparam))
                        (bind (_outactors _returnvalue_3) (`KismetSystemLibrary.SphereOverlapActors` _returnvalue_2 75.0 (`|MakeArray` "ObjectTypeQuery6" "ObjectTypeQuery8" :!type "EObjectTypeQuery Enum") null (`self.Actors to Ignore`)))
                        (if _returnvalue_3
                          (`KismetSystemLibrary.DrawDebugSphere` _returnvalue_2 75.0 12 (struct :`R` 1.0 :`B` 0.050213 :`A` 1.0) 2.0 1.0)
                          (else
                            (`KismetSystemLibrary.DrawDebugSphere` _returnvalue_2 75.0 12 (struct :`R` 1.0 :`G` 1.0 :`B` 1.0 :`A` 1.0) 2.0 1.0)))
                        (for _array_element _outactors
                          (`KismetArrayLibrary.Array_Add` (`self.Actors to Ignore`) _array_element))
                        (`self.BP_ApplyGameplayEffectToTarget` (`AbilitySystemBlueprintLibrary.AbilityTargetDataFromActorArray` _outactors) "/Game/Effects/BP_DAMAGE_REMOVEAFTER.BP_DAMAGE_REMOVEAFTER_C"))))
                  (:`EventReceived`
                    (`Actor.K2_DestroyActor` (`self.Spawned Sword`))
                    (`AbilityTask_WaitGameplayEvent.WaitGameplayEvent` (struct :`TagName` "Abilities.IntoCombo") null
                      (:`EventReceived`
                        (`self.BP_ApplyGameplayEffectToOwner` "/Game/Characters/Heroes/Hephaestus/Abilities/Blacksmith/ComboEffects/GE_SwordCombo1.GE_SwordCombo1_C")
                        (`KismetSystemLibrary.PrintString` "Hello"))))))
              (:`DidNotSpawn`
                (`KismetSystemLibrary.PrintString` "Didn'TSpawn")
                (`self.K2_EndAbility`))))))
      (:`OnCompleted`
        (`self.K2_EndAbility` :!label _label))
      (:`OnBlendOut`
        (goto _label))
      (:`OnInterrupted`
        (goto _label))
      (:`OnCancelled`
        (goto _label)))
    (else
      (`self.K2_CancelAbility`))))

(event `self.K2_OnEndAbility`
  (params (bWasCancelled :type Boolean))
  (`KismetArrayLibrary.Array_Clear` (`self.Actors to Ignore`))
  (`self.BP_RemoveGameplayEffectFromOwnerWithGrantedTags` (struct :`GameplayTags` (struct :`(TagName` "Abilities.Blacksmith.LightSword.Swing1")))))