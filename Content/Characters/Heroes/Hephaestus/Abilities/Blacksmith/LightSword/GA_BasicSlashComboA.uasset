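; Gameplay ability for Hephaestus's basic combo slash, which plays a montage with a spawned sword attached to the right-hand socket.
; The sword spawns right after the montage starts, without waiting for the SpawnWeapon event, and is destroyed on DespawnWeapon or cancellation.
; Activation commits the ability and clears IntoCombo effects.
; The Slash.Trace handler only validates the sword; overlap and damage logic is disconnected.
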(event `self.K2_ActivateAbility`
  (bind (_owneractor _avataractor _playercontroller _abilitysystemcomponent _skeletalmeshcomponent) (break `GameplayAbilityActorInfo` (`self.GetActorInfo`)))
  (bind _returnvalue (`self.K2_CommitAbility`))
  (`self.BP_RemoveGameplayEffectFromOwnerWithGrantedTags` (struct :`GameplayTags` (struct :`(TagName` "Abilities.IntoCombo"))))
  (if _returnvalue
    (`AbilityTask_PlayMontageAndWait.CreatePlayMontageAndWaitProxy` "Attack" "/Game/Characters/Heroes/Hephaestus/Animations/Abilities/InPlace/Montage_Hephaestus_ComboSlash.Montage_Hephaestus_ComboSlash" 1.0 "None" false
      (:`then`
        (`AbilityTask_WaitGameplayEvent.WaitGameplayEvent` (struct :`TagName` "Abilities.Blacksmith.SpawnWeapon") null true
          (:`then`
            (bind (_asynctaskproxy _spawnedactor) (`GameplayTask_SpawnActor.SpawnActor` null (`SceneComponent.GetSocketLocation` _skeletalmeshcomponent "Hand_R_MeleeSocket") (`SceneComponent.GetSocketRotation` _skeletalmeshcomponent "Hand_R_MeleeSocket") "/Game/Actors/Weapons/BP_B_ReplaceableSowrd.BP_B_ReplaceableSowrd_C" false null)
              (:`Success`
                (bind _output_get (set `self.SpawnedSword` _spawnedactor))
                (`Actor.K2_AttachToComponent` _output_get _skeletalmeshcomponent "Hand_R_MeleeSocket" "SnapToTarget" "SnapToTarget" "SnapToTarget" false)
                (`AbilityTask_WaitGameplayEvent.WaitGameplayEvent` (struct :`TagName` "Abilities.Blacksmith.DespawnWeapon") null true
                  (:`then`
                    (`AbilityTask_WaitGameplayEvent.WaitGameplayEvent` (struct :`TagName` "Abilities.Blacksmith.Slash.Trace") null
                      (:`EventReceived`
                        (`/Engine/EditorBlueprintResources/StandardMacros.IsValid` (`self.SpawnedSword`)))))
                  (:`EventReceived`
                    (`Actor.K2_DestroyActor` _output_get))))
              (:`DidNotSpawn`
                (`KismetSystemLibrary.PrintString` "Didn'TSpawn")
                (`self.K2_EndAbility`))))))
      (:`OnCompleted`
        (`self.K2_EndAbility` :!label _label))
      (:`OnBlendOut`
        (goto _label))
      (:`OnInterrupted`
        (goto _label))
      (:`OnCancelled`
        (goto _label)))
    (else
      (`self.K2_CancelAbility`))))

(event `self.K2_OnEndAbility`
  (params (bWasCancelled :type Boolean))
  (bind _spawnedsword (`self.SpawnedSword`))
  (`KismetArrayLibrary.Array_Clear` (`self.ActorsToIgnore`))
  (`/Engine/EditorBlueprintResources/StandardMacros.IsValid` _spawnedsword
    (:`Is Valid`
      (if bWasCancelled
        (`Actor.K2_DestroyActor` _spawnedsword)))))

(fn `GetCombatMode`
  (returns (NewParam :type "EHephaestusSet Enum"))
  (return "EHS_OOC"))

(fn `GetSceneComponentForTrace`
  (returns (NewParam :type "SceneComponent Object Reference"))
  (return null))