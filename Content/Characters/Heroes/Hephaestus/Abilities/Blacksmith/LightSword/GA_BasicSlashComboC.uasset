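; Gameplay ability for Hephaestus's basic slash combo, playing the ComboSlash3 montage after removing effects granting the IntoCombo tag.
; Montage gameplay events spawn a sword on the right-hand socket, trigger sphere-overlap traces from it, and destroy it.
; Traces apply a damage effect, ignore actors already hit until the ability ends, and draw debug spheres.
; Cancellation also destroys the sword.
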(event `self.K2_ActivateAbility`
  (bind _spawnedsword (`self.SpawnedSword`))
  (bind (_owneractor _avataractor _playercontroller _abilitysystemcomponent _skeletalmeshcomponent) (break `GameplayAbilityActorInfo` (`self.GetActorInfo`)))
  (bind _returnvalue (`self.K2_CommitAbility`))
  (`self.BP_RemoveGameplayEffectFromOwnerWithGrantedTags` (struct :`GameplayTags` (struct :`(TagName` "Abilities.IntoCombo"))))
  (if _returnvalue
    (`AbilityTask_PlayMontageAndWait.CreatePlayMontageAndWaitProxy` "Attack" "/Game/Characters/Heroes/Hephaestus/Animations/Abilities/InPlace/Montage_Hephaestus_ComboSlash3.Montage_Hephaestus_ComboSlash3" 1.0 "None" false
      (:`then`
        (`AbilityTask_WaitGameplayEvent.WaitGameplayEvent` (struct :`TagName` "Abilities.Blacksmith.SpawnWeapon") null true
          (:`then`
            (bind (_asynctaskproxy _spawnedactor) (`GameplayTask_SpawnActor.SpawnActor` null (`SceneComponent.GetSocketLocation` _skeletalmeshcomponent "Hand_R_MeleeSocket") (`SceneComponent.GetSocketRotation` _skeletalmeshcomponent "Hand_R_MeleeSocket") "/Game/Actors/Weapons/BP_B_ReplaceableSowrd.BP_B_ReplaceableSowrd_C" false null)
              (:`Success`
                (bind _output_get (set `self.SpawnedSword` _spawnedactor))
                (`Actor.K2_AttachToComponent` _output_get _skeletalmeshcomponent "Hand_R_MeleeSocket" "SnapToTarget" "SnapToTarget" "SnapToTarget" false)
                (`AbilityTask_WaitGameplayEvent.WaitGameplayEvent` (struct :`TagName` "Abilities.Blacksmith.DespawnWeapon") null true
                  (:`then`
                    (`AbilityTask_WaitGameplayEvent.WaitGameplayEvent` (struct :`TagName` "Abilities.Blacksmith.Slash.Trace") null
                      (:`EventReceived`
                        (`/Engine/EditorBlueprintResources/StandardMacros.IsValid` _spawnedsword
                          (:`Is Valid`
                            (bind _newparam (message `/Game/Interfaces/BPI_AbilityInterface.GetSceneComponentForTrace` _spawnedsword))
                            (bind _returnvalue_2 (`SceneComponent.K2_GetComponentLocation` _newparam))
                            (bind (_outactors _returnvalue_3) (`KismetSystemLibrary.SphereOverlapActors` _returnvalue_2 75.0 (`|MakeArray` "ObjectTypeQuery6" "ObjectTypeQuery8" :!type "EObjectTypeQuery Enum") null (`self.ActorsToIgnore`)))
                            (if _returnvalue_3
                              (`KismetSystemLibrary.DrawDebugSphere` _returnvalue_2 75.0 12 (struct :`R` 1.0 :`B` 0.050213 :`A` 1.0) 2.0 1.0)
                              (else
                                (`KismetSystemLibrary.DrawDebugSphere` _returnvalue_2 75.0 12 (struct :`R` 1.0 :`G` 1.0 :`B` 1.0 :`A` 1.0) 2.0 1.0)))
                            (for _array_element _outactors
                              (`KismetArrayLibrary.Array_Add` (`self.ActorsToIgnore`) _array_element))
                            (`self.BP_ApplyGameplayEffectToTarget` (`AbilitySystemBlueprintLibrary.AbilityTargetDataFromActorArray` _outactors) "/Game/Effects/BP_DAMAGE_REMOVEAFTER.BP_DAMAGE_REMOVEAFTER_C"))))))
                  (:`EventReceived`
                    (`Actor.K2_DestroyActor` _output_get))))
              (:`DidNotSpawn`
                (`KismetSystemLibrary.PrintString` "Didn'TSpawn")
                (`self.K2_EndAbility`))))))
      (:`OnCompleted`
        (`self.K2_EndAbility`)))
    (else
      (`self.K2_CancelAbility`))))

(event `self.K2_OnEndAbility`
  (params (bWasCancelled :type Boolean))
  (bind _spawnedsword (`self.SpawnedSword`))
  (`KismetArrayLibrary.Array_Clear` (`self.ActorsToIgnore`))
  (`/Engine/EditorBlueprintResources/StandardMacros.IsValid` _spawnedsword
    (:`Is Valid`
      (if bWasCancelled
        (`Actor.K2_DestroyActor` _spawnedsword)))))

(fn `GetCombatMode`
  (returns (NewParam :type "EHephaestusSet Enum"))
  (return "EHS_OOC"))

(fn `GetSceneComponentForTrace`
  (returns (NewParam :type "SceneComponent Object Reference"))
  (return null))