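; Gameplay Ability for Hephaestus's Blacksmith light sword attack, a slash combo of up to three montages.
; Montage gameplay events spawn a sword attached to the right-hand socket and destroy it.
; Combo2 events open input waits that chain the next montage through nested ability tasks.
; The sphere-overlap damage logic is disconnected and the Slash.Trace event has no handler, so this graph applies no damage.
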(event `self.K2_ActivateAbility`
  (bind _spawnedsword (`self.SpawnedSword`))
  (bind _spawnedsword_2 (`self.SpawnedSword`))
  (bind (_owneractor _avataractor _playercontroller _abilitysystemcomponent _skeletalmeshcomponent) (break `GameplayAbilityActorInfo` (`self.GetActorInfo`)))
  (bind (_owneractor_2 _avataractor_2 _playercontroller_2 _abilitysystemcomponent_2 _skeletalmeshcomponent_2) (break `GameplayAbilityActorInfo` (`self.GetActorInfo`)))
  (bind _returnvalue (`SceneComponent.GetSocketLocation` _skeletalmeshcomponent "Hand_R_MeleeSocket"))
  (bind _returnvalue_2 (`SceneComponent.GetSocketRotation` _skeletalmeshcomponent "Hand_R_MeleeSocket"))
  (bind _returnvalue_3 (`self.K2_CommitAbility`))
  (if _returnvalue_3
    (`AbilityTask_PlayMontageAndWait.CreatePlayMontageAndWaitProxy` "Attack" "/Game/Characters/Heroes/Hephaestus/Animations/Abilities/InPlace/Montage_Hephaestus_ComboSlash.Montage_Hephaestus_ComboSlash" 1.0 "None" false
      (:`then`
        (`AbilityTask_WaitGameplayEvent.WaitGameplayEvent` (struct :`TagName` "Abilities.Blacksmith.SpawnWeapon") null true
          (:`then`
            (bind (_asynctaskproxy _spawnedactor) (`GameplayTask_SpawnActor.SpawnActor` null (`SceneComponent.GetSocketLocation` _skeletalmeshcomponent_2 "Hand_R_MeleeSocket") (`SceneComponent.GetSocketRotation` _skeletalmeshcomponent_2 "Hand_R_MeleeSocket") "/Game/Actors/Weapons/BP_B_ReplaceableSowrd.BP_B_ReplaceableSowrd_C" false null)
              (:`Success`
                (bind _output_get (set `self.SpawnedSword` _spawnedactor))
                (`Actor.K2_AttachToComponent` _output_get _skeletalmeshcomponent_2 "Hand_R_MeleeSocket" "SnapToTarget" "SnapToTarget" "SnapToTarget" false)
                (`AbilityTask_WaitGameplayEvent.WaitGameplayEvent` (struct :`TagName` "Abilities.Blacksmith.DespawnWeapon") null true
                  (:`then`
                    (`AbilityTask_WaitGameplayEvent.WaitGameplayEvent` (struct :`TagName` "Abilities.Blacksmith.Slash.Trace") null
                      (:`then`
                        (`AbilityTask_WaitGameplayEvent.WaitGameplayEvent` (struct :`TagName` "Abilities.Blacksmith.Slash.Combo2") null true
                          (:`EventReceived`
                            (`AbilityTask_WaitInputPress.WaitInputPress` true
                              (:`OnPress`
                                (`KismetArrayLibrary.Array_Clear` (`self.ActorsToIgnore`))
                                (`AbilityTask_PlayMontageAndWait.CreatePlayMontageAndWaitProxy` "Attack" (`self.Montage to Play`) 1.0 "IntoCombo" false
                                  (:`then`
                                    (`AbilityTask_WaitGameplayEvent.WaitGameplayEvent` (struct :`TagName` "Abilities.Blacksmith.SpawnWeapon") null true
                                      (:`EventReceived`
                                        (bind (_asynctaskproxy_2 _spawnedactor_2) (`GameplayTask_SpawnActor.SpawnActor` null _returnvalue _returnvalue_2 "/Game/Actors/Weapons/BP_B_ReplaceableSowrd.BP_B_ReplaceableSowrd_C" false null)
                                          (:`Success`
                                            (bind _output_get_2 (set `self.SpawnedSword` _spawnedactor_2))
                                            (`Actor.K2_AttachToComponent` _output_get_2 _skeletalmeshcomponent "Hand_R_MeleeSocket" "SnapToTarget" "SnapToTarget" "SnapToTarget" false)
                                            (`AbilityTask_WaitGameplayEvent.WaitGameplayEvent` (struct :`TagName` "Abilities.Blacksmith.DespawnWeapon") null true
                                              (:`then`
                                                (`AbilityTask_WaitGameplayEvent.WaitGameplayEvent` (struct :`TagName` "Abilities.Blacksmith.Slash.Combo2") null true
                                                  (:`EventReceived`
                                                    (`AbilityTask_WaitInputPress.WaitInputPress` true
                                                      (:`OnPress`
                                                        (`KismetArrayLibrary.Array_Clear` (`self.ActorsToIgnore`))
                                                        (`AbilityTask_PlayMontageAndWait.CreatePlayMontageAndWaitProxy` "Attack" "/Game/Characters/Heroes/Hephaestus/Animations/Abilities/InPlace/Montage_Hephaestus_ComboSlash3.Montage_Hephaestus_ComboSlash3" 1.0 "None" false
                                                          (:`then`
                                                            (`AbilityTask_WaitGameplayEvent.WaitGameplayEvent` (struct :`TagName` "Abilities.Blacksmith.SpawnWeapon") null true
                                                              (:`EventReceived`
                                                                (bind (_asynctaskproxy_3 _spawnedactor_3) (`GameplayTask_SpawnActor.SpawnActor` null _returnvalue _returnvalue_2 "/Game/Actors/Weapons/BP_B_ReplaceableSowrd.BP_B_ReplaceableSowrd_C" false null)
                                                                  (:`Success`
                                                                    (bind _output_get_3 (set `self.SpawnedSword` _spawnedactor_3))
                                                                    (`Actor.K2_AttachToComponent` _output_get_3 _skeletalmeshcomponent "Hand_R_MeleeSocket" "SnapToTarget" "SnapToTarget" "SnapToTarget" false)
                                                                    (`AbilityTask_WaitGameplayEvent.WaitGameplayEvent` (struct :`TagName` "Abilities.Blacksmith.DespawnWeapon") null true
                                                                      (:`EventReceived`
                                                                        (`/Engine/EditorBlueprintResources/StandardMacros.IsValid` _spawnedsword_2
                                                                          (:`Is Valid`
                                                                            (`Actor.K2_DestroyActor` _spawnedsword_2))
                                                                          (:`Is Not Valid`
                                                                            (`KismetSystemLibrary.PrintString` "Nothing to delete"))))))
                                                                  (:`DidNotSpawn`
                                                                    (`KismetSystemLibrary.PrintString` "Did not spawn"))))))
                                                          (:`OnCompleted`
                                                            (`self.K2_EndAbility`))))))))
                                              (:`EventReceived`
                                                (`/Engine/EditorBlueprintResources/StandardMacros.IsValid` _spawnedsword
                                                  (:`Is Valid`
                                                    (`Actor.K2_DestroyActor` _spawnedsword))
                                                  (:`Is Not Valid`
                                                    (`KismetSystemLibrary.PrintString` "Nothing to delete"))))))
                                          (:`DidNotSpawn`
                                            (`KismetSystemLibrary.PrintString` "Did not spawn"))))))
                                  (:`OnCompleted`
                                    (`self.K2_EndAbility`))))))))))
                  (:`EventReceived`
                    (`Actor.K2_DestroyActor` _output_get))))
              (:`DidNotSpawn`
                (`KismetSystemLibrary.PrintString` "Didn'TSpawn")
                (`self.K2_EndAbility`))))))
      (:`OnCompleted`
        (`self.K2_EndAbility`)))
    (else
      (`self.K2_CancelAbility`))))

(event `self.K2_OnEndAbility`
  (params (bWasCancelled :type Boolean))
  (bind _spawnedsword (`self.SpawnedSword`))
  (`KismetArrayLibrary.Array_Clear` (`self.ActorsToIgnore`))
  (`/Engine/EditorBlueprintResources/StandardMacros.IsValid` _spawnedsword
    (:`Is Valid`
      (if bWasCancelled
        (`Actor.K2_DestroyActor` _spawnedsword)))))

(fn `GetCombatMode`
  (returns (NewParam :type "EHephaestusSet Enum"))
  (return "EHS_OOC"))

(fn `GetSceneComponentForTrace`
  (returns (NewParam :type "SceneComponent Object Reference"))
  (return null))