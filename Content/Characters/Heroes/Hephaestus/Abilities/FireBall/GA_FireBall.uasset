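; Hephaestus's fireball gameplay ability, which applies an overheat effect to the owner and throws a physics-driven fireball.
; It spawns BP_FireBall1 attached to the hand socket with gravity off, then plays the throw montage.
; A release gameplay event detaches it, restores gravity and launches it toward the camera trace point using a suggested toss velocity.
; Cancelling before release destroys the fireball, and a debug line of the aim is drawn.
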(event `self.K2_ActivateAbility`
  (`self.K2_CommitAbility`)
  (`self.BP_ApplyGameplayEffectToOwner` "/Game/Effects/Utility/BP_OverHeatEffect.BP_OverHeatEffect_C")
  (bind _asgb_playable_character (cast `GB_PlayableCharacter` (`.OwnerActor` (break `GameplayAbilityActorInfo` (`self.GetActorInfo`))))
    (:`then`
      (bind _mesh (`Character.Mesh` _asgb_playable_character))
      (bind (_asynctaskproxy _spawnedactor) (`GameplayTask_SpawnActor.SpawnActor` null (`SceneComponent.GetSocketLocation` _mesh "Hand_release") (`SceneComponent.GetSocketRotation` _mesh "Hand_release") "/Game/Actors/Projectiles/BP_FireBall1.BP_FireBall1_C" false null)
        (:`Success`
          (set `self.bIsReleased` false)
          (bind _asbp_fire_ball_1 (cast `/Game/Actors/Projectiles/BP_FireBall1` _spawnedactor))
          (bind _staticmesh (`Projectile.StaticMesh` _asbp_fire_ball_1))
          (`PrimitiveComponent.SetEnableGravity` _staticmesh false)
          (`Actor.K2_AttachToComponent` _spawnedactor (`Character.Mesh` _asgb_playable_character) "Hand_release" "KeepWorld" "KeepWorld" "KeepWorld" true)
          (`AbilityTask_PlayMontageAndWait.CreatePlayMontageAndWaitProxy` "None" "/Game/Characters/Heroes/Hephaestus/Animations/Abilities/InPlace/Montage_Hephaestus_R_Fireball.Montage_Hephaestus_R_Fireball"
            (:`then`
              (`AbilityTask_WaitGameplayEvent.WaitGameplayEvent` (struct :`TagName` "Damage.Fire.Fireball.Release") null
                (:`EventReceived`
                  (set `self.bIsReleased` true)
                  (bind _returnvalue (`GB_Character.TraceFromCamera` _asgb_playable_character))
                  (bind _returnvalue_2 (`SceneComponent.GetSocketLocation` (`Character.Mesh` _asgb_playable_character) "Hand_release"))
                  (`KismetSystemLibrary.DrawDebugLine` _returnvalue_2 _returnvalue (struct :`R` 1.0 :`B` 0.078579 :`A` 1.0) 5.0)
                  (`/Engine/EditorBlueprintResources/StandardMacros.IsValid` _asbp_fire_ball_1
                    (:`Is Valid`
                      (`Actor.K2_DetachFromActor` _asbp_fire_ball_1 "KeepWorld" "KeepWorld" "KeepWorld")
                      (`/Engine/EditorBlueprintResources/StandardMacros.IsValid` _staticmesh
                        (:`Is Valid`
                          (`PrimitiveComponent.SetEnableGravity` _staticmesh true)
                          (bind _tossvelocity (`GameplayStatics.BlueprintSuggestProjectileVelocity` _returnvalue_2 _returnvalue 1500.0 0.0 "DoNotTrace" 32.0))
                          (`PrimitiveComponent.SetAllPhysicsLinearVelocity` _staticmesh _tossvelocity true))))))))
            (:`OnCompleted`
              (`self.K2_EndAbility` :!label _label))
            (:`OnBlendOut`
              (goto _label))
            (:`OnInterrupted`
              (`self.K2_CancelAbility` :!label _label_2))
            (:`OnCancelled`
              (goto _label_2))))))
    (:`CastFailed`
      (`self.K2_CancelAbility`))))

(event `self.K2_OnEndAbility`
  (params (bWasCancelled :type Boolean))
  (if bWasCancelled
    (if (not (`self.bIsReleased`))
      (`/Engine/EditorBlueprintResources/StandardMacros.IsValid` (stale `self.K2_ActivateAbility` _spawnedactor)
        (:`Is Valid`
          (`Actor.K2_DestroyActor` (stale `self.K2_ActivateAbility` _spawnedactor)))))))