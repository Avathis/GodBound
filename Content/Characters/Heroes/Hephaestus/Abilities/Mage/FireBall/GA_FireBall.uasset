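; Hephaestus's fireball gameplay ability, which commits, applies an overheat effect to the owner and plays the right-hand fireball montage.
; On the montage's spawn event it attaches a BP_Fire_Atk_01 to the hand socket with gravity and collision off, then awaits a release event.
; Release only prints and checks the owner cast, as the detach, aim and launch logic sits in disconnected, partly older nodes.
; Montage completion, blend-out or interruption ends the ability.
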(event `self.K2_ActivateAbility`
  (bind (_owneractor _avataractor _playercontroller _abilitysystemcomponent _skeletalmeshcomponent) (break `GameplayAbilityActorInfo` (`self.GetActorInfo`)))
  (`self.K2_CommitAbility`)
  (`self.BP_ApplyGameplayEffectToOwner` "/Game/Effects/Utility/BP_OverHeatEffect.BP_OverHeatEffect_C")
  (`AbilityTask_PlayMontageAndWait.CreatePlayMontageAndWaitProxy` "None" "/Game/Characters/Heroes/Hephaestus/Animations/Abilities/InPlace/Montage_Hephaestus_R_Fireball.Montage_Hephaestus_R_Fireball"
    (:`then`
      (`AbilityTask_WaitGameplayEvent.WaitGameplayEvent` (struct :`TagName` "Abilities.Fire.Ball.Spawn") null
        (:`EventReceived`
          (`AbilityTask_WaitGameplayEvent.WaitGameplayEvent` (struct :`TagName` "Abilities.Fire.Ball.Release") null
            (:`then`
              (bind (_asynctaskproxy _spawnedactor) (`GameplayTask_SpawnActor.SpawnActor` null (`SceneComponent.GetSocketLocation` _skeletalmeshcomponent "Hand_R_Release") (`SceneComponent.GetSocketRotation` _skeletalmeshcomponent "Hand_R_Release") "/Game/Assets/Luos8Elements/Blueprints/Fire/BP_Fire_Atk_01.BP_Fire_Atk_01_C" false null)
                (:`Success`
                  (message `/Game/Interfaces/BPI_Projectile.SetGravity` _spawnedactor false)
                  (`Actor.SetActorEnableCollision` _spawnedactor false)
                  (`Actor.K2_AttachToComponent` _spawnedactor (`Character.Mesh` (cast `GB_PlayableCharacter` _owneractor :!pure true)) "Hand_R_Release" "KeepWorld" "KeepWorld" "KeepWorld" true))
                (:`DidNotSpawn`
                  (`KismetSystemLibrary.PrintString` "Didn't Spawn- Cancelling")
                  (`self.K2_CancelAbility`))))
            (:`EventReceived`
              (`KismetSystemLibrary.PrintString` "EventsRecieved")
              (cast `GB_PlayableCharacter` _owneractor
                (:`CastFailed`
                  (`self.K2_CancelAbility`))))))))
    (:`OnCompleted`
      (`self.K2_EndAbility` :!label _label))
    (:`OnBlendOut`
      (goto _label))
    (:`OnInterrupted`
      (goto _label))
    (:`OnCancelled`
      (`self.K2_CancelAbility`))))

(event `self.K2_OnEndAbility`
  (params (bWasCancelled :type Boolean)))