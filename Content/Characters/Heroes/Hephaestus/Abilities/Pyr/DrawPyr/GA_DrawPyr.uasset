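; Gameplay ability for Hephaestus that draws the Pyr weapon into the character's hand.
; It plays a montage and waits for the Pyr summon gameplay event, then spawns BP_Pyr at HandSocket with a pitch offset.
; The weapon becomes the ActiveWeapon, loses projectile gravity and attaches to the socket.
; It then applies GE_PyrActive, prints owned tags for debugging and ends; any montage exit also ends the ability.
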(event `self.K2_ActivateAbility`
  (`self.K2_CommitAbility`)
  (`AbilityTask_PlayMontageAndWait.CreatePlayMontageAndWaitProxy` "None"
    (:`then`
      (`AbilityTask_WaitGameplayEvent.WaitGameplayEvent` (struct :`TagName` "Abilities.Fire.Weapon.Pyr.Summon") null
        (:`EventReceived`
          (bind _asgb_playable_character (cast `GB_PlayableCharacter` (`self.GetAvatarActorFromActorInfo`)))
          (bind _mesh (`Character.Mesh` _asgb_playable_character))
          (bind (_asynctaskproxy _spawnedactor) (`GameplayTask_SpawnActor.SpawnActor` null (`SceneComponent.GetSocketLocation` _mesh "HandSocket") (`KismetMathLibrary.MakeRotator` (.roll (`SceneComponent.GetSocketRotation` _mesh "HandSocket")) (+ (.pitch (`SceneComponent.GetSocketRotation` _mesh "HandSocket")) 90.0) (.yaw (`SceneComponent.GetSocketRotation` _mesh "HandSocket"))) "/Game/Characters/Heroes/Hephaestus/Weapon/BP_Pyr.BP_Pyr_C" false null)
            (:`Success`
              (bind _asbp_pyr (cast `/Game/Characters/Heroes/Hephaestus/Weapon/BP_Pyr` _spawnedactor))
              (set `GB_PlayableCharacter.ActiveWeapon` _asbp_pyr _asgb_playable_character)
              (set `ProjectileMovementComponent.ProjectileGravityScale` 0.0 (`GB_Pyr.ProjectileMovementComponent` _asbp_pyr))
              (`Actor.K2_AttachToComponent` _spawnedactor (`Character.Mesh` _asgb_playable_character) "HandSocket" "KeepWorld" "KeepWorld" "KeepWorld" true)
              (`self.BP_ApplyGameplayEffectToOwner` "/Game/Characters/Heroes/Hephaestus/Abilities/Pyr/GE_PyrActive.GE_PyrActive_C")
              (bind _tagcontainer (message `GameplayTagAssetInterface.GetOwnedGameplayTags` (`AbilitySystemBlueprintLibrary.GetAbilitySystemComponent` (`self.GetAvatarActorFromActorInfo`))))
              (`KismetSystemLibrary.PrintString` (`BlueprintGameplayTagLibrary.GetDebugStringFromGameplayTagContainer` _tagcontainer))
              (`self.K2_EndAbility`))))))
    (:`OnCompleted`
      (`self.K2_EndAbility` :!label _label))
    (:`OnBlendOut`
      (goto _label))
    (:`OnInterrupted`
      (goto _label))
    (:`OnCancelled`
      (goto _label))))