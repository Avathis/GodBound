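; Gameplay ability that moves the hero Hephaestus into combat.
; On activation it commits and plays the enter-combat montage without stopping it when the ability ends.
; On completion, blend out or interruption, it sends EnterCombat to the avatar through BPI_AbilityInterface, applies GE_InCombat to the owner and ends.
; Cancellation only ends the ability; a missing interface only prints a message, leaving the ability un-ended.
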(event `self.K2_ActivateAbility`
  (bind _returnvalue (`self.GetAvatarActorFromActorInfo`))
  (`self.K2_CommitAbility`)
  (`AbilityTask_PlayMontageAndWait.CreatePlayMontageAndWaitProxy` "None" "/Game/Characters/Heroes/Hephaestus/Animations/Abilities/InPlace/Montage_Hephaestus_EnterCombat_IP.Montage_Hephaestus_EnterCombat_IP" 1.0 "None" false
    (:`OnCompleted`
      (if (`KismetSystemLibrary.DoesImplementInterface` _returnvalue "/Game/Interfaces/BPI_AbilityInterface.BPI_AbilityInterface_C") :!label _label
        (message `/Game/Interfaces/BPI_AbilityInterface.EnterCombatI` _returnvalue)
        (`self.BP_ApplyGameplayEffectToOwner` "/Game/Characters/Heroes/Hephaestus/Abilities/EnterExitCombat/GE_InCombat.GE_InCombat_C")
        (`self.K2_EndAbility`)
        (else
          (`KismetSystemLibrary.PrintString` "NotImplements"))))
    (:`OnBlendOut`
      (goto _label))
    (:`OnInterrupted`
      (goto _label))
    (:`OnCancelled`
      (`self.K2_EndAbility`))))