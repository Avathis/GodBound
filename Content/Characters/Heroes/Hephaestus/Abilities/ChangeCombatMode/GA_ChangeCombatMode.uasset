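; Gameplay ability for the hero Hephaestus that changes his combat mode.
; It plays the state-choice montage, waits for a State.Changing event, then applies GE_ChangeCombatMode to the owner.
; Four parallel waits for ability activation, all requiring State.Changing, each assign one combat set (B, F, M or W) and end the ability.
; On end, it passes the chosen set to the owning actor through ChangeCombatSetMessage.
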(event `self.K2_ActivateAbility`
  (`self.K2_CommitAbility`)
  (`AbilityTask_PlayMontageAndWait.CreatePlayMontageAndWaitProxy` "None" "/Game/Characters/Heroes/Hephaestus/Animations/Abilities/InPlace/Montage_Hephaestus_Choose_State_Start.Montage_Hephaestus_Choose_State_Start"
    (:`then`
      (`AbilityTask_WaitGameplayEvent.WaitGameplayEvent` (struct :`TagName` "State.Changing") null
        (:`EventReceived`
          (`self.BP_ApplyGameplayEffectToOwner` "/Game/Characters/Heroes/Hephaestus/Abilities/ChangeCombatMode/GE_ChangeCombatMode.GE_ChangeCombatMode_C")
          (`AbilityTask_WaitAbilityActivate.WaitForAbilityActivateWithTagRequirements` (make `GameplayTagRequirements` (struct :`GameplayTags` (struct :`(TagName` "State.Changing") :`(TagName` "State.Hephaestus.Blacksmith"))))
            (:`then`
              (`AbilityTask_WaitAbilityActivate.WaitForAbilityActivateWithTagRequirements` (make `GameplayTagRequirements` (struct :`GameplayTags` (struct :`(TagName` "State.Changing") :`(TagName` "State.Hephaestus.Brawl"))))
                (:`then`
                  (`AbilityTask_WaitAbilityActivate.WaitForAbilityActivateWithTagRequirements` (make `GameplayTagRequirements` (struct :`GameplayTags` (struct :`(TagName` "State.Changing") :`(TagName` "State.Hephaestus.Mage"))))
                    (:`then`
                      (`AbilityTask_WaitAbilityActivate.WaitForAbilityActivateWithTagRequirements` (make `GameplayTagRequirements` (struct :`GameplayTags` (struct :`(TagName` "State.Changing") :`(TagName` "State.Hephaestus.Weapons"))))
                        (:`OnActivate`
                          (set `self.CombatSetToChange` "EHS_W"))))
                    (:`OnActivate`
                      (set `self.CombatSetToChange` "EHS_M"))))
                (:`OnActivate`
                  (set `self.CombatSetToChange` "EHS_F"))))
            (:`OnActivate`
              (set `self.CombatSetToChange` "EHS_B")))
          (`self.K2_EndAbility`))))))

(event `self.K2_OnEndAbility`
  (params (bWasCancelled :type Boolean))
  (message `/Game/Interfaces/BPI_AbilityInterface.ChangeCombatSet` (`self.GetOwningActorFromActorInfo`) (`self.CombatSetToChange`)))