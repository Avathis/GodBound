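; Gameplay ability that makes the hero Hephaestus jump.
; On activation it commits, then runs a root motion jump force aimed along the avatar's current velocity, with distance equal to its speed and a fixed height and duration.
; The ability ends when the task finishes or lands, keeping the last root motion velocity on finish.
; An unconnected branch using the character's standard CanJump and Jump never runs.
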(event `self.K2_ActivateAbility`
  (bind _returnvalue (`Actor.GetVelocity` (`self.GetAvatarActorFromActorInfo`)))
  (`self.K2_CommitAbility`)
  (`AbilityTask_ApplyRootMotionJumpForce.ApplyRootMotionJumpForce` "Jumping" (`KismetMathLibrary.Conv_VectorToRotator` _returnvalue) (`KismetMathLibrary.VSize` _returnvalue) 100.0 1.0 1.0 false "MaintainLastRootMotionVelocity" _returnvalue
    (:`OnFinish`
      _)
    (:`OnLanded`
      _))
  (`self.K2_EndAbility`))