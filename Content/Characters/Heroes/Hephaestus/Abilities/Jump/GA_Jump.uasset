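; Gameplay ability for the hero's context-sensitive jump, which becomes a jump, mantle, vault or ledge hang depending on the obstacle.
; A distance trace picks the action; ledge and landing points feed motion warping targets for each montage.
; Mantles and vaults use flying without collision, while hangs enter climb mode.
; When already climbing, it climbs up the ledge or exits climbing; ending restores input, plus walking and collision if not climbing.
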(event `self.K2_ActivateAbility`
  (bind _returnvalue (`self.GetAvatarActorFromActorInfo`))
  (bind _returnvalue_2 (`self.GetAvatarActorFromActorInfo`))
  (bind _returnvalue_3 (`self.GetAvatarActorFromActorInfo`))
  (bind _returnvalue_4 (`self.GetAvatarActorFromActorInfo`))
  (bind _obstacleledgepoint (`self.ObstacleLedgePoint`))
  (bind _wallrotation (`self.WallRotation`))
  (bind _obstaclemidpoint (`self.ObstacleMidPoint`))
  (bind (_owneractor _avataractor _playercontroller) (break `GameplayAbilityActorInfo` (`self.GetActorInfo`)))
  (bind (_owneractor_2 _avataractor_2 _playercontroller_2) (break `GameplayAbilityActorInfo` (`self.GetActorInfo`)))
  (`self.K2_CommitAbility`)
  (bind _returnvalue_5 (`self.GetPlayerCharFromActorInfo`))
  (bind _output_get (set `self.PlayerChar` _returnvalue_5))
  (bind _output_get_2 (set `self.Character Movement Component` (`GB_Character.CharacterMovementComponent` _output_get)))
  (if (`GB_CharacterMovementComponent.bIsClimbing` _output_get_2)
    (bind _returnvalue_6 (`self.StartClimbTraceForDistance` 0.0))
    (if _returnvalue_6
      (message `/Game/Characters/Heroes/BI_Parkour.SendToMotionWarping` _returnvalue_4 "ClimbUp" (`self.ApplyWarpOffset` (`self.ObstacleLedgePoint`) 0.0 -30.0) (`self.WallRotation`))
      (`AbilityTask_PlayMontageAndWait.CreatePlayMontageAndWaitProxy` "None" "/Game/Characters/SharedAnimations/Parkour/Mantle/ClimbUpTheLedge_Montage.ClimbUpTheLedge_Montage"
        (:`OnCompleted`
          _)
        (:`OnBlendOut`
          _)
        (:`OnInterrupted`
          _)
        (:`OnCancelled`
          _))
      (message `/Game/Characters/Heroes/BI_Parkour.ExitClimb` (`self.PlayerChar`))
      (`self.K2_EndAbility`)
      (else
        (message `/Game/Characters/Heroes/BI_Parkour.ExitClimb` _returnvalue_4)
        (`self.K2_EndAbility`)))
    (else
      (`self.StartTraceForDistance`)
      (switch `EDistanceTraceType` (`self.ActionType`)
        (:`EDTT_NormalJump`
          (bind _returnvalue_7 (`self.GetPlayerCharFromActorInfo`))
          (`/Engine/EditorBlueprintResources/StandardMacros.IsValid` _returnvalue_7
            (:`Is Valid`
              (`Character.Jump` _returnvalue_7)
              (`AbilityTask_WaitInputRelease.WaitInputRelease` true
                (:`OnRelease`
                  (`Character.StopJumping` _returnvalue_7)
                  (`self.K2_EndAbility`))))
            (:`Is Not Valid`
              (`self.K2_EndAbility`))))
        (:`EDTT_MantleLow`
          (message `/Game/Characters/Heroes/BI_Parkour.SendToMotionWarping` _returnvalue "MantleLow1" (`self.ApplyWarpOffset` (`self.ObstacleLedgePoint`) -70.0 -70.0) (struct))
          (message `/Game/Characters/Heroes/BI_Parkour.SendToMotionWarping` _returnvalue "MantleLow2" (`self.ApplyWarpOffset` (`self.ObstacleLedgePoint`) 30.0 -10.0) (struct))
          (bind _returnvalue_8 (`self.GetPlayerCharFromActorInfo`))
          (`CharacterMovementComponent.SetMovementMode` (`GB_Character.CharacterMovementComponent` _returnvalue_8) "MOVE_Flying" 0)
          (`Actor.SetActorEnableCollision` _returnvalue false)
          (`AbilityTask_PlayMontageAndWait.CreatePlayMontageAndWaitProxy` "None" "/Game/Characters/SharedAnimations/Parkour/Mantle/LowMantleUE5_Montage.LowMantleUE5_Montage" 1.5
            (:`OnCompleted`
              _)
            (:`OnBlendOut`
              _)
            (:`OnInterrupted`
              _)
            (:`OnCancelled`
              _))
          (`self.K2_EndAbility`))
        (:`EDTT_MantleHigh`
          (message `/Game/Characters/Heroes/BI_Parkour.SendToMotionWarping` _returnvalue_3 "HighMantle1" (`self.ApplyWarpOffset` (`self.ObstacleLedgePoint`) -70.0 -90.0) (struct))
          (message `/Game/Characters/Heroes/BI_Parkour.SendToMotionWarping` _returnvalue_3 "HighMantle2" (`self.ApplyWarpOffset` (`self.ObstacleLedgePoint`) 30.0 -10.0) (struct))
          (bind _returnvalue_9 (`self.GetPlayerCharFromActorInfo`))
          (`CharacterMovementComponent.SetMovementMode` (`GB_Character.CharacterMovementComponent` _returnvalue_9) "MOVE_Flying" 0)
          (`Actor.SetActorEnableCollision` _returnvalue_3 false)
          (`AbilityTask_PlayMontageAndWait.CreatePlayMontageAndWaitProxy` "None" "/Game/Characters/SharedAnimations/Parkour/Mantle/MantleUE5_Montage.MantleUE5_Montage"
            (:`OnCompleted`
              _)
            (:`OnBlendOut`
              _)
            (:`OnInterrupted`
              _)
            (:`OnCancelled`
              _))
          (`self.K2_EndAbility`))
        (:`EDTT_Vault`
          (message `/Game/Characters/Heroes/BI_Parkour.SendToMotionWarping` _returnvalue_2 "VaultWarp1" (select `bool` (`self.bIsRunning`) :`false` (`self.ApplyWarpOffset` _obstacleledgepoint -70.0 -70.0) :`true` (`self.ApplyWarpOffset` _obstacleledgepoint -70.0 -60.0)) (struct))
          (message `/Game/Characters/Heroes/BI_Parkour.SendToMotionWarping` _returnvalue_2 "VaultWarp2" (select `bool` (`self.bIsRunning`) :`false` (`self.ApplyWarpOffset` _obstaclemidpoint -30.0 -35.0) :`true` (`self.ApplyWarpOffset` _obstaclemidpoint 0.0 -45.0)) (struct))
          (message `/Game/Characters/Heroes/BI_Parkour.SendToMotionWarping` _returnvalue_2 "VaultWarp3" (`self.LandPoint`) (struct))
          (bind _returnvalue_10 (`self.GetPlayerCharFromActorInfo`))
          (`CharacterMovementComponent.SetMovementMode` (`GB_Character.CharacterMovementComponent` _returnvalue_10) "MOVE_Flying" 0)
          (`Actor.SetActorEnableCollision` _returnvalue_2 false)
          (`AbilityTask_PlayMontageAndWait.CreatePlayMontageAndWaitProxy` "None" (select `bool` (`self.bIsRunning`) :`false` "/Game/Characters/SharedAnimations/Parkour/Mantle/ThinVault_Montage.ThinVault_Montage" :`true` "/Game/Characters/SharedAnimations/Parkour/Mantle/Vault_Montage.Vault_Montage" :!type "AnimMontage Object Reference")
            (:`OnCompleted`
              _)
            (:`OnBlendOut`
              _)
            (:`OnInterrupted`
              _)
            (:`OnCancelled`
              _))
          (`self.K2_EndAbility`))
        (:`EDTT_HangBraced`
          (`KismetSystemLibrary.PrintString` (`KismetStringLibrary.Conv_RotatorToString` _wallrotation))
          (message `/Game/Characters/Heroes/BI_Parkour.SendToMotionWarping` (`self.GetAvatarActorFromActorInfo`) "BracedHang1" (`self.ApplyWarpOffset` (`self.ObstacleLedgePoint`) -42.5 -190.0) _wallrotation)
          (bind _returnvalue_11 (`self.GetPlayerCharFromActorInfo`))
          (`AbilityTask_PlayMontageAndWait.CreatePlayMontageAndWaitProxy` "None" "/Game/Characters/SharedAnimations/Parkour/BracedHanges/Idle_To_Braced_Hang_Montage.Idle_To_Braced_Hang_Montage"
            (:`then`
              (`Controller.SetIgnoreMoveInput` _playercontroller_2 true)
              (message `/Game/Characters/Heroes/BI_Parkour.EnterClimb` _avataractor_2))
            (:`OnCompleted`
              (`MovementComponent.StopMovementImmediately` (`Character.CharacterMovement` _returnvalue_11) :!label _label)
              (`self.K2_EndAbility`))
            (:`OnBlendOut`
              (goto _label))
            (:`OnInterrupted`
              (goto _label))
            (:`OnCancelled`
              (goto _label))))
        (:`EDTT_HandFree`
          (message `/Game/Characters/Heroes/BI_Parkour.SendToMotionWarping` (`self.GetAvatarActorFromActorInfo`) "FreeHang1" (`self.ApplyWarpOffset` (`self.ObstacleLedgePoint`) 25.0 -220.0) (`self.WallRotation`))
          (bind _returnvalue_12 (`self.GetPlayerCharFromActorInfo`))
          (`AbilityTask_PlayMontageAndWait.CreatePlayMontageAndWaitProxy` "None" "/Game/Characters/SharedAnimations/Parkour/FreeHangs/Jump_To_Freehang_Montage.Jump_To_Freehang_Montage"
            (:`then`
              (`Controller.SetIgnoreMoveInput` _playercontroller true)
              (message `/Game/Characters/Heroes/BI_Parkour.EnterClimb` _avataractor))
            (:`OnCompleted`
              (`MovementComponent.StopMovementImmediately` (`GB_Character.CharacterMovementComponent` _returnvalue_12) :!label _label_2)
              (`self.K2_EndAbility`))
            (:`OnBlendOut`
              (goto _label_2))
            (:`OnInterrupted`
              (goto _label_2))
            (:`OnCancelled`
              (goto _label_2))))))))

(event `self.K2_OnEndAbility`
  (params (bWasCancelled :type Boolean))
  (`Controller.ResetIgnoreMoveInput` (`.PlayerController` (break `GameplayAbilityActorInfo` (`self.GetActorInfo`))))
  (bind _returnvalue (`self.GetPlayerCharFromActorInfo`))
  (bind _charactermovementcomponent (`GB_Character.CharacterMovementComponent` _returnvalue))
  (if (not (`GB_CharacterMovementComponent.bIsClimbing` _charactermovementcomponent))
    (`CharacterMovementComponent.SetMovementMode` _charactermovementcomponent "MOVE_Walking" 0)
    (`Actor.SetActorEnableCollision` (`self.GetAvatarActorFromActorInfo`) true))
  (set `self.LandPoint` (0.0 0.0 0.0))
  (set `self.ObstacleMidPoint` (0.0 0.0 0.0))
  (set `self.ActionType` "EDTT_NormalJump"))