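; Gameplay ability for Hephaestus that performs a sideways parkour hop between braced hang positions.
; An incoming gameplay event supplies the target hit and a signed magnitude that selects right or left.
; It sends a "ParkourHop" motion warping target, built from the hit location with per-side offsets and the reversed impact normal.
; The matching hop montage then plays, and the ability ends when it completes, blends out or is interrupted.
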(event `self.K2_ActivateAbilityFromEvent`
  (params (EventData :type "GameplayEventData Structure (by ref)"))
  (bind (_eventtag _instigator _target _optionalobject _optionalobject2 _contexthandle _instigatortags _targettags _eventmagnitude _targetdata) (break `GameplayEventData` EventData))
  (bind _returnvalue (`self.GetAvatarActorFromActorInfo`))
  (bind _returnvalue_2 (> _eventmagnitude 0.0))
  (bind (_bblockinghit _binitialoverlap _time _distance _location _impactpoint _normal _impactnormal) (`GameplayStatics.BreakHitResult` (`AbilitySystemBlueprintLibrary.GetHitResultFromTargetData` _targetdata)))
  (set `self.JumpDirection` (`Actor.GetActorForwardVector` _returnvalue))
  (set `self.JumpDirectionRight` (`Actor.GetActorRightVector` _returnvalue))
  (`self.K2_CommitAbility`)
  (message `/Game/Characters/Heroes/BI_Parkour.SendToMotionWarping` _returnvalue "ParkourHop" (select `bool` _returnvalue_2 :`false` (`self.ApplyWarpOffset` _location 30.0 (* _eventmagnitude 40.0) -188.030104) :`true` (`self.ApplyWarpOffset` _location 20.0 (* _eventmagnitude 45.0) -178.112474)) (`self.ReverseRotationZ` _impactnormal))
  (if _returnvalue_2
    (`AbilityTask_PlayMontageAndWait.CreatePlayMontageAndWaitProxy` "None" "/Game/Characters/SharedAnimations/Parkour/BracedHanges/Braced_Hang_Hop_Right_UE5_Montage.Braced_Hang_Hop_Right_UE5_Montage"
      (:`OnCompleted`
        _)
      (:`OnBlendOut`
        _)
      (:`OnInterrupted`
        _)
      (:`OnCancelled`
        _))
    (`self.K2_EndAbility`)
    (else
      (`AbilityTask_PlayMontageAndWait.CreatePlayMontageAndWaitProxy` "None" "/Game/Characters/SharedAnimations/Parkour/BracedHanges/Braced_Hang_Hop_LeftUE5_Montage.Braced_Hang_Hop_LeftUE5_Montage"
        (:`OnCompleted`
          _)
        (:`OnBlendOut`
          _)
        (:`OnInterrupted`
          _)
        (:`OnCancelled`
          _))
      (`self.K2_EndAbility`))))