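; Gameplay ability for Hephaestus's pull kick, which damages enemies along a forward line, then pulls them into it.
; It locks controller yaw and waits for the montage's kick event, then steps forward with down/up traces to spawn terrain-following helper actors.
; Helper box overlaps apply damage, then GE_PullIntoLine one second later, deduplicated per pass.
; Ending restores yaw and destroys helpers; disconnected earlier approaches remain in the graph.
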(event `self.K2_ActivateAbility`
  (bind _returnvalue (`self.GetAvatarActorFromActorInfo`))
  (bind _array (`|MakeArray` "ObjectTypeQuery1" :!type "EObjectTypeQuery Enum"))
  (bind _actorstohit (`self.ActorsToHit`))
  (bind _actorstohit_2 (`self.ActorsToHit`))
  (bind _actorstohit_3 (`self.ActorsToHit`))
  (bind _returnvalue_2 (`Actor.K2_GetActorRotation` _returnvalue))
  (bind _returnvalue_3 (+ (* (`Actor.GetActorForwardVector` _returnvalue) (`self.DistanceForHelper`)) (`Actor.K2_GetActorLocation` _returnvalue)))
  (`self.K2_CommitAbility`)
  (bind _asbp_ubhephaestus (cast `/Game/Characters/Heroes/Hephaestus/BP_UBHephaestus` (`self.GetAvatarActorFromActorInfo`)))
  (set `Pawn.bUseControllerRotationYaw` false _asbp_ubhephaestus)
  (`AbilityTask_PlayMontageAndWait.CreatePlayMontageAndWaitProxy` "None" "/Game/Characters/SharedAnimations/MeleeAnimations/FighterAnimations/Attacks/Hephaestus_PullKick.Hephaestus_PullKick"
    (:`then`
      (`AbilityTask_WaitGameplayEvent.WaitGameplayEvent` (struct :`TagName` "Abilities.Hephaestus.F.Kick") null true false
        (:`EventReceived`
          (for _ (range 13)
            (bind _outhit (`KismetSystemLibrary.LineTraceSingleForObjects` :`Start` _returnvalue_3 :`End` (`KismetMathLibrary.MakeVector` (.x _returnvalue_3) (.y _returnvalue_3) (- (.z _returnvalue_3) (`self.GradualDecline`))) :`ObjectTypes` _array :`DrawDebugType` "Persistent"))
            (bind (_bblockinghit _binitialoverlap _time _distance _location) (`GameplayStatics.BreakHitResult` _outhit))
            (if _bblockinghit
              (bind (_asynctaskproxy _spawnedactor) (`GameplayTask_SpawnActor.SpawnActor` null _location _returnvalue_2 "/Game/Actors/Abilityactors/AbilityHelperActors/Hephaestus_PullKickHelper.Hephaestus_PullKickHelper_C" false null)
                (:`Success`
                  (`KismetArrayLibrary.Array_Add` (`self.HelperActors`) _spawnedactor)
                  (bind _ashephaestus_pull_kick_helper (cast `/Game/Actors/Abilityactors/AbilityHelperActors/Hephaestus_PullKickHelper` _spawnedactor :!pure true))
                  (for _array_element (`PrimitiveComponent.GetOverlappingActors` (`/Game/Actors/Abilityactors/AbilityHelperActors/Hephaestus_PullKickHelper.Box` _ashephaestus_pull_kick_helper) "/Script/GodBound.GB_EnemyCharacter")
                    (if (not (`KismetArrayLibrary.Array_Contains` _actorstohit_2 _array_element))
                      (`KismetArrayLibrary.Array_Add` _actorstohit_2 _array_element)
                      (bind _returnvalue_4 (`AbilitySystemBlueprintLibrary.AssignTagSetByCallerMagnitude` (`self.MakeOutgoingGameplayEffectSpec` (`self.DamageEffect`)) (struct :`TagName` "Damage") 50.0))
                      (`AbilitySystemComponent.BP_ApplyGameplayEffectSpecToTarget` (`AbilitySystemBlueprintLibrary.GetAbilitySystemComponent` _ashephaestus_pull_kick_helper) _returnvalue_4 (`AbilitySystemBlueprintLibrary.GetAbilitySystemComponent` _array_element))))
                  (set `self.GradualDecline` (+ (`self.GradualDecline`) 30.0))
                  (set `self.GradualIncline` 50.0)
                  (set `self.DistanceForHelper` (+ (`self.DistanceForHelper`) 60.0) :!label _label)))
              (else
                (bind (_outhit_2 _returnvalue_5) (`KismetSystemLibrary.LineTraceSingleForObjects` :`Start` _returnvalue_3 :`End` (`KismetMathLibrary.MakeVector` (.x _returnvalue_3) (.y _returnvalue_3) (+ (.z _returnvalue_3) (`self.GradualIncline`))) :`ObjectTypes` _array :`DrawDebugType` "Persistent"))
                (if _returnvalue_5
                  (bind (_asynctaskproxy_2 _spawnedactor_2) (`GameplayTask_SpawnActor.SpawnActor` null (`.Location` (`GameplayStatics.BreakHitResult` _outhit_2)) _returnvalue_2 "/Game/Actors/Abilityactors/AbilityHelperActors/Hephaestus_PullKickHelper.Hephaestus_PullKickHelper_C" false null)
                    (:`Success`
                      (`KismetArrayLibrary.Array_Add` (`self.HelperActors`) _spawnedactor_2)
                      (bind _ashephaestus_pull_kick_helper_2 (cast `/Game/Actors/Abilityactors/AbilityHelperActors/Hephaestus_PullKickHelper` _spawnedactor_2 :!pure true))
                      (for _array_element_2 (`PrimitiveComponent.GetOverlappingActors` (`/Game/Actors/Abilityactors/AbilityHelperActors/Hephaestus_PullKickHelper.Box` _ashephaestus_pull_kick_helper_2) "/Script/GodBound.GB_EnemyCharacter")
                        (if (not (`KismetArrayLibrary.Array_Contains` _actorstohit _array_element_2))
                          (`KismetArrayLibrary.Array_Add` _actorstohit _array_element_2)
                          (bind _returnvalue_6 (`AbilitySystemBlueprintLibrary.AssignTagSetByCallerMagnitude` (`self.MakeOutgoingGameplayEffectSpec` (`self.DamageEffect`)) (struct :`TagName` "Damage") 50.0))
                          (`AbilitySystemComponent.BP_ApplyGameplayEffectSpecToTarget` (`AbilitySystemBlueprintLibrary.GetAbilitySystemComponent` _ashephaestus_pull_kick_helper_2) _returnvalue_6 (`AbilitySystemBlueprintLibrary.GetAbilitySystemComponent` _array_element_2))
                          (goto _label)))
                      (set `self.GradualIncline` (+ (`self.GradualIncline`) 50.0))
                      (set `self.GradualDecline` 120.0)))
                  (else
                    (break))))))
          (`KismetArrayLibrary.Array_Clear` (`self.ActorsToHit`))
          (`GameplayTask_WaitDelay.TaskWaitDelay` null 1.0
            (:`OnFinish`
              (for _array_element_3 (`self.HelperActors`)
                (bind _ashephaestus_pull_kick_helper_3 (cast `/Game/Actors/Abilityactors/AbilityHelperActors/Hephaestus_PullKickHelper` _array_element_3))
                (for _array_element_4 (`PrimitiveComponent.GetOverlappingActors` (`/Game/Actors/Abilityactors/AbilityHelperActors/Hephaestus_PullKickHelper.Box` _ashephaestus_pull_kick_helper_3) "/Script/GodBound.GB_EnemyCharacter")
                  (if (`KismetArrayLibrary.Array_Contains` _actorstohit_3 _array_element_4)
                    (`KismetSystemLibrary.PrintString` "Hello")
                    (else
                      (`KismetArrayLibrary.Array_Add` _actorstohit_3)
                      (`AbilitySystemComponent.BP_ApplyGameplayEffectToTarget` :`self` (`AbilitySystemBlueprintLibrary.GetAbilitySystemComponent` _ashephaestus_pull_kick_helper_3) :`GameplayEffectClass` "/Game/Characters/Heroes/Hephaestus/CharacterSpecificEffects/GE_PullIntoLine.GE_PullIntoLine_C" :`Target` (`AbilitySystemBlueprintLibrary.GetAbilitySystemComponent` _array_element_4))))))
              (`self.K2_EndAbility`))))))))

(event `self.K2_OnEndAbility`
  (params (bWasCancelled :type Boolean))
  (bind _helperactors (`self.HelperActors`))
  (bind _asbp_ubhephaestus (cast `/Game/Characters/Heroes/Hephaestus/BP_UBHephaestus` (`self.GetAvatarActorFromActorInfo`))
    (:`then`
      (set `Pawn.bUseControllerRotationYaw` true _asbp_ubhephaestus))
    (:`CastFailed`
      _))
  (set `self.DistanceForHelper` 60.0)
  (`KismetArrayLibrary.Array_Clear` (`self.ActorsToHit`))
  (set `self.GradualDecline` 120.0)
  (set `self.GradualIncline` 50.0)
  (for _array_element _helperactors
    (`Actor.K2_DestroyActor` _array_element))
  (`KismetArrayLibrary.Array_Clear` _helperactors))