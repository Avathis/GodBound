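; Hephaestus Fighter ability that dashes forward, leaps up while knocking up nearby actors, then dives to a player-confirmed target.
; Root motion move-to tasks drive each phase, with montages, a jump gameplay event and a timed targeting window between them.
; During the dive, delayed sphere overlaps attach caught actors to the foot socket while capsule collision switches to overlap.
; Landing detaches them, applies knockback and restores collision.
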(event `self.K2_ActivateAbility`
  (bind _returnvalue (`self.GetAvatarActorFromActorInfo`))
  (bind _returnvalue_2 (`self.GetAvatarActorFromActorInfo`))
  (bind _returnvalue_3 (`self.GetAvatarActorFromActorInfo`))
  (bind _array (`|MakeArray` "ObjectTypeQuery8" :!type "EObjectTypeQuery Enum"))
  (bind _attachedactors (`self.AttachedActors`))
  (bind (_locationtype _literaltransform _sourceactor _sourcecomponent _sourceability _sourcesocketname) (break `GameplayAbilityTargetingLocationInfo` (`self.MakeTargetLocationInfoFromOwnerActor`)))
  (bind _returnvalue_4 (`SceneComponent.GetSocketLocation` (`self.GetOwningComponentFromActorInfo`) "Foot_L_Kick"))
  (bind _returnvalue_5 (`Actor.K2_GetActorLocation` _returnvalue_2))
  (`self.K2_CommitAbility`)
  (`AbilityTask_ApplyRootMotionMoveToForce.ApplyRootMotionMoveToForce` "None" (+ (* (`Actor.GetActorForwardVector` _returnvalue) (`KismetMathLibrary.Conv_DoubleToVector` 200.0)) (`Actor.K2_GetActorLocation` _returnvalue)) 0.44 false "MOVE_None" false null "MaintainLastRootMotionVelocity"
    (:`then`
      (`AbilityTask_PlayMontageAndWait.CreatePlayMontageAndWaitProxy` "None" "/Game/Characters/SharedAnimations/MeleeAnimations/FighterAnimations/Attacks/Montage_Hephaestus_UpAndDOwn.Montage_Hephaestus_UpAndDOwn" 1.0 "None" true 0.0
        (:`then`
          (`AbilityTask_WaitGameplayEvent.WaitGameplayEvent` (struct :`TagName` "Abilities.Hephaestus.F.Jump") null
            (:`EventReceived`
              (bind _outactors (`KismetSystemLibrary.SphereOverlapActors` _returnvalue_5 200.0 (`|MakeArray` "ObjectTypeQuery8" :!type "EObjectTypeQuery Enum")))
              (`self.BP_ApplyGameplayEffectToTarget` (`AbilitySystemBlueprintLibrary.AbilityTargetDataFromActorArray` _outactors) "/Game/Characters/Heroes/SharedAbilities/GE_KnockUp_UAD.GE_KnockUp_UAD_C")
              (`AbilityTask_ApplyRootMotionMoveToForce.ApplyRootMotionMoveToForce` "None" (+ (* (`Actor.GetActorForwardVector` _returnvalue_2) (`KismetMathLibrary.Conv_DoubleToVector` 200.0)) _returnvalue_5 (0.0 0.0 300.0)) 0.5 false "MOVE_Flying" false null "MaintainLastRootMotionVelocity"
                (:`OnTimedOut`
                  _)
                (:`OnTimedOutAndDestinationReached`
                  _))
              (bind (_asynctaskproxy _data) (`AbilityTask_WaitTargetData.WaitTargetData` "None" "UserConfirmed" "/Game/Actors/TargetActors/BP_HephaestusUAD_TA.BP_HephaestusUAD_TA_C" 0.0 0.0 1000.0 (struct :`Name` "TargetActorGroundLocation") true (make `GameplayAbilityTargetingLocationInfo` _locationtype _literaltransform _sourceactor _sourcecomponent _sourceability _sourcesocketname) (struct) null (struct) true)
                (:`then`
                  (`AbilityTask_PlayMontageAndWait.CreatePlayMontageAndWaitProxy` "None" "/Game/Characters/SharedAnimations/MeleeAnimations/FighterAnimations/Attacks/Hephaestus_Air_to_Floor_02_Start_Seq_Retargeted_Montage.Hephaestus_Air_to_Floor_02_Start_Seq_Retargeted_Montage" 0.3
                    (:`then`
                      (`AbilityTask_WaitDelay.WaitDelay` 1.0
                        (:`OnFinish`
                          (`/Engine/EditorBlueprintResources/StandardMacros.IsValid` _asynctaskproxy
                            (:`Is Valid`
                              (`GameplayTask.EndTask` _asynctaskproxy)
                              (`self.K2_EndAbility`))))))))
                (:`ValidData`
                  (`AbilityTask_ApplyRootMotionMoveToForce.ApplyRootMotionMoveToForce` "None" (`.Location` (`GameplayStatics.BreakHitResult` (`AbilitySystemBlueprintLibrary.GetHitResultFromTargetData` _data))) 0.3 false "MOVE_None" false null "SetVelocity"
                    (:`then`
                      (bind _asgb_playable_character (cast `GB_PlayableCharacter` (`self.GetOwningActorFromActorInfo`))
                        (:`then`
                          (`PrimitiveComponent.SetCollisionResponseToChannel` (`Character.CapsuleComponent` _asgb_playable_character) "ECC_GameTraceChannel2" "ECR_Overlap")
                          (bind _asynctaskproxy_2 (`AbilityTask_WaitDelay.WaitDelay` 0.05 :!label _label)
                            (:`then`
                              (`AbilityTask_PlayMontageAndWait.CreatePlayMontageAndWaitProxy` "None" "/Game/Characters/SharedAnimations/MeleeAnimations/FighterAnimations/Attacks/Hephaestus_Air_to_Floor_02_Loop_Seq_Retargeted_Montage.Hephaestus_Air_to_Floor_02_Loop_Seq_Retargeted_Montage" 0.01))
                            (:`OnFinish`
                              (bind _outactors_2 (`KismetSystemLibrary.SphereOverlapActors` _returnvalue_4 200.0 _array))
                              (`KismetSystemLibrary.DrawDebugSphere` _returnvalue_4 200.0 12 (struct :`R` 1.0 :`G` 1.0 :`B` 1.0 :`A` 1.0) 5.0)
                              (for _array_element _outactors_2
                                (if (not (`KismetArrayLibrary.Array_Contains` (`self.AttachedActors`) _array_element))
                                  (`Actor.K2_AttachToActor` _array_element _returnvalue_3 "Foot_L_Kick" "KeepWorld" "KeepWorld" "KeepWorld" true)
                                  (`KismetArrayLibrary.Array_Add` (`self.AttachedActors`) _array_element)
                                  (goto _label))))))
                        (:`CastFailed`
                          (`self.K2_EndAbility`))))
                    (:`OnTimedOut`
                      (`/Engine/EditorBlueprintResources/StandardMacros.IsValid` _asynctaskproxy_2 :!label _label_2
                        (:`Is Valid`
                          (`GameplayTask.EndTask` _asynctaskproxy_2))
                        (:`Is Not Valid`
                          _))
                      (`AbilityTask_PlayMontageAndWait.CreatePlayMontageAndWaitProxy` "None" "/Game/Characters/SharedAnimations/MeleeAnimations/FighterAnimations/Attacks/Hephaestus_Air_to_Floor_02_End_Seq_Retargeted_Montage.Hephaestus_Air_to_Floor_02_End_Seq_Retargeted_Montage" 1.0 "None" false
                        (:`then`
                          (if (`KismetArrayLibrary.Array_IsNotEmpty` _attachedactors)
                            (for _array_element_2 _attachedactors
                              (`Actor.K2_DetachFromActor` _array_element_2 "KeepWorld" "KeepWorld" "KeepWorld"))
                            (`KismetArrayLibrary.Array_Clear` _attachedactors))
                          (bind _outactors_3 (`KismetSystemLibrary.SphereOverlapActors` (`Actor.K2_GetActorLocation` _returnvalue_3) 200.0 _array))
                          (`self.BP_ApplyGameplayEffectToTarget` (`AbilitySystemBlueprintLibrary.AbilityTargetDataFromActorArray` _outactors_3) "/Game/Characters/Heroes/SharedAbilities/KnockBack/GE_KnockBack.GE_KnockBack_C"))
                        (:`OnCompleted`
                          (bind _asgb_playable_character_2 (cast `GB_PlayableCharacter` (`self.GetAvatarActorFromActorInfo`) :!label _label_3))
                          (`PrimitiveComponent.SetCollisionResponseToChannel` (`Character.CapsuleComponent` _asgb_playable_character_2) "ECC_GameTraceChannel2" "ECR_Block")
                          (`self.K2_EndAbility`))
                        (:`OnBlendOut`
                          (goto _label_3))
                        (:`OnInterrupted`
                          (goto _label_3))
                        (:`OnCancelled`
                          (goto _label_3))))
                    (:`OnTimedOutAndDestinationReached`
                      (goto _label_2))))
                (:`Cancelled`
                  (`self.K2_EndAbility`))))))
        (:`OnCancelled`
          (`self.K2_CancelAbility`))))))

(event `self.K2_OnEndAbility`
  (params (bWasCancelled :type Boolean))
  (bind _attachedactors (`self.AttachedActors`))
  (if (`KismetArrayLibrary.Array_IsNotEmpty` _attachedactors)
    (for _array_element _attachedactors
      (`Actor.K2_DetachFromActor` _array_element "KeepWorld" "KeepWorld" "KeepWorld")
      (`Actor.SetActorEnableCollision` _array_element true))
    (`KismetArrayLibrary.Array_Clear` _attachedactors)))