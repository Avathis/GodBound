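; Gameplay ability for Hephaestus's Rise of the Inferno, a charged leap to a targeted point ending in a ground slam.
; Input release or a three-second cap confirms targeting, then an arc-solved impulse launches the character through start and loop montages.
; Walking again triggers the landing montage and a sphere overlap applying GE_LandingDamage, with radius and SetByCaller damage scaled by hold time and distance.
; Debug sphere and print remain active.
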(event `self.K2_ActivateAbility`
  (bind _returnvalue (`self.GetAbilitySystemComponentFromActorInfo`))
  (bind (_locationtype _literaltransform _sourceactor _sourcecomponent _sourceability _sourcesocketname) (break `GameplayAbilityTargetingLocationInfo` (`self.MakeTargetLocationInfoFromOwnerActor`)))
  (bind _returnvalue_2 (`Actor.K2_GetActorLocation` (`self.GetOwningActorFromActorInfo`)))
  (bind _returnvalue_3 (/ (`self.Distance`) (`self.MaxDistance`)))
  (bind _returnvalue_4 (`KismetMathLibrary.FClamp` (* (`self.TimeHeld`) _returnvalue_3 200.0) 200.0 1550.0))
  (`self.K2_CommitAbility`)
  (`AbilityTask_PlayMontageAndWait.CreatePlayMontageAndWaitProxy` "None"
    (:`then`
      (bind (_asynctaskproxy _data) (`AbilityTask_WaitTargetData.WaitTargetData` "None" "Custom" "/Game/Actors/TargetActors/BP_TA_HephPowerJump.BP_TA_HephPowerJump_C" 0.0 0.0 400.0 (struct :`Name` "TargetActorGroundLocation") true (make `GameplayAbilityTargetingLocationInfo` _locationtype _literaltransform _sourceactor _sourcecomponent _sourceability _sourcesocketname) (struct) null (struct) true)
        (:`then`
          (bind (_asynctaskproxy_2 _timeheld) (`AbilityTask_WaitInputRelease.WaitInputRelease` false)
            (:`then`
              (bind _asynctaskproxy_3 (`AbilityTask_WaitDelay.WaitDelay` 3.0)
                (:`OnFinish`
                  (`/Engine/EditorBlueprintResources/StandardMacros.IsValid` _asynctaskproxy_2
                    (:`Is Valid`
                      (`GameplayTask.EndTask` _asynctaskproxy_2)
                      (set `self.TimeHeld` 3.0)
                      (`AbilitySystemComponent.TargetConfirm` _returnvalue))))))
            (:`OnRelease`
              (set `self.TimeHeld` _timeheld)
              (`AbilitySystemComponent.TargetConfirm` _returnvalue)
              (`/Engine/EditorBlueprintResources/StandardMacros.IsValid` _asynctaskproxy_3
                (:`Is Valid`
                  (`GameplayTask.EndTask` _asynctaskproxy_3))))))
        (:`ValidData`
          (bind (_bblockinghit _binitialoverlap _time _distance _location _impactpoint _normal _impactnormal _physmat _hitactor _hitcomponent _hitbonename _bonename _hititem _elementindex _faceindex _tracestart) (`GameplayStatics.BreakHitResult` (`AbilitySystemBlueprintLibrary.GetHitResultFromTargetData` _data)))
          (set `self.Distance` (`KismetMathLibrary.Vector_Distance` _tracestart _location))
          (bind _outlaunchvelocity (`GameplayStatics.SuggestProjectileVelocity_CustomArc` _tracestart _location 0.0 0.4))
          (bind _asgb_character_movement_component (cast `GB_CharacterMovementComponent` (`.MovementComponent` (break `GameplayAbilityActorInfo` (`self.GetActorInfo`)))))
          (`CharacterMovementComponent.AddImpulse` _asgb_character_movement_component _outlaunchvelocity true)
          (`AbilityTask_PlayMontageAndWait.CreatePlayMontageAndWaitProxy` "None" "/Game/Characters/SharedAnimations/MeleeAnimations/FighterAnimations/Attacks/Attack_Air_to_Floor_01_Start_Seq_Retargeted_Montage.Attack_Air_to_Floor_01_Start_Seq_Retargeted_Montage" 0.5
            (:`then`
              (`AbilityTask_WaitMovementModeChange.CreateWaitMovementModeChange` "MOVE_Walking"
                (:`OnChange`
                  (`AbilityTask_PlayMontageAndWait.CreatePlayMontageAndWaitProxy` "None" "/Game/Characters/SharedAnimations/MeleeAnimations/FighterAnimations/Attacks/Attack_Air_to_Floor_01_End_Seq_Retargeted_Montage.Attack_Air_to_Floor_01_End_Seq_Retargeted_Montage" 1.0 "None" false
                    (:`then`
                      (bind _outactors (`KismetSystemLibrary.SphereOverlapActors` _returnvalue_2 _returnvalue_4 (`|MakeArray` "ObjectTypeQuery8" :!type "EObjectTypeQuery Enum")))
                      (`KismetSystemLibrary.DrawDebugSphere` _returnvalue_2 _returnvalue_4 12 (struct :`R` 1.0 :`G` 1.0 :`B` 1.0 :`A` 1.0) 5.0 1.0)
                      (`KismetSystemLibrary.PrintString` (`KismetStringLibrary.Conv_DoubleToString` _returnvalue_4))
                      (bind _returnvalue_5 (`AbilitySystemBlueprintLibrary.AssignTagSetByCallerMagnitude` (`self.MakeOutgoingGameplayEffectSpec` "/Game/Characters/Heroes/Hephaestus/Abilities/Fighter/RiseOfTheInferno/GE_LandingDamage.GE_LandingDamage_C") (struct :`TagName` "Damage") (`KismetMathLibrary.FClamp` (* (`self.Damage`) (* _returnvalue_3 (`self.TimeHeld`))) 50.0 400.0)))
                      (`self.K2_ApplyGameplayEffectSpecToTarget` _returnvalue_5 (`AbilitySystemBlueprintLibrary.AbilityTargetDataFromActorArray` _outactors))
                      (`self.K2_EndAbility`))))))
            (:`OnBlendOut`
              (`AbilityTask_PlayMontageAndWait.CreatePlayMontageAndWaitProxy` "None" "/Game/Characters/SharedAnimations/MeleeAnimations/FighterAnimations/Attacks/Attack_Air_to_Floor_01_Loop_Seq_Retargeted_Montage.Attack_Air_to_Floor_01_Loop_Seq_Retargeted_Montage"))))))))