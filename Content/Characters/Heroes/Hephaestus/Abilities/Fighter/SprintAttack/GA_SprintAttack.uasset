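; Gameplay ability for Hephaestus's Fighter sprint attack, a punch montage launched with constant root-motion force.
; Once the montage starts, it removes effects granting the Run tag and stops sprinting on the custom movement component.
; The first Big hit gameplay event triggers a sphere overlap and debug sphere at the right-hand punch socket, but the overlap results go unused.
; The ability ends when the montage completes, blends out, is interrupted or cancelled.
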(event `self.K2_ActivateAbility`
  (bind (_owneractor _avataractor _playercontroller _abilitysystemcomponent _skeletalmeshcomponent _animinstance _movementcomponent) (break `GameplayAbilityActorInfo` (`self.GetActorInfo`)))
  (bind _returnvalue (`SceneComponent.GetSocketLocation` _skeletalmeshcomponent "Hand_R_Punch"))
  (`self.K2_CommitAbility`)
  (`AbilityTask_ApplyRootMotionConstantForce.ApplyRootMotionConstantForce` "None" (0.0 0.0 0.0) 0.0 0.0 false null "MaintainLastRootMotionVelocity"
    (:`then`
      (`AbilityTask_PlayMontageAndWait.CreatePlayMontageAndWaitProxy` "None" "/Game/Characters/SharedAnimations/MeleeAnimations/FighterAnimations/Attacks/Hephaestus_SprintAttack.Hephaestus_SprintAttack"
        (:`then`
          (`self.BP_RemoveGameplayEffectFromOwnerWithGrantedTags` (struct :`GameplayTags` (struct :`(TagName` "State.Movement.Run"))))
          (bind _asgb_character_movement_component (cast `GB_CharacterMovementComponent` _movementcomponent))
          (`GB_CharacterMovementComponent.StopSprinting` _asgb_character_movement_component)
          (`AbilityTask_WaitGameplayEvent.WaitGameplayEvent` (struct :`TagName` "Abilities.Hephaestus.F.Hit.Big") null true
            (:`EventReceived`
              (`KismetSystemLibrary.SphereOverlapActors` _returnvalue 100.0 (`|MakeArray` "ObjectTypeQuery8" :!type "EObjectTypeQuery Enum"))
              (`KismetSystemLibrary.DrawDebugSphere` _returnvalue 100.0 12 (struct :`R` 1.0 :`G` 1.0 :`B` 1.0 :`A` 1.0) 5.0 1.0))))
        (:`OnCompleted`
          (`self.K2_EndAbility` :!label _label))
        (:`OnBlendOut`
          (goto _label))
        (:`OnInterrupted`
          (goto _label))
        (:`OnCancelled`
          (goto _label))))))