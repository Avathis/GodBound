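; Second-step ability of Hephaestus's Fighter Combo 1, playing a punch montage with a small left-hand hit and a big right-hand hit.
; Montage-timed gameplay events trigger sphere overlaps at the fist sockets, applying set-by-caller damage, with knockback targeting wired only for the big hit.
; An IntoCombo event applies the combo-progression effect to the owner.
; Montage end or interruption ends the ability, which removes Combo1.Three-tagged effects.
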(event `self.K2_ActivateAbility`
  (`self.K2_CommitAbility`)
  (`AbilityTask_PlayMontageAndWait.CreatePlayMontageAndWaitProxy` "None" (`self.AbilityMontage`) 0.75 "None" false
    (:`then`
      (`AbilityTask_WaitGameplayEvent.WaitGameplayEvent` (struct :`TagName` "Abilities.Hephaestus.F.Hit.Small") null true
        (:`then`
          (`AbilityTask_WaitGameplayEvent.WaitGameplayEvent` (struct :`TagName` "Abilities.Hephaestus.F.Hit.Big") null true
            (:`then`
              (`AbilityTask_WaitGameplayEvent.WaitGameplayEvent` (struct :`TagName` "Abilities.IntoCombo") null
                (:`EventReceived`
                  (`self.BP_ApplyGameplayEffectToOwner` "/Game/Characters/Heroes/Hephaestus/Abilities/Fighter/Combo1/GE_C1_IntoCombo2.GE_C1_IntoCombo2_C"))))
            (:`EventReceived`
              (bind _outactors (`KismetSystemLibrary.SphereOverlapActors` (`SceneComponent.GetSocketLocation` (`self.GetOwningComponentFromActorInfo`) "Hand_R_Punch") 100.0 (`|MakeArray` "ObjectTypeQuery6" "ObjectTypeQuery8" :!type "EObjectTypeQuery Enum")))
              (bind _returnvalue (`AbilitySystemBlueprintLibrary.AssignTagSetByCallerMagnitude` (`self.MakeOutgoingGameplayEffectSpec` (`self.PunchDamageEffect`) (`KismetMathLibrary.Conv_IntToDouble` (`self.GetAbilityLevel`))) (struct :`TagName` "Damage") (`self.BigPunchDamage`)))
              (bind _returnvalue_2 (`AbilitySystemBlueprintLibrary.AbilityTargetDataFromActorArray` _outactors))
              (`self.K2_ApplyGameplayEffectSpecToTarget` _returnvalue _returnvalue_2)
              (`self.BP_ApplyGameplayEffectToTarget` _returnvalue_2 (`self.KnockBackEffect`) 2))))
        (:`EventReceived`
          (bind _outactors_2 (`KismetSystemLibrary.SphereOverlapActors` (`SceneComponent.GetSocketLocation` (`self.GetOwningComponentFromActorInfo`) "Hand_L_Punch") 100.0 (`|MakeArray` "ObjectTypeQuery6" "ObjectTypeQuery8" :!type "EObjectTypeQuery Enum")))
          (bind _returnvalue_3 (`AbilitySystemBlueprintLibrary.AssignTagSetByCallerMagnitude` (`self.MakeOutgoingGameplayEffectSpec` (`self.PunchDamageEffect`) (`KismetMathLibrary.Conv_IntToDouble` (`self.GetAbilityLevel`))) (struct :`TagName` "Damage") (`self.SmallPunchDamage`)))
          (`self.K2_ApplyGameplayEffectSpecToTarget` _returnvalue_3 (`AbilitySystemBlueprintLibrary.AbilityTargetDataFromActorArray` _outactors_2))
          (`self.BP_ApplyGameplayEffectToTarget` (struct) (`self.KnockBackEffect`)))))
    (:`OnCompleted`
      (`self.K2_EndAbility` :!label _label))
    (:`OnBlendOut`
      (goto _label))
    (:`OnInterrupted`
      (goto _label))
    (:`OnCancelled`
      (goto _label))))

(event `self.K2_OnEndAbility`
  (params (bWasCancelled :type Boolean))
  (`self.BP_RemoveGameplayEffectFromOwnerWithGrantedTags` (struct :`GameplayTags` (struct :`(TagName` "Abilities.Hephaestus.F.Combo1.Three")))))