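; GA_Combo01_1 is a Hephaestus fighter combo ability: a lunging punch that damages and knocks back targets.
; Root motion moves him toward the closest enemy in melee range, or a short dash forward if none, as the montage plays.
; A hit event triggers a sphere overlap at the punch socket to apply both effects, then a combo event applies GE_C1_IntoCombo1.
; Ending resets targeting, restores controller yaw and removes Combo1.Two-tagged effects.
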(event `self.K2_ActivateAbility`
  (bind _returnvalue (`self.GetOwningActorFromActorInfo`))
  (bind _returnvalue_2 (`self.GetAvatarActorFromActorInfo`))
  (`self.K2_CommitAbility`)
  (bind _asbp_hephaestus (cast `/Game/Characters/Heroes/Hephaestus/BP_Hephaestus` _returnvalue_2))
  (set `Pawn.bUseControllerRotationYaw` false _asbp_hephaestus)
  (bind _overlappingactors (`PrimitiveComponent.GetOverlappingActors` (`/Game/Characters/Heroes/Hephaestus/BP_Hephaestus.MeeleRange` _asbp_hephaestus) "/Script/GodBound.GB_EnemyCharacter"))
  (if (`KismetArrayLibrary.Array_IsEmpty` _overlappingactors)
    (`AbilityTask_ApplyRootMotionMoveToForce.ApplyRootMotionMoveToForce` "None" (+ (* (`Actor.GetActorForwardVector` _returnvalue) (`KismetMathLibrary.Conv_DoubleToVector` 200.0)) (`Actor.K2_GetActorLocation` _returnvalue)) 0.2 false "MOVE_None" false null "SetVelocity"
      (:`then`
        _))
    (else
      (for _array_element _overlappingactors
        (bind _returnvalue_3 (`Actor.GetDistanceTo` _array_element _returnvalue_2))
        (if (< _returnvalue_3 (`self.ClosestEnemyDistance`))
          (set `self.ClosestEnemyDistance` _returnvalue_3)
          (set `self.ClosestEnemy` _array_element)))
      (bind _asynctaskproxy (`AbilityTask_ApplyRootMotionMoveToActorForce.ApplyRootMotionMoveToActorForce` "None" (`self.ClosestEnemy`) (0.0 0.0 0.0) "AlignToWorldSpace" 0.5 null null false "MOVE_None" false null null "SetVelocity")
        (:`then`
          _))))
  (`AbilityTask_PlayMontageAndWait.CreatePlayMontageAndWaitProxy` "None" (`self.AbilityMontage`) 1.0 "None" false
    (:`then`
      (`AbilityTask_WaitGameplayEvent.WaitGameplayEvent` (struct :`TagName` "Abilities.Hephaestus.F.Hit.Big") null
        (:`EventReceived`
          (if (`KismetSystemLibrary.IsValid` _asynctaskproxy)
            (`GameplayTask.EndTask` _asynctaskproxy))
          (bind _outactors (`KismetSystemLibrary.SphereOverlapActors` (`SceneComponent.GetSocketLocation` (`self.GetOwningComponentFromActorInfo`) "Hand_R_Punch") 100.0 (`|MakeArray` "ObjectTypeQuery8" "ObjectTypeQuery6" :!type "EObjectTypeQuery Enum")))
          (bind _returnvalue_4 (`AbilitySystemBlueprintLibrary.AssignTagSetByCallerMagnitude` (`self.MakeOutgoingGameplayEffectSpec` (`self.PunchDamageEffect`) (`KismetMathLibrary.Conv_IntToDouble` (`self.GetAbilityLevel`))) (struct :`TagName` "Damage") 50.0))
          (bind _returnvalue_5 (`AbilitySystemBlueprintLibrary.AbilityTargetDataFromActorArray` _outactors))
          (`self.K2_ApplyGameplayEffectSpecToTarget` _returnvalue_4 _returnvalue_5)
          (bind _returnvalue_6 (`self.SetContextEffectStrength` 1500.0 (`self.MakeOutgoingGameplayEffectSpec` "/Game/Characters/Heroes/SharedAbilities/KnockBack/GE_KnockBack.GE_KnockBack_C")))
          (`self.K2_ApplyGameplayEffectSpecToTarget` _returnvalue_6 _returnvalue_5)
          (`AbilityTask_WaitGameplayEvent.WaitGameplayEvent` (struct :`TagName` "Abilities.IntoCombo") null
            (:`EventReceived`
              (`self.BP_ApplyGameplayEffectToOwner` "/Game/Characters/Heroes/Hephaestus/Abilities/Fighter/Combo1/GE_C1_IntoCombo1.GE_C1_IntoCombo1_C"))))))
    (:`OnCompleted`
      (`self.K2_EndAbility` :!label _label))
    (:`OnBlendOut`
      (goto _label))
    (:`OnInterrupted`
      (goto _label))
    (:`OnCancelled`
      (goto _label))))

(event `self.K2_OnEndAbility`
  (params (bWasCancelled :type Boolean))
  (set `self.ClosestEnemy` null)
  (set `self.ClosestEnemyDistance` 10000.0)
  (`self.BP_RemoveGameplayEffectFromOwnerWithGrantedTags` (struct :`GameplayTags` (struct :`(TagName` "Abilities.Hephaestus.F.Combo1.Two"))))
  (bind _asbp_hephaestus (cast `/Game/Characters/Heroes/Hephaestus/BP_Hephaestus` (`self.GetAvatarActorFromActorInfo`)))
  (set `Pawn.bUseControllerRotationYaw` true _asbp_hephaestus))