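; Gameplay ability for step 4 of Hephaestus's fighter Combo 1: a lunging heavy punch.
; On activation it disables controller yaw until the ability ends and root-motion moves to the closest enemy in melee range, or forward if none.
; It plays the montage alongside the move and waits for the big-hit event.
; That event sphere-overlaps at the punch socket, applying SetByCaller damage and knockback effects to actors found.
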(event `self.K2_ActivateAbility`
  (bind _returnvalue (`self.GetOwningActorFromActorInfo`))
  (bind _returnvalue_2 (`self.GetOwningActorFromActorInfo`))
  (`self.K2_CommitAbility`)
  (bind _asbp_hephaestus (cast `/Game/Characters/Heroes/Hephaestus/BP_Hephaestus` _returnvalue_2))
  (set `Pawn.bUseControllerRotationYaw` false _asbp_hephaestus)
  (bind _overlappingactors (`PrimitiveComponent.GetOverlappingActors` (`/Game/Characters/Heroes/Hephaestus/BP_Hephaestus.MeeleRange` _asbp_hephaestus) "/Script/GodBound.GB_EnemyCharacter"))
  (if (`KismetArrayLibrary.Array_IsEmpty` _overlappingactors)
    (`AbilityTask_ApplyRootMotionMoveToForce.ApplyRootMotionMoveToForce` "None" (+ (* (`Actor.GetActorForwardVector` _returnvalue) (`KismetMathLibrary.Conv_DoubleToVector` 300.0)) (`Actor.K2_GetActorLocation` _returnvalue)) 0.5 false "MOVE_None" false null "MaintainLastRootMotionVelocity"
      (:`then`
        _))
    (else
      (for _array_element _overlappingactors
        (bind _returnvalue_3 (`Actor.GetDistanceTo` _array_element _returnvalue_2))
        (if (< _returnvalue_3 (`self.ClosestEnemyDistance`))
          (set `self.ClosestEnemy` _array_element)
          (set `self.ClosestEnemyDistance` _returnvalue_3)))
      (`AbilityTask_ApplyRootMotionMoveToActorForce.ApplyRootMotionMoveToActorForce` "None" (`self.ClosestEnemy`) (0.0 0.0 0.0) "AlignToWorldSpace" 0.5 null null false "MOVE_None" false null null "MaintainLastRootMotionVelocity"
        (:`then`
          _))))
  (`AbilityTask_PlayMontageAndWait.CreatePlayMontageAndWaitProxy` "None" (`self.AbilityMontage`) 1.0 "None" false 0.5
    (:`then`
      (`AbilityTask_WaitGameplayEvent.WaitGameplayEvent` (struct :`TagName` "Abilities.Hephaestus.F.Hit.Big") null
        (:`EventReceived`
          (bind _outactors (`KismetSystemLibrary.SphereOverlapActors` (`SceneComponent.GetSocketLocation` (`self.GetOwningComponentFromActorInfo`) "Hand_R_Punch") 200.0 (`|MakeArray` "ObjectTypeQuery6" "ObjectTypeQuery8" :!type "EObjectTypeQuery Enum")))
          (bind _returnvalue_4 (`AbilitySystemBlueprintLibrary.AssignTagSetByCallerMagnitude` (`self.MakeOutgoingGameplayEffectSpec` (`self.PunchDamageEffect`) (`KismetMathLibrary.Conv_IntToDouble` (`self.GetAbilityLevel`))) (struct :`TagName` "Damage") (`self.PunchDamage`)))
          (bind _returnvalue_5 (`AbilitySystemBlueprintLibrary.AbilityTargetDataFromActorArray` _outactors))
          (`self.K2_ApplyGameplayEffectSpecToTarget` _returnvalue_4 _returnvalue_5)
          (`self.BP_ApplyGameplayEffectToTarget` _returnvalue_5 (`self.KnockBackEffect`) 3 2))))
    (:`OnCompleted`
      (`self.K2_EndAbility` :!label _label))
    (:`OnBlendOut`
      (goto _label))
    (:`OnInterrupted`
      (goto _label))
    (:`OnCancelled`
      (goto _label))))

(event `self.K2_OnEndAbility`
  (params (bWasCancelled :type Boolean))
  (set `self.ClosestEnemy` null)
  (set `self.ClosestEnemyDistance` 10000.0)
  (bind _asbp_hephaestus (cast `/Game/Characters/Heroes/Hephaestus/BP_Hephaestus` (`self.GetOwningActorFromActorInfo`)))
  (set `Pawn.bUseControllerRotationYaw` true _asbp_hephaestus))