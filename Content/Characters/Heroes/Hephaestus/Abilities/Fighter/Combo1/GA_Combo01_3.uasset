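; Hephaestus Fighter Combo 1 ability (GA_Combo01_3): a montage-driven punch, punch, kick attack.
; On activation it root-motion moves toward the closest enemy in melee range, if any, while starting the montage.
; Gameplay events trigger socket sphere overlaps applying SetByCaller damage and knockback effects, though the big punch's knockback has no target data wired.
; An IntoCombo event applies GE_C1_IntoCombo3; ending removes Combo1.four-tagged effects and resets targeting.
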(event `self.K2_ActivateAbility`
  (bind _returnvalue (`self.GetOwningActorFromActorInfo`))
  (`self.K2_CommitAbility`)
  (bind _asbp_hephaestus (cast `/Game/Characters/Heroes/Hephaestus/BP_Hephaestus` _returnvalue))
  (bind _overlappingactors (`PrimitiveComponent.GetOverlappingActors` (`/Game/Characters/Heroes/Hephaestus/BP_Hephaestus.MeeleRange` _asbp_hephaestus) "/Script/GodBound.GB_EnemyCharacter"))
  (if (not (`KismetArrayLibrary.Array_IsEmpty` _overlappingactors))
    (for _array_element _overlappingactors
      (bind _returnvalue_2 (`Actor.GetDistanceTo` _array_element _returnvalue))
      (if (< _returnvalue_2 (`self.ClosestEnemyDistance`))
        (set `self.ClosestEnemyDistance` _returnvalue_2)
        (set `self.ClosestEnemy` _array_element)))
    (`AbilityTask_ApplyRootMotionMoveToActorForce.ApplyRootMotionMoveToActorForce` "None" (`self.ClosestEnemy`) (0.0 0.0 0.0) "AlignToWorldSpace" 0.2 null null false "MOVE_None" false null null "MaintainLastRootMotionVelocity"
      (:`then`
        _)))
  (`AbilityTask_PlayMontageAndWait.CreatePlayMontageAndWaitProxy` "None" (`self.AbilityMontage`) 1.0 "None" false
    (:`then`
      (`AbilityTask_WaitGameplayEvent.WaitGameplayEvent` (struct :`TagName` "Abilities.Hephaestus.F.Hit.Small") null true
        (:`then`
          (`AbilityTask_WaitGameplayEvent.WaitGameplayEvent` (struct :`TagName` "Abilities.Hephaestus.F.Hit.Big") null true
            (:`then`
              (`AbilityTask_WaitGameplayEvent.WaitGameplayEvent` (struct :`TagName` "Abilities.Hephaestus.F.Kick.Big") null true
                (:`then`
                  (`AbilityTask_WaitGameplayEvent.WaitGameplayEvent` (struct :`TagName` "Abilities.IntoCombo") null
                    (:`EventReceived`
                      (`self.BP_ApplyGameplayEffectToOwner` "/Game/Characters/Heroes/Hephaestus/Abilities/Fighter/Combo1/GE_C1_IntoCombo3.GE_C1_IntoCombo3_C"))))
                (:`EventReceived`
                  (bind _outactors (`KismetSystemLibrary.SphereOverlapActors` (`SceneComponent.GetSocketLocation` (`self.GetOwningComponentFromActorInfo`) "Foot_L_Kick") 100.0 (`|MakeArray` "ObjectTypeQuery6" "ObjectTypeQuery8" :!type "EObjectTypeQuery Enum")))
                  (bind _returnvalue_3 (`AbilitySystemBlueprintLibrary.AssignTagSetByCallerMagnitude` (`self.MakeOutgoingGameplayEffectSpec` (`self.KickDamageEffect`) (`KismetMathLibrary.Conv_IntToDouble` (`self.GetAbilityLevel`))) (struct :`TagName` "Damage") (`self.KickBigDamage`)))
                  (bind _returnvalue_4 (`AbilitySystemBlueprintLibrary.AbilityTargetDataFromActorArray` _outactors))
                  (`self.K2_ApplyGameplayEffectSpecToTarget` _returnvalue_3 _returnvalue_4)
                  (`self.BP_ApplyGameplayEffectToTarget` _returnvalue_4 (`self.KnockBackEffect`) 2))))
            (:`EventReceived`
              (bind _outactors_2 (`KismetSystemLibrary.SphereOverlapActors` (`SceneComponent.GetSocketLocation` (`self.GetOwningComponentFromActorInfo`) "Hand_R_Punch") 100.0 (`|MakeArray` "ObjectTypeQuery6" "ObjectTypeQuery8" :!type "EObjectTypeQuery Enum")))
              (bind _returnvalue_5 (`AbilitySystemBlueprintLibrary.AssignTagSetByCallerMagnitude` (`self.MakeOutgoingGameplayEffectSpec` (`self.PunchDamageEffect`) (`KismetMathLibrary.Conv_IntToDouble` (`self.GetAbilityLevel`))) (struct :`TagName` "Damage") (`self.PunchBigDamage`)))
              (`self.K2_ApplyGameplayEffectSpecToTarget` _returnvalue_5 (`AbilitySystemBlueprintLibrary.AbilityTargetDataFromActorArray` _outactors_2))
              (`self.BP_ApplyGameplayEffectToTarget` (struct) (`self.KnockBackEffect`)))))
        (:`EventReceived`
          (bind _outactors_3 (`KismetSystemLibrary.SphereOverlapActors` (`SceneComponent.GetSocketLocation` (`self.GetOwningComponentFromActorInfo`) "Hand_L_Punch") 100.0 (`|MakeArray` "ObjectTypeQuery6" "ObjectTypeQuery8" :!type "EObjectTypeQuery Enum")))
          (bind _returnvalue_6 (`AbilitySystemBlueprintLibrary.AssignTagSetByCallerMagnitude` (`self.MakeOutgoingGameplayEffectSpec` (`self.PunchDamageEffect`) (`KismetMathLibrary.Conv_IntToDouble` (`self.GetAbilityLevel`))) (struct :`TagName` "Damage") (`self.PunchSmallDamage`)))
          (bind _returnvalue_7 (`AbilitySystemBlueprintLibrary.AbilityTargetDataFromActorArray` _outactors_3))
          (`self.K2_ApplyGameplayEffectSpecToTarget` _returnvalue_6 _returnvalue_7)
          (`self.BP_ApplyGameplayEffectToTarget` _returnvalue_7 (`self.KnockBackEffect`)))))
    (:`OnCompleted`
      (`self.K2_EndAbility` :!label _label))
    (:`OnBlendOut`
      (goto _label))
    (:`OnInterrupted`
      (goto _label))
    (:`OnCancelled`
      (goto _label))))

(event `self.K2_OnEndAbility`
  (params (bWasCancelled :type Boolean))
  (`self.BP_RemoveGameplayEffectFromOwnerWithGrantedTags` (struct :`GameplayTags` (struct :`(TagName` "Abilities.Hephaestus.F.Combo1.four"))))
  (set `self.ClosestEnemyDistance` 10000.0)
  (set `self.ClosestEnemy` null))