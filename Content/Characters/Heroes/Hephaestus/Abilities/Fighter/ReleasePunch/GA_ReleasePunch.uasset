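; GA_ReleasePunch is a Gameplay Ability for Hephaestus's Fighter kit that throws a punch damaging targets in a line ahead.
; It commits, plays the punch montage at half speed and waits for the big-hit gameplay event.
; That event fires a forward multi-sphere trace from the right-hand socket, with debug drawing on, applying set-by-caller damage through GE_PulledKickDamage to each hit.
; The ability ends when the montage completes, blends out, is interrupted or is cancelled.
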(event `self.K2_ActivateAbility`
  (bind _returnvalue (`SceneComponent.GetSocketLocation` (`self.GetOwningComponentFromActorInfo`) "Hand_R_Punch"))
  (`self.K2_CommitAbility`)
  (`AbilityTask_PlayMontageAndWait.CreatePlayMontageAndWaitProxy` "None" "/Game/Characters/SharedAnimations/MeleeAnimations/FighterAnimations/Attacks/Hephaestus_ReleasePunch.Hephaestus_ReleasePunch" 0.5
    (:`then`
      (`AbilityTask_WaitGameplayEvent.WaitGameplayEvent` (struct :`TagName` "Abilities.Hephaestus.F.Hit.Big") null true
        (:`EventReceived`
          (bind _outhits (`KismetSystemLibrary.SphereTraceMultiForObjects` :`Start` _returnvalue :`End` (+ (* (`Actor.GetActorForwardVector` (`self.GetOwningActorFromActorInfo`)) (`KismetMathLibrary.Conv_DoubleToVector` 720.0)) _returnvalue) :`Radius` 100.0 :`ObjectTypes` (`|MakeArray` "ObjectTypeQuery8" :!type "EObjectTypeQuery Enum") :`DrawDebugType` "ForDuration"))
          (for _array_element _outhits
            (bind _returnvalue_2 (`AbilitySystemBlueprintLibrary.AssignTagSetByCallerMagnitude` (`self.MakeOutgoingGameplayEffectSpec` "/Game/Characters/Heroes/Hephaestus/Abilities/Fighter/PullKick/GE_PulledKickDamage.GE_PulledKickDamage_C") (struct :`TagName` "Damage") 150.0))
            (`self.K2_ApplyGameplayEffectSpecToTarget` _returnvalue_2 (`AbilitySystemBlueprintLibrary.AbilityTargetDataFromHitResult` _array_element))))))
    (:`OnCompleted`
      (`self.K2_EndAbility` :!label _label))
    (:`OnBlendOut`
      (goto _label))
    (:`OnInterrupted`
      (goto _label))
    (:`OnCancelled`
      (goto _label))))