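; Gameplay ability for a fallen hero who cannot move manually and can be executed before getting up.
; It attaches a BP_ExecutionArea in front of the avatar and applies each overlapping actor's own execution effect to that actor.
; An Abilities.Execution event plays the target montage supplied by the effect causer; otherwise a timed delay leads to the get-up montage and restored movement.
; Ending removes the granting effect and destroys the area.
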(event `self.K2_ActivateAbility`
  (bind _returnvalue (`self.GetAvatarActorFromActorInfo`))
  (bind _returnvalue_2 (`self.GetAvatarActorFromActorInfo`))
  (`self.K2_CommitAbility`)
  (message `/Game/Characters/Heroes/BI_AbilitiesGeneral.SetCanManuallyMove` _returnvalue false)
  (message `/Game/Characters/Heroes/BI_AbilitiesGeneral.SetInAbilityMontage` _returnvalue false)
  (`KismetSystemLibrary.PrintString` "Hello")
  (bind (_asynctaskproxy _spawnedactor) (`GameplayTask_SpawnActor.SpawnActor` null (+ (`Actor.K2_GetActorLocation` _returnvalue) (* (`Actor.GetActorForwardVector` _returnvalue) (`KismetMathLibrary.Conv_DoubleToVector` 70.0))) (`Actor.K2_GetActorRotation` _returnvalue) "/Game/Characters/Heroes/BP_ExecutionArea.BP_ExecutionArea_C" false null)
    (:`Success`
      (`Actor.K2_AttachToActor` _spawnedactor (`self.GetAvatarActorFromActorInfo`) "None" "KeepWorld" "KeepWorld" "KeepWorld" true)
      (set `self.ExecutionArea` _spawnedactor)
      (add `Actor.OnActorBeginOverlap` _spawnedactor (delegate `OnActorBeginOverlap_Event`))
      (`AbilityAsync_WaitGameplayEvent.WaitGameplayEventToActor` (`self.GetAvatarActorFromActorInfo`) (struct :`TagName` "Abilities.Execution")
        (:`then`
          (`AbilityTask_WaitDelay.WaitDelay` 10.0
            (:`OnFinish`
              (`AbilityTask_PlayMontageAndWait.CreatePlayMontageAndWaitProxy` "None" "/Game/Characters/SharedAnimations/MeleeAnimations/FighterAnimations/Hit/Montage_Fallen_GetUp.Montage_Fallen_GetUp" 1.0 "None" false
                (:`OnCompleted`
                  _)
                (:`OnBlendOut`
                  _)
                (:`OnInterrupted`
                  _)
                (:`OnCancelled`
                  _))
              (message `/Game/Characters/Heroes/BI_AbilitiesGeneral.SetCanManuallyMove` _returnvalue_2 true)
              (`self.K2_EndAbility`))))
        (:`EventReceived`
          (`Actor.K2_DestroyActor` (`self.ExecutionArea`))
          (set `self.ExecutionArea` null)
          (bind _returnvalue_3 (`AbilitySystemBlueprintLibrary.GetEffectContext` (struct)))
          (`KismetSystemLibrary.PrintString` "EXECUTING")
          (bind _newparam (message `/Game/Characters/Heroes/BI_AbilitiesGeneral.GetExecuteTargetAnimation` (`AbilitySystemBlueprintLibrary.EffectContextGetEffectCauser` _returnvalue_3)))
          (message `/Game/Characters/Heroes/BI_AbilitiesGeneral.PlayMontageMC` _returnvalue_2 _newparam)
          (`self.K2_EndAbility`))))
    (:`DidNotSpawn`
      (`self.K2_EndAbility`))))

(event `self.K2_OnEndAbility`
  (params (bWasCancelled :type Boolean))
  (bind _executionarea (`self.ExecutionArea`))
  (`self.RemoveGrantedByEffect`)
  (`/Engine/EditorBlueprintResources/StandardMacros.IsValid` _executionarea
    (:`Is Valid`
      (`Actor.K2_DestroyActor` _executionarea)
      (set `self.ExecutionArea` null))))

(event `OnActorBeginOverlap_Event`
  (params (OverlappedActor :type "Actor Object Reference") (OtherActor :type "Actor Object Reference"))
  (bind _newparam (message `/Game/Characters/Heroes/BI_AbilitiesGeneral.GetExecutionEffect` OtherActor))
  (`self.K2_ApplyGameplayEffectSpecToTarget` (`self.MakeOutgoingGameplayEffectSpec` _newparam) (`AbilitySystemBlueprintLibrary.AbilityTargetDataFromActor` OtherActor)))