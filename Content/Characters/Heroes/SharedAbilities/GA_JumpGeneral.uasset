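; Shared hero Gameplay Ability that makes the avatar and nearby GB_Character actors jump.
; On activation it commits, then runs a sphere overlap around the avatar, filtered to one object type and excluding the avatar.
; Each overlapped actor's name is printed and GB_Characters jump, then the avatar jumps and the ability ends.
; The commit result is not checked, and EndAbility only runs if the avatar casts to GB_Character.
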(event `self.K2_ActivateAbility`
  (bind _returnvalue (`self.GetAvatarActorFromActorInfo`))
  (`self.K2_CommitAbility`)
  (bind _outactors (`KismetSystemLibrary.SphereOverlapActors` (`Actor.K2_GetActorLocation` _returnvalue) 400.0 (`|MakeArray` "ObjectTypeQuery7" :!type "EObjectTypeQuery Enum") null (`|MakeArray` _returnvalue)))
  (for _array_element _outactors
    (`KismetSystemLibrary.PrintString` (`KismetSystemLibrary.GetObjectName` _array_element))
    (bind _asgb_character (cast `GB_Character` _array_element))
    (`Character.Jump` _asgb_character))
  (bind _asgb_character_2 (cast `GB_Character` _returnvalue))
  (`Character.Jump` _asgb_character_2)
  (`self.K2_EndAbility`))