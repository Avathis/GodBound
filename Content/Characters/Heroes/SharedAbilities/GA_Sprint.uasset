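; GA_Sprint is a shared hero gameplay ability that applies a running effect while its input is held.
; On activation it applies that effect, prints debug text and owned gameplay tags, then ends on input release.
; Ending sets the owner's movement type to Walking, removes the running effect by handle and applies a walking effect.
; An unconnected older branch that sets Sprinting on the cast movement component never runs.
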(event `self.K2_ActivateAbility`
  (bind _returnvalue (`self.BP_ApplyGameplayEffectToOwner` (`self.RunningeEffect`)))
  (`KismetSystemLibrary.PrintString` "Hello")
  (bind _tagcontainer (message `GameplayTagAssetInterface.GetOwnedGameplayTags` (`.AbilitySystemComponent` (break `GameplayAbilityActorInfo` (`self.GetActorInfo`)))))
  (`KismetSystemLibrary.PrintString` (`BlueprintGameplayTagLibrary.GetDebugStringFromGameplayTagContainer` _tagcontainer))
  (`AbilityTask_WaitInputRelease.WaitInputRelease` false
    (:`OnRelease`
      (`self.K2_EndAbility`))))

(event `self.K2_OnEndAbility`
  (params (bWasCancelled :type Boolean))
  (message `/Game/Interfaces/BPI_MovementInterface.Change Movement Type` (`.OwnerActor` (break `GameplayAbilityActorInfo` (`self.GetActorInfo`))) "EMS_Walking")
  (`self.BP_RemoveGameplayEffectFromOwnerWithHandle` (stale `self.K2_ActivateAbility` _returnvalue))
  (`self.BP_ApplyGameplayEffectToOwner` (`self.WalkingEffect`)))