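; Gameplay Ability that knocks its owner up and away, using the context of the Gameplay Effect that granted it.
; On activation it commits, then runs a root motion move-to-force task toward a point offset along the effect instigator's forward vector and raised above the owner.
; The short move keeps its final root motion velocity, and the ability ends when the task times out, whether or not the destination is reached.
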(event `self.K2_ActivateAbility`
  (`self.K2_CommitAbility`)
  (`AbilityTask_ApplyRootMotionMoveToForce.ApplyRootMotionMoveToForce` "None" (+ (* (`Actor.GetActorForwardVector` (`AbilitySystemBlueprintLibrary.EffectContextGetInstigatorActor` (`self.GetGrantedByEffectContext`))) (`KismetMathLibrary.Conv_DoubleToVector` 200.0)) (`Actor.K2_GetActorLocation` (`self.GetOwningActorFromActorInfo`)) (0.0 0.0 250.0)) 0.5 false "MOVE_None" false null "MaintainLastRootMotionVelocity"
    (:`OnTimedOut`
      _)
    (:`OnTimedOutAndDestinationReached`
      _))
  (`self.K2_EndAbility`))