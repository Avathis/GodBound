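; Shared hero gameplay ability that knocks its owner back, driven by the gameplay effect that granted it.
; An additive root motion constant force pushes along the effect causer's forward vector, scaled by the effect's strength, shaped by a curve and with gravity enabled.
; A half-speed knockback montage plays alongside and may outlast the ability, which ends when the brief force finishes.
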(event `self.K2_ActivateAbility`
  (`self.K2_CommitAbility`)
  (`AbilityTask_ApplyRootMotionConstantForce.ApplyRootMotionConstantForce` "None" (`Actor.GetActorForwardVector` (`AbilitySystemBlueprintLibrary.EffectContextGetEffectCauser` (`self.GetGrantedByEffectContext`))) (`GB_AbilitySystemLibrary.GetEffectStrength` (`self.GetGrantedByEffectContext`)) 0.3 true "/Game/Characters/Heroes/SharedAbilities/KnockBack/Curve_KnockBack.Curve_KnockBack" "MaintainLastRootMotionVelocity" (0.0 0.0 0.0) 0.0 true
    (:`then`
      (`AbilityTask_PlayMontageAndWait.CreatePlayMontageAndWaitProxy` "None" "/Game/Characters/SharedAnimations/MeleeAnimations/FighterAnimations/Hit/Montage_KnockBack.Montage_KnockBack" 0.5 "None" false))
    (:`OnFinish`
      (`self.K2_EndAbility`))))