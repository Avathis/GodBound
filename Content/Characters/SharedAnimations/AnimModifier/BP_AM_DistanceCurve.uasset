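; Animation modifier that bakes a distance float curve into an animation sequence from the root bone's position.
; On apply it removes any existing curve of the configured name, re-adds it, then loops over the frames writing the length of the root bone's location vector as keys.
; Each key's time comes from the total frame count instead of the loop index, so all keys target the same end time.
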(event `self.OnApply`
  (params (AnimationSequence :type "AnimSequence Object Reference"))
  (bind _animsequence (`self.AnimSequence`))
  (bind _numframes (`AnimationBlueprintLibrary.GetNumFrames` _animsequence))
  (bind _output_get (set `self.AnimSequence` AnimationSequence))
  (bind _returnvalue (`AnimationBlueprintLibrary.DoesCurveExist` _output_get (`self.CurveName`) "RCT_Float"))
  (if _returnvalue
    (`AnimationBlueprintLibrary.RemoveCurve` (`self.AnimSequence`) (`self.CurveName`)))
  (`AnimationBlueprintLibrary.AddCurve` (`self.AnimSequence`) (`self.CurveName`))
  (for _index (range (+ _numframes 1))
    (bind _pose_location (`KismetMathLibrary.BreakTransform` (`AnimationBlueprintLibrary.GetBonePoseForFrame` (`self.AnimSequence`) (`self.RootBoneName`) _index)))
    (`AnimationBlueprintLibrary.AddFloatCurveKey` (`self.AnimSequence`) (`self.CurveName`) (`AnimationBlueprintLibrary.GetTimeAtFrame` _animsequence _numframes) (`KismetMathLibrary.VSize` _pose_location))))