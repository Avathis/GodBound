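; Melee minion target dummy character that uses the Gameplay Ability System to hold attributes and react to hits.
; On BeginPlay it applies the default attributes effect to itself and grants the hit react ability under the Abilities tag.
; Leftover disconnected test nodes print health, trigger the hit react and self-apply set-by-caller Grux damage, but none of them run.
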(event `self.ReceiveBeginPlay`
  (`AbilitySystemComponent.BP_ApplyGameplayEffectToSelf` :`self` (`self.ASC`) :`GameplayEffectClass` "/Game/Characters/Targets/MeleeTargetDummy/GE_DefaultAttributes.GE_DefaultAttributes_C")
  (`self.GrantAbility` "/Game/Characters/Targets/MeleeTargetDummy/GA_HitReact.GA_HitReact_C" 0 0 (struct :`TagName` "Abilities")))

(event `self.ReceiveTick`
  (params (DeltaSeconds :type "Float (single-precision)")))

(fn `UserConstructionScript`)